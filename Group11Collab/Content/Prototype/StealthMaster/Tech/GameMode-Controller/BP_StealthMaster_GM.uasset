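; BP_StealthMaster_GM is the game mode for the StealthMaster prototype, handling enemy spawning and respawning.
; On BeginPlay it finds every AISPawner actor, triggers an initial spawn from each and caches them in Spawners.
; The AIDeath event removes the dead enemy from Enemies, then calls FSpawnAIRecur to spawn a replacement at a randomly chosen cached spawner.
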(event Custom|AIDeath
  (params (Enemy :type Enemy%20Base%20Class%20SM%20Object%20Reference))
  (Utilities|Array|RemoveItem (Variables|Default|GetEnemies) Enemy)
  (CallFunction|FSpawnAIRecur))

(event EventBeginPlay
  (bind _outactors (Actor|GetAllActorsOfClass "/Game/Prototype/StealthMaster/Tech/AI/AISPawner.AISPawner_C"))
  (for _array_element _outactors
    (Default|SpawnAI _array_element)
    (Utilities|Array|Add (Variables|Default|GetSpawners) _array_element)))

(fn ConstructionScript)

(fn FSpawnAIRecur
  (bind _spawners (Variables|Default|GetSpawners))
  (Default|SpawnAI (Utilities|Array|Get(acopy) _spawners (Math|Random|RandomIntegerinRange 0 (- (Utilities|Array|Length _spawners) 1)))))