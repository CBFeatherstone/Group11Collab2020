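; AI controller for StealthMaster enemies that runs a behavior tree and feeds its blackboard on sight, range and patrol.
; On possess it caches the enemy and first player character, seeds patrol and wait-time keys, and starts a looping range check against the enemy's attack range.
; Perception updates set player visibility, storing the player's location and a recently-sighted flag when perception is lost.
; Walk, Run and Attack events forward to the controlled enemy.
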(event OnTargetPerceptionUpdated(AIPerception)
  (params (Actor :type Actor%20Object%20Reference) (Stimulus :type AI%20Stimulus%20Structure))
  (bind _bsuccessfullysensed (Utilities|Struct|BreakAIStimulus Stimulus))
  (bind _returnvalue (AI|GetBlackboard 0))
  (Utilities|Casting|CastToBP_StealthMaster Actor
    (:then
      _)
    (:CastFailed
      (Utilities|Casting|CastToBP_PlayerController_StealthMaster Actor
        (:then
          _)
        (:CastFailed
          (Utilities|Casting|CastToBP_PlayerController_Korruption Actor)))))
  (AI|Components|Blackboard|SetValueasBool _returnvalue (Utilities|Name|MakeLiteralName "CanSeePlayer?") _bsuccessfullysensed)
  (if (not _bsuccessfullysensed)
    (AI|Components|Blackboard|SetValueasVector _returnvalue (Utilities|Name|MakeLiteralName "PlayerLocation") (Transformation|GetActorLocation (Game|Player|GetPlayerPawn 0)))
    (AI|Components|Blackboard|SetValueasBool _returnvalue (Utilities|Name|MakeLiteralName "RecentlySightedPlayer") true)))

(event Custom|Walk
  (Default|Walk (Variables|Default|GetAI_CharacterRef)))

(event Custom|Run
  (Default|Run (Variables|Default|GetAI_CharacterRef)))

(event Custom|Attack
  (Default|Attack (Variables|Default|GetAI_CharacterRef)))

(event EventBeginPlay
  (bind _asenemy_base_class_sm (Utilities|Casting|CastToEnemyBaseClass_SM (Pawn|GetControlledPawn)))
  (Variables|Default|SetminAttackRange (Variables|/Game/Prototype/StealthMaster/Tech/Enemies/EnemyBaseClass_SM.EnemyBaseClass_SM_C|GetRange _asenemy_base_class_sm)))

(event EventPossess
  (params (PossessedPawn :type Pawn%20Object%20Reference))
  (bind _returnvalue (AI|GetBlackboard 0))
  (bind _asenemy_base_class_sm (Utilities|Casting|CastToEnemyBaseClass_SM PossessedPawn))
  (Variables|Default|SetAI_CharacterRef _asenemy_base_class_sm)
  (AI|RunBehaviorTree "/Game/Prototype/StealthMaster/Tech/AI/BehaviourTree.BehaviourTree")
  (bind _outactors (Actor|GetAllActorsOfClass "/Game/Prototype/StealthMaster/Tech/Character/BP_StealthMaster.BP_StealthMaster_C"))
  (Variables|Default|SetCharacterRef (Utilities|Array|Get(acopy) _outactors))
  (Utilities|Time|SetTimerbyFunctionName 0 "F_CheckRange" 0.5 true)
  (AI|Components|Blackboard|SetValueasBool _returnvalue (Utilities|Name|MakeLiteralName "Patrol?") (Variables|/Game/Prototype/StealthMaster/Tech/Enemies/EnemyBaseClass_SM.EnemyBaseClass_SM_C|GetPatrol? (Variables|Default|GetAI_CharacterRef)))
  (AI|Components|Blackboard|SetValueasFloat _returnvalue (Utilities|Name|MakeLiteralName "WaitTime") 0.0))

(fn ConstructionScript)

(fn FCheckRange
  (bind _output_get (Variables|Default|SetRange (Math|Vector|Distance(Vector) (Transformation|GetWorldLocation (Variables|/Script/Engine.Actor|GetRootComponent (Variables|Default|GetAI_CharacterRef))) (Transformation|GetWorldLocation (Variables|/Script/Engine.Character|GetMesh (Variables|Default|GetCharacterRef))))))
  (AI|Components|Blackboard|SetValueasBool (AI|GetBlackboard 0) (Utilities|Name|MakeLiteralName "inRange") (<= _output_get (Variables|Default|GetminAttackRange)))
  (if (<= (Variables|Default|GetRange) 1e+03)
    _))