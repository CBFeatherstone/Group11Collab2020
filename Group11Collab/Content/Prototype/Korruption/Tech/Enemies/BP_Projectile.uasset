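; BP_Projectile is a thrown projectile whose size and damage scale with ThrowPower.
; On BeginPlay it raises MaxDamage to at least BaseDamage and sets its scale from ThrowPower plus a small offset.
; On collision overlap it applies damage interpolated between base and max by ThrowPower, then destroys itself.
; Damage always names the first player's controller as instigator and the projectile's owner as causer.
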(event OnComponentBeginOverlap(ProjectileCollision)
  (params (OverlappedComponent :type Primitive%20Component%20Object%20Reference) (OtherActor :type Actor%20Object%20Reference) (OtherComp :type Primitive%20Component%20Object%20Reference) (OtherBodyIndex :type Integer) (bFromSweep :type Boolean) (SweepResult :type Hit%20Result%20Structure%20%28by%20ref%29))
  (Utilities|IsValid OtherActor
    (:Is%20Valid
      (Game|Damage|ApplyDamage OtherActor (Math|Float|Lerp (Variables|Default|GetBaseDamage) (Variables|Default|GetMaxDamage) (Variables|Default|GetThrowPower)) (Game|GetPlayerController 0) (Components|GetOwner))
      (Actor|DestroyActor))))

(event EventBeginPlay
  (bind _throwpower (Variables|Default|GetThrowPower))
  (bind _returnvalue (+ _throwpower 0.2))
  (Utilities|FlowControl|Sequence
    (:then_0
      ;[1 1 1 1 12] In the event that max damage is not set correctly, then make it equal to base damage.
      (if (< (Variables|Default|GetMaxDamage) (Variables|Default|GetBaseDamage))
        (Variables|Default|SetMaxDamage (Variables|Default|GetBaseDamage))))
    (:then_1
      ;[1 1 1 1 16] Scale projectile size by throw power
      (Transformation|SetActorScale3D (Math|Vector|MakeVector _returnvalue _returnvalue _returnvalue)))))

(fn ConstructionScript)