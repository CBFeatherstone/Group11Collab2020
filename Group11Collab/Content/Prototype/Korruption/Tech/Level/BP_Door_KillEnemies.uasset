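; Level door that blows itself up, with explosion effect and sound, once all of its linked enemies are dead.
; On BeginPlay it attaches an objective marker to each enemy and starts a fast looping timer that counts invalid enemy references as kills, removing their markers.
; A trigger volume, sized and positioned in the construction script, turns marker visibility on the first time it is overlapped.
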(event OnComponentBeginOverlap(MarkerTriggerVolume)
  (params (OverlappedComponent :type Primitive%20Component%20Object%20Reference) (OtherActor :type Actor%20Object%20Reference) (OtherComp :type Primitive%20Component%20Object%20Reference) (OtherBodyIndex :type Integer) (bFromSweep :type Boolean) (SweepResult :type Hit%20Result%20Structure%20%28by%20ref%29))
  (Utilities|FlowControl|DoOnce false
    (:Completed
      (CallFunction|ToggleMarkers true))))

(event Custom|OpenDoor
  (Effects|SpawnEmitteratLocation "/Game/TemplateContent/StarterContent/Particles/P_Explosion.P_Explosion" (Transformation|GetActorLocation) "0, 0, 0" "5.000000,5.000000,5.000000")
  (Audio|PlaySound2D "/Game/StarterContent/Audio/Explosion02.Explosion02" 1.25 (Math|Random|RandomFloatinRange 0.9 1.5) 0.0 0 0)
  (for _array_element (Variables|Default|GetMarkers)
    (Utilities|IsValid _array_element
      (:Is%20Valid
        (Actor|DestroyActor _array_element))))
  (Actor|DestroyActor))

(event Custom|Check%20Enemies%20Are%20Alive
  ;[1 1 1] Open the door when all enemies are dead
  (bind _alldead (CallFunction|AreEnemiesDead))
  (if _alldead
    (CallFunction|OpenDoor)))

(event EventBeginPlay
  ;[1 1 1] Add Markers to each enemy
  (for _array_element (Variables|Default|GetLinkedEnemies)
    (bind _returnvalue (Game|SpawnActorfromClass "/Game/StealthMaster/Tech/UI/ObjectiveMarker.ObjectiveMarker_C" (Math|Transform|MakeTransform "0, 0, 0" "0, 0, 0" "1,1,1") "AlwaysSpawn" 0 "NewEnumerator1" 0))
    (Utilities|Array|Add (Variables|Default|GetMarkers) _returnvalue)
    (Variables|/Game/StealthMaster/Tech/UI/ObjectiveMarker.ObjectiveMarker_C|SetHideWhenPlayerClose _returnvalue false)
    (Transformation|AttachActorToActor _returnvalue _array_element "None" "KeepRelative" "KeepRelative" "KeepRelative" true))
  ;[1 1 1] Open the door when all enemies are dead
  (Utilities|Time|SetTimerbyEvent (delegate Custom|Check%20Enemies%20Are%20Alive) 0.05 true))

(fn ConstructionScript
  (Components|Box|SetBoxExtent (Variables|Default|GetMarkerTriggerVolume) (Variables|Default|GetMarkerTriggerVolumeExtents) false)
  (Transformation|SetRelativeLocation (Variables|Default|GetMarkerTriggerVolume) (Variables|Default|GetTriggerPos) false true))

(fn ToggleMarkers
  (params (Toggle :type Boolean))
  (if Toggle
    (for _array_element (Variables|Default|GetMarkers)
      (Utilities|IsValid _array_element
        (:Is%20Valid
          (Default|ToggleVisibility _array_element true))))
    (else
      (for _array_element_2 (Variables|Default|GetMarkers)
        (Utilities|IsValid _array_element_2
          (:Is%20Valid
            (Default|ToggleVisibility _array_element_2 false)))))))

(fn AreEnemiesDead
  (for (_array_element _array_index) (Variables|Default|GetLinkedEnemies)
    (Utilities|IsValid _array_element
      (:Is%20Not%20Valid
        (Math|Integer|IncrementInt (LocalVariables|GetNumDeadEnemies)
          (:%20%20
            (Utilities|IsValid (Utilities|Array|Get(acopy) (Variables|Default|GetMarkers) _array_index)
              (:Is%20Valid
                (Actor|DestroyActor (Utilities|Array|Get(acopy) (Variables|Default|GetMarkers) _array_index)))))))))
  (if (== (Utilities|Array|Length (Variables|Default|GetLinkedEnemies)) (LocalVariables|GetNumDeadEnemies))
    (return true)
    (else
      (return false))))