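; Wall Blueprint that procedurally builds a straight run of concrete wall segments with metal piping in the Construction Script.
; When EndPoint has a nonzero XY component, two loops add static mesh components at fixed intervals, their count derived from the vector's length.
; Pieces always extend along local X, so EndPoint's direction does not steer the wall.
; The event graph holds no active logic.
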(event EventBeginPlay)

(event Collision|EventActorBeginOverlap
  (params (OtherActor :type Actor%20Object%20Reference)))

(event EventTick
  (params (DeltaSeconds :type Float%20%28single-precision%29)))

(fn ConstructionScript
  (bind _end_point (Variables|Default|GetEnd_Point))
  (bind _returnvalue (Math|Vector|VectorLength _end_point))
  (bind _returnvalue_2 (/ _returnvalue 5e+02))
  (bind _returnvalue_3 (Math|Float|Floor _returnvalue_2))
  (if (Class|KismetMathLibrary|NotEqualExactlyVectorVector (* (Variables|Default|GetEnd_Point) "1.000000,1.000000, 0") "0, 0, 0")
    (Utilities|FlowControl|Sequence
      (:then_0
        (for _index (range 0 _returnvalue_3)
          (bind _returnvalue_4 (AddComponent|AddStaticMeshComponent false))
          (Components|StaticMesh|SetStaticMesh _returnvalue_4 "/Game/Assets/Wall_Segment_01.Wall_Segment_01")
          (Rendering|Material|SetMaterial _returnvalue_4 0 "/Game/Materials/MasterMaterials/Concrete_Inst.Concrete_Inst")
          (Transformation|SetRelativeLocation _returnvalue_4 (Math|Vector|MakeVector (* _index 5e+02) 0.0 0.0) false false)))
      (:then_1
        (for _index_2 (range 0 _returnvalue_3)
          (bind _returnvalue_5 (AddComponent|AddStaticMeshComponent false))
          (Components|StaticMesh|SetStaticMesh _returnvalue_5 "/Game/Assets/Piping_Variation_01.Piping_Variation_01")
          (Rendering|Material|SetMaterial _returnvalue_5 0 "/Game/Materials/MasterMaterials/Metal_Inst.Metal_Inst")
          (Transformation|SetRelativeLocation _returnvalue_5 (Math|Vector|MakeVector (* _index_2 5e+02) 0.0 0.0) false false))))))