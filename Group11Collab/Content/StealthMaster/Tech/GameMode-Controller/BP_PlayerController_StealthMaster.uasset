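; Player controller Blueprint for the StealthMaster stealth game, implementing a set of interface getter functions.
; Only I_GetActor does real work, returning the controlled pawn.
; The other getters for controller, cover, occupancy, patrol, range, stun, visibility and wait time are stubs returning empty, false or zero values.
; BeginPlay, Tick and the construction script contain no logic.
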(event EventBeginPlay)

(event EventTick
  (params (DeltaSeconds :type Float%20%28single-precision%29)))

(fn ConstructionScript)

(fn IGetActor
  (return (Pawn|GetControlledPawn)))

(fn IGetController
  (return 0))

(fn IGetLookforCover
  (return false))

(fn IGetOccupied
  (return false))

(fn IGetPatrol?
  (return false))

(fn IGetPatrolLoop?
  (return false))

(fn IGetPatrolPathActor
  (return 0))

(fn IGetPatrolPathPoints
  (return 0))

(fn IGetRange
  (return 0.0))

(fn IGetStunned?
  (return false))

(fn IGetVisibilityGM
  (return 0.0 false))

(fn IGetWaitTime
  (return 0.0))