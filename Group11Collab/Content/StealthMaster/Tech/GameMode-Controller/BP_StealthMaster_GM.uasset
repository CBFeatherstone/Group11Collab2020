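; Stealth game mode that tracks player visibility, an enemy list and AI sectors.
; Visibility sums reported light with a per-tick sun trace, though both trace branches set 100, so the player always passes the visible threshold.
; Camera and drone alerts set retriggerable timed spotted flags, returned with visibility through an interface.
; Sectors are mapped by index; player sector changes broadcast an AI toggle and respawn that sector's missing enemies.
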(event Custom|PlayerSeenByCamera
  (params (PlayerLocation :type Vector))
  (Variables|Default|SetplayerSpotted_SecurityCamera true)
  (Utilities|FlowControl|RetriggerableDelay (Variables|Default|GetplayerCameraSpottedDuration))
  (Variables|Default|SetplayerSpotted_SecurityCamera false))

(event EventBeginPlay
  (CallFunction|FDirectionalLightSetup)
  (CallFunction|FCharacterRef)
  (CallFunction|FSetupSectors)
  (Default|CallDToggleAISectors)
  (bind _outactors (Actor|GetAllActorsOfClass "/Game/StealthMaster/Tech/AI/BluePrints/BP_SecurityCamera.BP_SecurityCamera_C"))
  (for _array_element _outactors
    (bind _output (Class|IAI|IGetCameraObject(Message) _array_element))
    (EventDispatchers|BindEventtoAlertAI _output (EventDispatchers|CreateEvent :!event Custom|PlayerSeenByCamera))))

(event EventIGMAddEnemy
  (params (Input :type Actor%20Object%20Reference))
  (Utilities|Array|Add (Variables|Default|GetEnemies) Input))

(event EventIAIDeathPassthrough
  (params (Input :type Actor%20Object%20Reference))
  (Utilities|Array|RemoveItem (Variables|Default|GetEnemies) Input))

(event EventTick
  (params (DeltaSeconds :type Float%20%28single-precision%29))
  (CallFunction|FChechSun))

(event EventIUpdateVisibility
  (params (Input :type Float%20%28single-precision%29))
  (CallFunction|FUpdateVisibility Input))

(event EventIUpdatePlayerSector
  (params (Input :type Integer))
  (Variables|Default|SetplayerSector Input)
  (Default|CallDToggleAISectors)
  (CallFunction|FRespawnDeadAgents Input))

(event EventIKillAllAIDEBUG
  (params (input :type Integer))
  (Class|IAI|IKillAllAIDEBUG(Message) (.Value (Utilities|Map|Find (Variables|Default|GetSectors) input))))

(event EventIAlertAI
  (params (hitLocation :type Vector :default "0, 0, 0"))
  (Variables|Default|SetplayerSpotted_Drone true)
  (Utilities|FlowControl|RetriggerableDelay (Variables|Default|GetplayerDroneSpottedDuration))
  (Variables|Default|SetplayerSpotted_Drone false))

(fn ConstructionScript)

(fn FDirectionalLightSetup
  (bind _outactors (Actor|GetAllActorsOfClass "/Script/Engine.DirectionalLight"))
  (Variables|Default|SetsunRef (Utilities|Array|Get(acopy) _outactors)))

(fn FCharacterRef
  (Variables|Default|SetplayerRef (Pawn|GetControlledPawn (Game|GetPlayerController 0))))

(fn FChechSun
  (bind _playerref (Variables|Default|GetplayerRef))
  (bind _returnvalue (Transformation|GetActorLocation _playerref))
  (bind _returnvalue_2 (Collision|LineTraceByChannel _returnvalue (+ _returnvalue (* (Transformation|GetActorForwardVector (Variables|Default|GetsunRef)) -1e+05)) "TraceTypeQuery1" false 0 "None" true "(R=1.000000,G=0.000000,B=0.000000,A=1.000000)" "(R=0.000000,G=0.848716,B=1.000000,A=1.000000)"))
  (if _returnvalue_2
    (Variables|Default|SetsunAffect 1e+02)
    (else
      (Variables|Default|SetsunAffect 1e+02))))

(fn FUpdateVisibility
  (params (Input :type Float%20%28single-precision%29))
  (if (< Input 0.01)
    (Variables|Default|SetlightAffect 0.0)
    (else
      (Variables|Default|SetlightAffect Input))))

(fn FPrintVisibility
  (bind _output_get (Variables|Default|SetplayerVisibility (Math|Float|Clamp(Float) (* (+ (Variables|Default|GetlightAffect) (Variables|Default|GetsunAffect)) 1e+02) 0.0 1e+02)))
  (Development|PrintText (Utilities|Text|FormatText "You're {x}% Visible" _output_get)))

(fn FSetupSectors
  (bind _outactors (Actor|GetAllActorsOfClass "/Game/StealthMaster/Tech/AI/BluePrints/BP_Sector.BP_Sector_C"))
  (for _array_element _outactors
    (bind _output (Class|IAI|IGetSectorIndex(Message) _array_element))
    (Utilities|Map|Add (Variables|Default|GetSectors) _output _array_element)))

(fn FRespawnDeadAgents
  (params (SectorIndex :type Integer))
  (bind _returnvalue (+ SectorIndex 0))
  (bind _returnvalue_2 (+ SectorIndex 0))
  (bind _sectors (Variables|Default|GetSectors))
  (bind _value (Utilities|Map|Find _sectors _returnvalue_2))
  (bind _value_2 (Utilities|Map|Find _sectors _returnvalue))
  (Utilities|FlowControl|Sequence
    (:then_0
      (bind (_current _max) (Class|IAI|IGetEnemyCurr/Max(Message) _value))
      (if (not (>= _current _max))
        (Class|IAI|IRespawnAI(Message) _value _returnvalue_2 (- _max _current))))
    (:then_1
      (bind (_current_2 _max_2) (Class|IAI|IGetEnemyCurr/Max(Message) _value_2))
      (if (not (>= _current_2 _max_2))
        (Class|IAI|IRespawnAI(Message) _value_2 _returnvalue (- _max_2 _current_2))))))

(fn IGetActive
  (return false))

(fn IGetActor
  (return 0))

(fn IGetCameraObject
  (return 0))

(fn IGetController
  (return 0))

(fn IGetElevatorLevel
  (return 0))

(fn IGetEnemyCurr/Max
  (return 0 0))

(fn IGetIsDrone
  (return false))

(fn IGetLookforCover
  (return false))

(fn IGetObjectType
  (return "NewEnumerator0"))

(fn IGetOccupied
  (return false))

(fn IGetOverlappingActors
  (return 0))

(fn IGetPatrol?
  (return false))

(fn IGetPatrolLoop?
  (return false))

(fn IGetPatrolPathActor
  (return 0))

(fn IGetPatrolPathPoints
  (return 0))

(fn IGetPawnReference
  (return 0))

(fn IGetPlayerSector
  (return (Variables|Default|GetplayerSector)))

(fn IGetPlaystyle
  (return "NewEnumerator0"))

(fn IGetRange
  (return 0.0))

(fn IGetSector
  (params (Input :type Integer))
  (return (.Value (Utilities|Map|Find (Variables|Default|GetSectors) Input))))

(fn IGetSectorIndex
  (return (Variables|Default|GetplayerSector)))

(fn IGetSectorSize
  (return "0, 0, 0"))

(fn IGetStance
  (return "NewEnumerator0"))

(fn IGetStunned?
  (return false))

(fn IGetVisibilityGM
  (bind _playerspotted_securitycamera (Variables|Default|GetplayerSpotted_SecurityCamera))
  (bind _playerspotted_drone (Variables|Default|GetplayerSpotted_Drone))
  (Variables|Default|SetplayerVisibility (+ (Variables|Default|GetsunAffect) (Variables|Default|GetlightAffect)))
  (if (Variables|Default|GetplayerSpotted_Drone)
    (return (Variables|Default|GetplayerVisibility) _playerspotted_drone false _playerspotted_drone)
    (elif _playerspotted_securitycamera
      (return (Variables|Default|GetplayerVisibility) _playerspotted_securitycamera _playerspotted_securitycamera false)
      (elif (>= (Variables|Default|GetplayerVisibility) 6e+01)
        (return (Variables|Default|GetplayerVisibility) (>= (Variables|Default|GetplayerVisibility) 6e+01) false false)
        (else
          (return (Variables|Default|GetplayerVisibility) (>= (Variables|Default|GetplayerVisibility) 6e+01) false false))))))

(fn IGetWaitTime
  (return 0.0))