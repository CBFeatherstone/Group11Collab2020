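; BP_EMPProjectile_V1 is an EMP projectile that detonates on a fixed timer after spawning.
; BeginPlay waits a short delay, then calls Explode.
; Explode fires the RadialForce impulse, applies full, non-falloff radial damage around the collision sphere using ExplosionDamage, then destroys the actor.
; The graph has no impact-triggered detonation or EMP-specific effect; overlap and tick events are disabled stubs.
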(event Custom|Explode
  ;[1 1 1] Explode
  (Class|RadialForceComponent|FireImpulse (Variables|Default|GetRadialForce))
  (Game|Damage|ApplyRadialDamage (Variables|Default|GetExplosionDamage) (Transformation|GetWorldLocation (Variables|Default|GetSphereCollision)) 1e+03 0 0 0 0 true "ECC_Visibility")
  (Actor|DestroyActor))

(event Collision|EventActorBeginOverlap
  (params (OtherActor :type Actor%20Object%20Reference))
  (|CallParentFunction OtherActor) ; This node is disabled and will not be called.\nDrag off pins to build functionality.
)

(event EventTick
  (params (DeltaSeconds :type Float%20%28single-precision%29))
  (|CallParentFunction DeltaSeconds) ; This node is disabled and will not be called.\nDrag off pins to build functionality.
)

(event EventBeginPlay
  ;[1 1 1] Explosion Delay
  (Utilities|FlowControl|Delay 3.0)
  (CallFunction|Explode))

(fn ConstructionScript
  (|CallParentFunction))