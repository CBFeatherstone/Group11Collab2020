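; BP_Taser_Weapon_V1 is a taser weapon Blueprint that fires a short-range hitscan shot through the IFireWeapon event.
; Firing runs a Visibility line trace 500 units forward from WeaponFirePoint, with debug drawing for a set duration.
; A hit calls ApplyDamage with LineTraceDamage, but no damaged actor is connected, so the hit actor receives no damage.
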(event EventBeginPlay
  (|CallParentFunction) ; This node is disabled and will not be called.\nDrag off pins to build functionality.
)

(event Collision|EventActorBeginOverlap
  (params (OtherActor :type Actor%20Object%20Reference))
  (|CallParentFunction OtherActor) ; This node is disabled and will not be called.\nDrag off pins to build functionality.
)

(event EventTick
  (params (DeltaSeconds :type Float%20%28single-precision%29))
  (|CallParentFunction DeltaSeconds) ; This node is disabled and will not be called.\nDrag off pins to build functionality.
)

(event EventIFireWeapon
  (bind _weaponfirepoint (Variables|Default|GetWeaponFirePoint))
  (bind _returnvalue (Transformation|GetWorldLocation _weaponfirepoint))
  ;[1 1 1] Spawn Line Trace
  (bind (_outhit _returnvalue_2) (Collision|LineTraceByChannel _returnvalue (+ _returnvalue (* (Math|Vector|GetForwardVector _weaponfirepoint) 5e+02)) "TraceTypeQuery1" false 0 "ForDuration"))
  (if _returnvalue_2
    (Game|Damage|ApplyDamage 0 (Variables|Default|GetLineTraceDamage) 0 0)))

(fn ConstructionScript
  (|CallParentFunction))