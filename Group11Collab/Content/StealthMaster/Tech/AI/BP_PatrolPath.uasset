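; BP_PatrolPath is an AI patrol path actor that supplies route data and tracks whether an AI has claimed it.
; Interface calls expose its path points, loop flag, wait time and occupied state, and return the actor itself as the path.
; Occupy and unoccupy events set or clear the assigned actor and occupied flag.
; The remaining getters, such as range, stunned and cover search, return empty defaults.
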(event EventIUnOccupyPatrolPoint
  (Variables|Default|SetAssignedActorRef 0)
  (Variables|Default|SetOccupied false))

(event EventIOccupyPatrolPoint
  (params (Occupying%20Actor :type Actor%20Object%20Reference))
  (Variables|Default|SetAssignedActorRef Occupying%20Actor)
  (Variables|Default|SetOccupied true))

(fn ConstructionScript)

(fn IGetActor
  (return 0))

(fn IGetController
  (return 0))

(fn IGetLookforCover
  (return false))

(fn IGetOccupied
  (return (Variables|Default|GetOccupied)))

(fn IGetPatrol?
  (return false))

(fn IGetPatrolLoop?
  (return (Variables|Default|GetLoop?)))

(fn IGetPatrolPathActor
  (return self))

(fn IGetPatrolPathPoints
  (return (Variables|Default|GetPathPoints)))

(fn IGetRange
  (return 0.0))

(fn IGetStunned?
  (return false))

(fn IGetWaitTime
  (return (Variables|Default|GetWaitTime)))