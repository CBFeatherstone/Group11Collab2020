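; Stealth security camera that sweeps between two points and flags when it spots the player.
; Two chained timelines loop, easing the camera's rotation toward billboard markers offset by Point1 and Point2 at setup.
; Each tick, a debug-drawn forward sphere trace for pawns resolves the hit actor through an interface and compares it to the cached player, updating PlayerDetection.
; Player-tracking and reset logic exists but is disconnected.
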(event EventBeginPlay
  (bind _camera (Variables|Default|GetCamera))
  (bind _billboard (Variables|Default|GetBillboard))
  (bind _camera_2 (Variables|Default|GetCamera))
  (bind _camera_3 (Variables|Default|GetCamera))
  (bind _returnvalue (Transformation|GetWorldLocation _camera))
  (bind _returnvalue_2 (Transformation|GetWorldLocation _billboard))
  (bind _returnvalue_3 (Transformation|GetWorldRotation _camera_2))
  (bind _returnvalue_4 (Math|Rotator|FindLookatRotation _returnvalue _returnvalue_2))
  (CallFunction|FSetup)
  (Transformation|SetWorldRotation (Variables|Default|GetCamera) _returnvalue_4 false false)
  (bind _alpha (Timeline|Lerp1 PlayFromStart)
    (:Update
      (Transformation|SetWorldRotation _camera_3 (Math|Interpolation|Ease "EaseInOut" _alpha _returnvalue_3 _returnvalue_4 true) false false))
    (:Finished
      (bind _alpha_2 (Timeline|Lerp2 PlayFromStart)
        (:Update
          (Transformation|SetWorldRotation _camera_3 (Math|Interpolation|Ease "EaseInOut" _alpha_2 _returnvalue_3 (Math|Rotator|FindLookatRotation _returnvalue (Transformation|GetWorldLocation (Variables|Default|GetBillboard1))) true) false false))
        (:Finished
          (Timeline|Lerp1 PlayFromStart))))))

(event EventTick
  (params (DeltaSeconds :type Float%20%28single-precision%29))
  (CallFunction|FTrace))

(fn ConstructionScript)

(fn FTrace
  (bind _camera (Variables|Default|GetCamera))
  (bind _returnvalue (Transformation|GetWorldLocation _camera))
  (bind (_outhit _returnvalue_2) (Collision|SphereTraceForObjects _returnvalue (+ _returnvalue (* (Math|Vector|GetForwardVector (Variables|Default|GetCamera)) 1e+04)) 1.5e+02 (Utilities|Array|MakeArray "ObjectTypeQuery3") false 0 "ForDuration"))
  (if _returnvalue_2
    (bind _output (Class|IAI|IGetActor(Message) (.HitActor (Collision|BreakHitResult _outhit))))
    (if (== _output (Variables|Default|GetPlayerRef))
      (Variables|Default|SetplayerDetection true))
    (else
      (Variables|Default|SetplayerDetection false))))

(fn FSetup
  (bind _output (Class|IAI|IGetActor(Message) (Pawn|GetControlledPawn (Game|GetPlayerController 0))))
  (Variables|Default|SetPlayerRef _output)
  (Transformation|AddLocalOffset (Variables|Default|GetBillboard) (Variables|Default|GetPoint1) false false)
  (Transformation|AddLocalOffset (Variables|Default|GetBillboard1) (Variables|Default|GetPoint2) false false))