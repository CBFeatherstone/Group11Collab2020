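; Test AI enemy character whose Class enum sets engagement range and selects a melee, explosion or ground-traced area attack.
; AI interface passthroughs trigger attacks and walk/run speeds, while getters expose patrol, range, cover and stun state.
; Damage reports to AI perception, updates a player-facing health bar, flags cover below half health, and on death frees the patrol path and notifies the GameMode.
; The automatic cooldown attack loop is disconnected.
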(event OnComponentBeginOverlap(AttackRange)
  (params (OverlappedComponent :type Primitive%20Component%20Object%20Reference) (OtherActor :type Actor%20Object%20Reference) (OtherComp :type Primitive%20Component%20Object%20Reference) (OtherBodyIndex :type Integer) (bFromSweep :type Boolean) (SweepResult :type Hit%20Result%20Structure%20%28by%20ref%29))
  (Utilities|IsValid OtherActor
    (:Is%20Valid
      (if (not (== OtherActor self))
        (Variables|Default|SetOtherActor OtherActor)))))

(event OnComponentEndOverlap(AttackRange)
  (params (OverlappedComponent :type Primitive%20Component%20Object%20Reference) (OtherActor :type Actor%20Object%20Reference) (OtherComp :type Primitive%20Component%20Object%20Reference) (OtherBodyIndex :type Integer))
  (Variables|Default|SetCanAttack false))

(event Custom|Attack
  (switch Utilities|FlowControl|Switch|SwitchonAttackClass_SM (Variables|Default|GetClass)
    (:NewEnumerator0
      (CallFunction|MeleeAttack)
      (Development|PrintString "Melee"))
    (:NewEnumerator1
      (CallFunction|RangedAttack)
      (Development|PrintString "Ranged"))
    (:NewEnumerator2
      (CallFunction|Ability)
      (Development|PrintString "Boss"))))

(event Custom|Enemy_Unstun
  (Input|EnableInput 0)
  (Variables|Default|SetStunned false))

(event Custom|EnemyStunned
  (Utilities|FlowControl|Delay (Variables|Default|GetStunDuration))
  (CallFunction|EnemyUnstun))

(event Custom|RemoveOrb
  (Utilities|FlowControl|Delay 4.0)
  (ChildActorComponent|SetChildActorClass (Variables|Default|GetChildActor) 0))

(event EventTick
  (params (DeltaSeconds :type Float%20%28single-precision%29))
  (CallFunction|RotateHealthBartoPlayer) ; Only turns when health bar isn't facing the player
)

(event EventBeginPlay
  (CallFunction|UpdateHealthBar))

(event Game|Damage|EventAnyDamage
  (params (Damage :type Float%20%28single-precision%29) (DamageType :type Damage%20Type%20Object%20Reference) (InstigatedBy :type Controller%20Object%20Reference) (DamageCauser :type Actor%20Object%20Reference))
  (CallFunction|TakeDamage Damage)
  (Class|AISenseDamage|ReportDamageEvent self InstigatedBy Damage (Transformation|GetActorLocation InstigatedBy)))

(event EventIAIRunPassthrough
  (Variables|/Script/Engine.CharacterMovementComponent|SetMaxWalkSpeed (Variables|Character|GetCharacterMovement) (Variables|Default|GetRunSpeed)))

(event EventIAIWalkPassthrough
  (Variables|/Script/Engine.CharacterMovementComponent|SetMaxWalkSpeed (Variables|Character|GetCharacterMovement) (Variables|Default|GetWalkSpeed)))

(event EventIAIAttackPassthrough
  (CallFunction|Attack))

(fn ConstructionScript
  (switch Utilities|FlowControl|Switch|SwitchonAttackClass_SM (Variables|Default|GetClass)
    (:NewEnumerator0
      (Variables|Default|SetRange 5e+01))
    (:NewEnumerator1
      (Variables|Default|SetRange 5e+02))
    (:NewEnumerator2
      (Variables|Default|SetRange 1e+03))
    (:NewEnumerator3
      (Variables|Default|SetRange 5e+01))))

(fn MeleeAttack
  (Game|Damage|ApplyDamage (Variables|Default|GetOtherActor) (Variables|Default|GetAttackDamage) 0 self))

(fn Death
  (Class|IAI|IUnOccupyPatrolPoint(Message) (Variables|Default|GetPatrolPath))
  (Class|IAI|IAIDeathPassthrough(Message) (Game|GetGameMode) self)
  (Actor|DestroyActor))

(fn TakeDamage
  (params (DamageTaken :type Float%20%28single-precision%29))
  (bind _output_get (Variables|Default|SetHealth (- (Variables|Default|GetHealth) DamageTaken)))
  (CallFunction|UpdateHealthBar)
  (if (<= _output_get 0.0)
    (CallFunction|Death)
    (elif (< (/ (Variables|Default|GetHealth) (Variables|Default|GetMaxHealth)) 0.5)
      (Variables|Default|SetlookForCover true)
      (else
        (Variables|Default|SetlookForCover false)))))

(fn RangedAttack
  (bind _rangedarrow (Variables|Default|GetRangedArrow))
  (bind _returnvalue (Transformation|GetWorldTransform _rangedarrow))
  (Game|SpawnActorfromClass "/Game/StealthMaster/Tech/Enemies/Explosion.Explosion_C" (Math|Transform|MakeTransform (+ (.location _returnvalue) (* (Math|Vector|GetForwardVector _rangedarrow) 1e+02)) (.rotation _returnvalue) "1,1,1") "AlwaysSpawn" 0 0)
  (return false))

(fn Ability
  (bind _rangedarrow (Variables|Default|GetRangedArrow))
  (bind _returnvalue (Math|Vector|GetForwardVector _rangedarrow))
  (bind _returnvalue_2 (Transformation|GetWorldTransform _rangedarrow))
  (bind _returnvalue_3 (* _returnvalue 5e+02))
  (bind _returnvalue_4 (+ _returnvalue_3 (.location _returnvalue_2)))
  (bind _outhit (Collision|LineTraceByChannel _returnvalue_4 (+ _returnvalue_4 (* (Math|Vector|GetUpVector _rangedarrow) -1e+03)) "TraceTypeQuery1" false 0 "ForDuration"))
  (Game|SpawnActorfromClass "/Game/Prototype/Korruption/Tech/Enemies/AreaOfEffect.AreaOfEffect_C" (Math|Transform|MakeTransform (+ (.impactpoint _outhit) "0, 0,6.000000") "0, 0, 0" "1,1,1") "Undefined" 0 0))

(fn 3rdRangedAttack
  (ChildActorComponent|SetChildActorClass (Variables|Default|GetChildActor) "/Game/StealthMaster/Tech/Enemies/RotatingOrb.RotatingOrb_C")
  (CallFunction|RemoveOrb))

(fn StunEnemy
  (params (Stun :type Integer))
  (if (<= (Math|Random|RandomIntegerinRange 0 (Variables|Default|GetStunResistance)) Stun)
    (CallFunction|TakeDamage (Variables|Default|GetStunDamage))
    (Variables|Default|SetStunned true)
    (Input|DisableInput 0)
    (CallFunction|EnemyStunned)))

(fn UpdateHealthBar
  (bind _asenemy_health_bar (Utilities|Casting|CastToEnemyHealthBar (UserInterface|GetUserWidgetObject (Variables|Default|GetHealthBar))))
  (Variables|/Game/StealthMaster/Tech/Enemies/EnemyHealthBar.EnemyHealthBar_C|SetHealth _asenemy_health_bar (/ (Variables|Default|GetHealth) (Variables|Default|GetMaxHealth))))

(fn GetRotationtoPlayer
  (bind _returnvalue (Game|GetPlayerController 0))
  (bind _returnvalue_2 (Pawn|GetControlledPawn _returnvalue))
  (Utilities|IsValid _returnvalue
    (:Is%20Valid
      (Utilities|IsValid _returnvalue_2
        (:Is%20Valid
          (return (Math|Rotator|MakeRotator 0.0 0.0 (.yaw (Math|Conversions|RotationFromXVector (- (Transformation|GetActorLocation _returnvalue_2) (Transformation|GetWorldLocation (Variables|Default|GetHealthBar))))))))
        (:Is%20Not%20Valid
          _)))
    (:Is%20Not%20Valid
      _))
  (return "0, 0, 0"))

(fn RotateHealthBartoPlayer
  (if (Utilities|Enum|NotEqual(Enum) (Transformation|GetWorldRotation (Variables|Default|GetHealthBar)) (CallFunction|GetRotationtoPlayer) 1.0)
    (Transformation|SetWorldRotation (Variables|Default|GetHealthBar) (CallFunction|GetRotationtoPlayer) false false)))

(fn IGetActor
  (return self))

(fn IGetController
  (return 0))

(fn IGetLookforCover
  (return (Variables|Default|GetlookForCover)))

(fn IGetOccupied
  (return false))

(fn IGetPatrol?
  (return (Variables|Default|GetPatrol?)))

(fn IGetPatrolLoop?
  (return (Variables|Default|GetPatrolLoop)))

(fn IGetPatrolPathActor
  (return (Variables|Default|GetPatrolPath)))

(fn IGetPatrolPathPoints
  (return 0))

(fn IGetRange
  (return (Variables|Default|GetRange)))

(fn IGetStunned?
  (return (Variables|Default|GetStunned)))

(fn IGetWaitTime
  (return 0.0))