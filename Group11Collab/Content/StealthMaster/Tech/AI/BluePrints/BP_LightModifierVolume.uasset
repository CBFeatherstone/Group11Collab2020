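; BP_LightModifierVolume is a box volume that modifies light values, apparently for the stealth visibility system.
; Begin overlap broadcasts the UpdateLightValuesVolume dispatcher with itself and its LightValue, and end overlap broadcasts zero, with no filter on the overlapping actor.
; The construction script sizes the box from BoxSize.
; The many interface getters are stubs that return empty or fixed values.
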(event OnComponentBeginOverlap(Box)
  (params (OverlappedComponent :type Primitive%20Component%20Object%20Reference) (OtherActor :type Actor%20Object%20Reference) (OtherComp :type Primitive%20Component%20Object%20Reference) (OtherBodyIndex :type Integer) (bFromSweep :type Boolean) (SweepResult :type Hit%20Result%20Structure%20%28by%20ref%29))
  (Default|CallDUpdateLightValuesVolume self (Variables|Default|GetlightValue)))

(event OnComponentEndOverlap(Box)
  (params (OverlappedComponent :type Primitive%20Component%20Object%20Reference) (OtherActor :type Actor%20Object%20Reference) (OtherComp :type Primitive%20Component%20Object%20Reference) (OtherBodyIndex :type Integer))
  (Default|CallDUpdateLightValuesVolume self 0.0))

(fn ConstructionScript
  (Components|Box|SetBoxExtent (Variables|Default|GetBox) (Variables|Default|GetboxSize) true))

(fn IGetActive
  (return false))

(fn IGetActor
  (return 0))

(fn IGetCameraObject
  (return 0))

(fn IGetCanTakeDamage
  (return false))

(fn IGetCodeLockNumber
  (return ""))

(fn IGetCollected
  (return false))

(fn IGetController
  (return 0))

(fn IGetCurrentPhase
  (return 0))

(fn IGetElevatorLevel
  (return 0))

(fn IGetEnemyCurr/Max
  (return 0 0))

(fn IGetFinalePhase
  (return false))

(fn IGetGenericController
  (return 0))

(fn IGetIsDrone
  (return false))

(fn IGetIsEnemy
  (return false))

(fn IGetLookforCover
  (return false))

(fn IGetObjectType
  (return "NewEnumerator3"))

(fn IGetOccupied
  (return false))

(fn IGetOverlappingActors
  (return 0))

(fn IGetPatrol?
  (return false))

(fn IGetPatrolLoop?
  (return false))

(fn IGetPatrolPathActor
  (return 0))

(fn IGetPatrolPathPoints
  (return 0))

(fn IGetPawnReference
  (return 0))

(fn IGetPlayerSector
  (return 0))

(fn IGetPlaystyle
  (return "NewEnumerator0"))

(fn IGetRange
  (return 0.0))

(fn IGetSceneComponentHumanoid
  (return 0))

(fn IGetScore
  (return 0.0))

(fn IGetSector
  (params (Input :type Integer))
  (return 0))

(fn IGetSectorIndex
  (return 0))

(fn IGetSectorSize
  (return "0, 0, 0"))

(fn IGetStance
  (return "NewEnumerator0"))

(fn IGetStunned?
  (return false))

(fn IGetVisibilityGM
  (return 0.0 false false false))

(fn IGetVisibilitySL
  (return 0.0))

(fn IGetWaitTime
  (return 0.0))

(fn IReturnDetectedVariables
  (return 0.0 0.0))

(fn ISectorGetContainedEnemies
  (return 0))