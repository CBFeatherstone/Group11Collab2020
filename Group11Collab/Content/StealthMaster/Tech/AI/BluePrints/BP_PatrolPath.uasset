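; BP_PatrolPath is a patrol route actor for Stealth Master's AI, exposing its path points, loop flag and wait time through interface getters.
; Occupy and unoccupy interface events record or clear the assigned actor and toggle an occupied flag that can be queried.
; The other interface functions return fixed or empty defaults, apart from the object type, which reports a set enum value.
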(event EventIUnOccupyPatrolPoint
  (Variables|Default|SetAssignedActorRef 0)
  (Variables|Default|SetOccupied false))

(event EventIOccupyPatrolPoint
  (params (Occupying%20Actor :type Actor%20Object%20Reference))
  (Variables|Default|SetAssignedActorRef Occupying%20Actor)
  (Variables|Default|SetOccupied true))

(fn ConstructionScript)

(fn IGetActor
  (return 0))

(fn IGetCameraObject
  (return 0))

(fn IGetController
  (return 0))

(fn IGetEnemyCurr/Max
  (return 0 0))

(fn IGetIsDrone
  (return false))

(fn IGetLookforCover
  (return false))

(fn IGetObjectType
  (return "NewEnumerator3"))

(fn IGetOccupied
  (return (Variables|Default|GetOccupied)))

(fn IGetPatrol?
  (return false))

(fn IGetPatrolLoop?
  (return (Variables|Default|GetLoop?)))

(fn IGetPatrolPathActor
  (return self))

(fn IGetPatrolPathPoints
  (return (Variables|Default|GetPathPoints)))

(fn IGetPawnReference
  (return 0))

(fn IGetPlayerSector
  (return 0))

(fn IGetRange
  (return 0.0))

(fn IGetSector
  (params (Input :type Integer))
  (return 0))

(fn IGetSectorIndex
  (return 0))

(fn IGetSectorSize
  (return "0, 0, 0"))

(fn IGetStunned?
  (return false))

(fn IGetVisibilityGM
  (return 0.0 false false false))

(fn IGetWaitTime
  (return (Variables|Default|GetWaitTime)))