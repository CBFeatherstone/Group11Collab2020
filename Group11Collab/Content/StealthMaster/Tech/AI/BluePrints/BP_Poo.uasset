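; BP_Poo is a poo actor that snaps to the surface beneath its spawn point and grows into place.
; On BeginPlay it traces downward on the Camera channel and teleports to the impact point, destroying itself if nothing is hit.
; A timeline then scales up the static mesh, and the actor destroys itself a minute after the growth finishes.
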(event EventBeginPlay
  (bind _defaultsceneroot (Variables|Default|GetDefaultSceneRoot))
  (bind _returnvalue (Transformation|GetWorldLocation _defaultsceneroot))
  (bind (_outhit _returnvalue_2) (Collision|LineTraceByChannel _returnvalue (- _returnvalue "0, 0,1000.000000") "TraceTypeQuery2" false 0 "None"))
  (if _returnvalue_2
    (Transformation|SetWorldLocation (Variables|Default|GetDefaultSceneRoot) (.ImpactPoint (Collision|BreakHitResult _outhit)) false true)
    (bind _newtrack_0 (Timeline|Lerp Play)
      (:Update
        (Transformation|SetWorldScale3D (Variables|Default|GetStaticMesh) (Math|Vector|Lerp(Vector) "0.200000,0.200000,0.200000" "1.500000,1.500000,1.500000" _newtrack_0)))
      (:Finished
        (Utilities|FlowControl|Delay 6e+01)
        (Actor|DestroyActor)))
    (else
      (Actor|DestroyActor))))

(fn ConstructionScript)