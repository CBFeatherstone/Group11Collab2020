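; AI spawner actor that creates either a drone or an enemy character at its location, unless disabled.
; Each spawn gets its own BP_AIController, handed the pawn and sector, plus an optional patrol path that gets marked occupied.
; Non-drone spawns receive a weapon and a data table row, overridden for known alien classes.
; Interface messages link it to a sector, whose enable/disable events toggle IsActive, though spawning never checks that flag.
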(event Custom|SpawnAI
  (params (Sector :type Integer))
  (CallFunction|FSpawnAI Sector))

(event Custom|D_Disable
  (params (Sector%20Index :type Integer))
  (Variables|Default|SetisActive false))

(event Custom|D_Enable
  (params (Sector%20Index :type Integer))
  (Variables|Default|SetisActive true))

(event EventISetSpawnerSectorRef
  (params (Input :type Integer))
  (Variables|Default|SetsectorRef Input))

(event EventISectorPassThrough
  (params (Sector :type BP%20Sector%20Object%20Reference))
  (EventDispatchers|BindEventtoDEnableSector Sector (EventDispatchers|CreateEvent :!event Custom|D_Enable))
  (EventDispatchers|BindEventtoDDisableSector Sector (EventDispatchers|CreateEvent :!event Custom|D_Disable))
  (Variables|Default|SetsectorActorRef Sector))

(fn ConstructionScript)

(fn FSpawnAI
  (params (inputSecotrRef :type Integer))
  (bind _candamageaispawned_ (Variables|Default|GetcanDamageAISpawned?))
  (bind _weapononspawn (Variables|Default|GetweaponOnSpawn))
  (bind _candamageaispawned__2 (Variables|Default|GetcanDamageAISpawned?))
  (Variables|Default|SetinputSecotrRef inputSecotrRef)
  (if (not (Variables|Default|GetDisabled))
    (if (Variables|Default|GetdroneSpawner)
      (if (Utilities|IsValid (Variables|Default|GetpatrolPath))
        (bind _returnvalue (Game|SpawnActorfromClass (Variables|Default|GetDroneToSpawn) (Math|Transform|MakeTransform (Transformation|GetWorldLocation (Variables|Default|GetDefaultSceneRoot)) "0, 0, 0" "1,1,1") "AlwaysSpawn" 0 0))
        (Utilities|IsValid _returnvalue
          (:Is%20Valid
            (Class|IAI|ISetPatrolValues(Message) _returnvalue true (Variables|Default|GetpatrolPath))
            (bind _output (Class|IAI|IGetPawnReference(Message) _returnvalue))
            (bind _returnvalue_2 (Game|SpawnActorfromClass "/Game/StealthMaster/Tech/AI/BP_AIController.BP_AIController_C" (Math|Transform|MakeTransform "0, 0, 0" "0, 0, 0" "1,1,1") "AdjustIfPossibleButAlwaysSpawn" 0 (Variables|Default|GetpatrolPath) _output true true _candamageaispawned_ (Variables|Default|GetinputSecotrRef) 0))
            (Utilities|IsValid _returnvalue
              (:Is%20Valid
                (Class|IAI|IInitiate(Message) _returnvalue)
                (Class|IAI|IOccupyPatrolPoint(Message) (Variables|Default|GetpatrolPath) _returnvalue)
                (Class|IAI|ISectorPassThrough(Message) _returnvalue_2 (Variables|Default|GetsectorActorRef))))))
        (else
          (bind _returnvalue_3 (Game|SpawnActorfromClass (Variables|Default|GetDroneToSpawn) (Math|Transform|MakeTransform (Transformation|GetWorldLocation (Variables|Default|GetDefaultSceneRoot)) "0, 0, 0" "1,1,1") "AlwaysSpawn" 0 0))
          (Utilities|IsValid _returnvalue_3
            (:Is%20Valid
              (bind _output_2 (Class|IAI|IGetPawnReference(Message) _returnvalue_3))
              (bind _returnvalue_4 (Game|SpawnActorfromClass "/Game/StealthMaster/Tech/AI/BP_AIController.BP_AIController_C" (Math|Transform|MakeTransform "0, 0, 0" "0, 0, 0" "1,1,1") "AdjustIfPossibleButAlwaysSpawn" 0 0 _output_2 false true _candamageaispawned_ (Variables|Default|GetinputSecotrRef) 0))
              (Utilities|IsValid _returnvalue_3
                (:Is%20Valid
                  (Class|IAI|IInitiate(Message) _returnvalue_3)
                  (Class|IAI|ISectorPassThrough(Message) _returnvalue_4 (Variables|Default|GetsectorActorRef))))))))
      (else
        (CallFunction|FCheckActortoSpawn)
        (if (Utilities|IsValid (Variables|Default|GetpatrolPath))
          (bind _returnvalue_5 (Game|SpawnActorfromClass (Variables|Default|GetActorToSpawn) (Math|Transform|MakeTransform (Transformation|GetWorldLocation (Variables|Default|GetDefaultSceneRoot)) "0, 0, 0" "1,1,1") "AlwaysSpawn" 0 (Variables|Default|GetdataTableRowName) _weapononspawn true (Variables|Default|GetpatrolPath) 0))
          (Utilities|IsValid _returnvalue_5
            (:Is%20Valid
              (bind _output_3 (Class|IAI|IGetPawnReference(Message) _returnvalue_5))
              (bind _returnvalue_6 (Game|SpawnActorfromClass "/Game/StealthMaster/Tech/AI/BP_AIController.BP_AIController_C" (Math|Transform|MakeTransform "0, 0, 0" "0, 0, 0" "1,1,1") "AdjustIfPossibleButAlwaysSpawn" 0 (Variables|Default|GetpatrolPath) _output_3 true false _candamageaispawned__2 (Variables|Default|GetinputSecotrRef) 0))
              (Utilities|IsValid _returnvalue_5
                (:Is%20Valid
                  (Class|IAI|IInitiate(Message) _returnvalue_5)
                  (Class|IAI|IOccupyPatrolPoint(Message) (Variables|Default|GetpatrolPath) _returnvalue_5)
                  (Class|IAI|ISectorPassThrough(Message) _returnvalue_6 (Variables|Default|GetsectorActorRef))))))
          (else
            (bind _returnvalue_7 (Game|SpawnActorfromClass (Variables|Default|GetActorToSpawn) (Math|Transform|MakeTransform (Transformation|GetWorldLocation (Variables|Default|GetDefaultSceneRoot)) "0, 0, 0" "1,1,1") "AlwaysSpawn" 0 (Variables|Default|GetdataTableRowName) _weapononspawn false 0 0))
            (Utilities|IsValid _returnvalue_7
              (:Is%20Valid
                (bind _output_4 (Class|IAI|IGetPawnReference(Message) _returnvalue_7))
                (bind _returnvalue_8 (Game|SpawnActorfromClass "/Game/StealthMaster/Tech/AI/BP_AIController.BP_AIController_C" (Math|Transform|MakeTransform "0, 0, 0" "0, 0, 0" "1,1,1") "AdjustIfPossibleButAlwaysSpawn" 0 0 _output_4 false false _candamageaispawned__2 (Variables|Default|GetinputSecotrRef) 0))
                (Utilities|IsValid _returnvalue_7
                  (:Is%20Valid
                    (Class|IAI|IInitiate(Message) _returnvalue_7)
                    (Class|IAI|ISectorPassThrough(Message) _returnvalue_8 (Variables|Default|GetsectorActorRef))))))))))))

(fn FCheckActortoSpawn
  (bind _actortospawn (Variables|Default|GetActorToSpawn))
  (if (== _actortospawn "/Game/StealthMaster/Tech/Enemies/Enemy_BaseRangedCharacter_Class.Enemy_BaseRangedCharacter_Class_C")
    (Variables|Default|SetdataTableRowName "BigAlien")
    (elif (== _actortospawn "/Game/StealthMaster/Tech/Enemies/Enemy_Alien_Class.Enemy_Alien_Class_C")
      (Variables|Default|SetdataTableRowName "SmallAlien"))))

(fn IGetActive
  (return false))

(fn IGetActor
  (return 0))

(fn IGetCameraObject
  (return 0))

(fn IGetCanTakeDamage
  (return false))

(fn IGetCodeLockNumber
  (return ""))

(fn IGetCollected
  (return false))

(fn IGetController
  (return 0))

(fn IGetCurrentPhase
  (return 0))

(fn IGetElevatorLevel
  (return 0))

(fn IGetEnemyCurr/Max
  (return 0 0))

(fn IGetFinalePhase
  (return false))

(fn IGetGenericController
  (return 0))

(fn IGetIsDrone
  (return false))

(fn IGetIsEnemy
  (return false))

(fn IGetLookforCover
  (return false))

(fn IGetObjectType
  (return (Variables|Default|GetType)))

(fn IGetOccupied
  (bind _output (Class|IAI|IGetOccupied(Message) (Variables|Default|GetpatrolPath)))
  (return _output))

(fn IGetOverlappingActors
  (return 0))

(fn IGetPatrol?
  (return false))

(fn IGetPatrolLoop?
  (return false))

(fn IGetPatrolPathActor
  (return (Variables|Default|GetpatrolPath)))

(fn IGetPatrolPathPoints
  (return 0))

(fn IGetPawnReference
  (return 0))

(fn IGetPlayerSector
  (return 0))

(fn IGetPlaystyle
  (return "NewEnumerator0"))

(fn IGetRange
  (return 0.0))

(fn IGetSceneComponentHumanoid
  (return 0))

(fn IGetScore
  (return 0.0))

(fn IGetSector
  (params (Input :type Integer))
  (return 0))

(fn IGetSectorIndex
  (return 0))

(fn IGetSectorSize
  (return "0, 0, 0"))

(fn IGetStance
  (return "NewEnumerator0"))

(fn IGetStunned?
  (return false))

(fn IGetVisibilityGM
  (return 0.0 false false false))

(fn IGetVisibilitySL
  (return 0.0))

(fn IGetWaitTime
  (return 0.0))

(fn IReturnDetectedVariables
  (return 0.0 0.0))

(fn ISectorGetContainedEnemies
  (return 0))