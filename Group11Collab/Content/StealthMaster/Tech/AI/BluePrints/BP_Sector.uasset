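; BP_Sector is a box volume for a stealth level sector that manages its AI spawners, cameras, lights and enemies.
; On BeginPlay it registers overlapping assets, spawns AI and subscribes to game mode sector toggles, with respawns favouring unoccupied patrol spawners.
; Overlaps report the player's sector and track enemies, while a sector check broadcasts enable or disable.
; Spotlight dispatchers feed a map that is summed into clamped visibility.
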(event OnComponentBeginOverlap(Box)
  (params (OverlappedComponent :type Primitive%20Component%20Object%20Reference) (OtherActor :type Actor%20Object%20Reference) (OtherComp :type Primitive%20Component%20Object%20Reference) (OtherBodyIndex :type Integer) (bFromSweep :type Boolean) (SweepResult :type Hit%20Result%20Structure%20%28by%20ref%29))
  (Utilities|IsValid OtherActor
    (:Is%20Valid
      (Utilities|FlowControl|Sequence
        (:then_0
          (bind _output (Class|IAI|IGetActor(Message) OtherActor))
          (if (== _output (Pawn|GetControlledPawn (Game|GetPlayerController 0)))
            (Class|IAI|IUpdatePlayerSector(Message) (Game|GetGameMode) (Variables|Default|GetsectorIndex))))
        (:then_1
          (bind _output_2 (Class|IAI|IGetIsEnemy(Message) OtherActor))
          (if _output_2
            (Utilities|Array|AddUnique (Variables|Default|GetenemiesInSector) OtherActor)))))))

(event OnComponentEndOverlap(Box)
  (params (OverlappedComponent :type Primitive%20Component%20Object%20Reference) (OtherActor :type Actor%20Object%20Reference) (OtherComp :type Primitive%20Component%20Object%20Reference) (OtherBodyIndex :type Integer))
  (Utilities|IsValid OtherActor
    (:Is%20Valid
      (bind _output (Class|IAI|IGetIsEnemy(Message) OtherActor))
      (if _output
        (Utilities|Array|RemoveItem (Variables|Default|GetenemiesInSector) OtherActor)))))

(event EventBeginPlay
  (CallFunction|FSetupContainedAssets)
  (CallFunction|FInitialAISpawn)
  (CallFunction|FSubscribetoGameMode)
  (Utilities|FlowControl|Delay 0.2)
  (CallFunction|FSetupEnemiesContained)
  (CallFunction|FSetupLights))

(event EventIRespawnAI
  (params (SectorIndex :type Integer) (EnemiesNeeded :type Integer))
  (for _index (range 1 EnemiesNeeded)
    (CallFunction|FSpawnAIRecur)))

(fn ConstructionScript
  (Components|Box|SetBoxExtent (Variables|Default|GetBox) (Variables|Default|GetboxSize%20) true))

(fn FSetupContainedAssets
  (bind _box (Variables|Default|GetBox))
  (bind _overlappingactors (Collision|GetOverlappingActors _box 0 :!class /Script/Engine.PrimitiveComponent))
  (if (> (Utilities|Array|Length _overlappingactors) 0)
    (for _array_element _overlappingactors
      (bind _output (Class|IAI|IGetObjectType(Message) _array_element))
      (switch Utilities|FlowControl|Switch|SwitchonE_ObjectType _output
        (:NewEnumerator0
          (Utilities|Array|Add (Variables|Default|GetlightsRef) _array_element))
        (:NewEnumerator1
          (bind _asbp_aispawner (Utilities|Casting|CastToBP_AISPawner _array_element))
          (Utilities|Array|Add (Variables|Default|GetaiSpawnersRef) _asbp_aispawner))
        (:NewEnumerator2
          (Utilities|Array|Add (Variables|Default|GetcamerasRef) _array_element)
          (Class|IAI|ISetSpawnerSectorRef(Message) _array_element (Variables|Default|GetsectorIndex))))
      (Class|IAI|ISectorPassThrough(Message) _array_element self))
    (else
      (Development|PrintString "NoObjectsInSector"))))

(fn FDEBUGPrintAssets
  (for _array_element (Variables|Default|GetcamerasRef)
    (Development|PrintString (Utilities|String|Append (Utilities|String|ToString(Integer) (Variables|Default|GetsectorIndex)) ": " (Utilities|GetDisplayName _array_element))))
  (for _array_element_2 (Variables|Default|GetlightsRef)
    (Development|PrintString (Utilities|String|Append (Utilities|String|ToString(Integer) (Variables|Default|GetsectorIndex)) ": " (Utilities|GetDisplayName _array_element_2))))
  (for _array_element_3 (Variables|Default|GetaiSpawnersRef)
    (Development|PrintString (Utilities|String|Append (Utilities|String|ToString(Integer) (Variables|Default|GetsectorIndex)) ": " (Utilities|GetDisplayName _array_element_3)))))

(fn FInitialAISpawn
  (for _array_element (Variables|Default|GetaiSpawnersRef)
    (Default|SpawnAI _array_element (Variables|Default|GetsectorIndex))
    (bind _output (Class|IAI|IGetPatrolPathActor(Message) _array_element))
    (Utilities|IsValid _output
      (:Is%20Valid
        (Utilities|Array|Add (Variables|Default|GetPatrolSpawners) _array_element))
      (:Is%20Not%20Valid
        (Utilities|Array|Add (Variables|Default|GetNonPatrolSpawners) _array_element)))))

(fn FSpawnAIRecur
  (bind _nonpatrolspawners (Variables|Default|GetNonPatrolSpawners))
  (bind _returnvalue (Utilities|Array|Length _nonpatrolspawners))
  (bind _returnvalue_2 (Math|Random|RandomInteger _returnvalue))
  (bind _output (Utilities|Array|Get(acopy) _nonpatrolspawners _returnvalue_2))
  (LocalVariables|SetSpawned false)
  (bind _array_element (Utilities|Array|ForEachLoopwithBreak (Variables|Default|GetPatrolSpawners) :!label _label)
    (:LoopBody
      (bind _output_2 (Class|IAI|IGetOccupied(Message) _array_element))
      (if (not _output_2)
        (Default|SpawnAI _array_element (Variables|Default|GetsectorIndex))
        (LocalVariables|SetSpawned true)
        (goto _label Break)))
    (:Completed
      (if (not (LocalVariables|GetSpawned))
        (Utilities|IsValid _output
          (:Is%20Valid
            (Default|SpawnAI _output (Variables|Default|GetsectorIndex))))))))

(fn FSubscribetoGameMode
  (bind _asbp_stealth_master_gm (Utilities|Casting|CastToBP_StealthMaster_GM (Game|GetGameMode)))
  (EventDispatchers|BindEventtoDToggleAISectors _asbp_stealth_master_gm (EventDispatchers|CreateEvent :!event FCheckSector)))

(fn FCheckSector
  (bind _sectorindex (Variables|Default|GetsectorIndex))
  (bind _output (Class|IAI|IGetPlayerSector(Message) (Game|GetGameMode)))
  (if (== (Variables|Default|GetsectorIndex) _output)
    (Default|CallDEnableSector _sectorindex)
    (else
      (Default|CallDDisableSector _sectorindex))))

(fn FSetupEnemiesContained
  (for _array_element (Collision|GetOverlappingActors 0 :!class /Script/Engine.Actor)
    (bind _output (Class|IAI|IGetIsEnemy(Message) _array_element))
    (if _output
      (Utilities|Array|AddUnique (Variables|Default|GetenemiesInSector) _array_element))))

(fn FSetupLights
  (for _array_element (Collision|GetOverlappingActors (Variables|Default|GetBox) "/Game/StealthMaster/Tech/AI/BluePrints/BP_Spotlight.BP_Spotlight_C" :!class /Script/Engine.PrimitiveComponent)
    (bind _asbp_spotlight (Utilities|Casting|CastToBP_Spotlight _array_element))
    (Utilities|Map|Add (Variables|Default|GetlightsEffectMap) _asbp_spotlight 0.0)
    (EventDispatchers|BindEventtoDUpdateLightValues _asbp_spotlight (EventDispatchers|CreateEvent :!event FUpdateLightMap))))

(fn FUpdateLightMap
  (params (Light :type BP%20Spotlight%20Object%20Reference) (Input :type Float%20%28single-precision%29))
  (Utilities|Map|Add (Variables|Default|GetlightsEffectMap) Light Input))

(fn IGetActive
  (return false))

(fn IGetActor
  (return 0))

(fn IGetCameraObject
  (return 0))

(fn IGetCodeLockNumber
  (return ""))

(fn IGetController
  (return 0))

(fn IGetElevatorLevel
  (return 0))

(fn IGetEnemyCurr/Max
  (return (+ (Utilities|Array|Length (Collision|GetOverlappingActors "/Game/StealthMaster/Tech/Enemies/Enemy_BaseCharacter_Class.Enemy_BaseCharacter_Class_C" :!class /Script/Engine.Actor)) (Utilities|Array|Length (Collision|GetOverlappingActors "/Game/StealthMaster/Tech/Enemies/New_Enemy_Drone_Class.New_Enemy_Drone_Class_C" :!class /Script/Engine.Actor))) (Variables|Default|GetmaxEnemyNumber)))

(fn IGetIsDrone
  (return false))

(fn IGetIsEnemy
  (return false))

(fn IGetLookforCover
  (return false))

(fn IGetObjectType
  (return "NewEnumerator3"))

(fn IGetOccupied
  (return false))

(fn IGetOverlappingActors
  (return 0))

(fn IGetPatrol?
  (return false))

(fn IGetPatrolLoop?
  (return false))

(fn IGetPatrolPathActor
  (return 0))

(fn IGetPatrolPathPoints
  (return 0))

(fn IGetPawnReference
  (return 0))

(fn IGetPlayerSector
  (return 0))

(fn IGetPlaystyle
  (return "NewEnumerator0"))

(fn IGetRange
  (return 0.0))

(fn IGetSector
  (params (Input :type Integer))
  (return 0))

(fn IGetSectorIndex
  (return (Variables|Default|GetsectorIndex)))

(fn IGetSectorSize
  (return (Variables|Default|GetboxSize%20)))

(fn IGetStance
  (return "NewEnumerator0"))

(fn IGetStunned?
  (return false))

(fn IGetVisibilityGM
  (return 0.0 false false false))

(fn IGetVisibilitySL
  (bind _values (Utilities|Map|Values (Variables|Default|GetlightsEffectMap)))
  (for _array_element _values
    (LocalVariables|SetcumulativeVisibility (Math|Float|Clamp(Float) (+ _array_element (LocalVariables|GetcumulativeVisibility)) 0.0 1e+02)))
  (return (LocalVariables|GetcumulativeVisibility)))

(fn IGetWaitTime
  (return 0.0))

(fn IReturnDetectedVariables
  (return 0.0 0.0))

(fn ISectorGetContainedEnemies
  (return (Variables|Default|GetenemiesInSector)))