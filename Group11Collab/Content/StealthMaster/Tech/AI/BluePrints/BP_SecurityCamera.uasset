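; Stealth security camera that sweeps between two billboard points and alerts AI on spotting the player.
; Two chained timelines swing camera and turret back and forth while its sector is active; sector dispatchers toggle scanning and status material.
; Each active tick sphere-traces forward, then line-traces five upper-body sockets, alerting once the never-reset clear-trace count exceeds three.
; Any damage explodes and permanently disables it.
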(event Custom|STOP
  (bind _originalcamerarotation (Variables|Default|GetoriginalCameraRotation))
  (bind _cameraturret (Variables|Default|GetCameraTurret))
  (bind _cameraturret_2 (Variables|Default|GetCameraTurret))
  (bind _camera (Variables|Default|GetCamera))
  (bind _returnvalue (Transformation|GetWorldLocation _cameraturret_2))
  ;[1 1 1] Camera Rotation / Setup
  (Utilities|FlowControl|Sequence
    (:then_0
      (bind _alpha (Timeline|Lerp1 Stop)
        (:Update
          (Transformation|SetWorldRotation _camera (Math|Interpolation|RInterpTo _originalcamerarotation (Math|Rotator|FindLookatRotation _returnvalue (Transformation|GetWorldLocation (Variables|Default|GetBillboard))) _alpha 1.0) false false)
          (Transformation|SetWorldRotation _cameraturret (Math|Rotator|MakeRotator 0.0 0.0 (.yaw (Math|Rotator|CombineRotators (Math|Rotator|MakeRotator 0.0 0.0 -9e+01) (Math|Rotator|MakeRotator 0.0 0.0 (.Yaw (Math|Rotator|BreakRotator (Math|Interpolation|RInterpTo _originalcamerarotation (Math|Rotator|FindLookatRotation _returnvalue (Transformation|GetWorldLocation (Variables|Default|GetBillboard))) _alpha 1.0))))))) false false))
        (:Finished
          (CallFunction|FUpdateRotation)
          (bind _alpha_2 (Timeline|Lerp2 PlayFromStart)
            (:Update
              (Transformation|SetWorldRotation _camera (Math|Interpolation|RInterpTo _originalcamerarotation (Math|Rotator|FindLookatRotation _returnvalue (Transformation|GetWorldLocation (Variables|Default|GetBillboard1))) _alpha_2 1.0) false false)
              (Transformation|SetWorldRotation _cameraturret (Math|Rotator|MakeRotator 0.0 0.0 (.yaw (Math|Rotator|CombineRotators (Math|Rotator|MakeRotator 0.0 0.0 -9e+01) (Math|Rotator|MakeRotator 0.0 0.0 (.Yaw (Math|Rotator|BreakRotator (Math|Interpolation|RInterpTo _originalcamerarotation (Math|Rotator|FindLookatRotation _returnvalue (Transformation|GetWorldLocation (Variables|Default|GetBillboard1))) _alpha_2 1.0))))))) false false))
            (:Finished
              (CallFunction|FUpdateRotation)
              (Timeline|Lerp1 PlayFromStart))))))
    (:then_1
      (Timeline|Lerp2 Stop))))

(event Custom|D_Disable
  (params (Sector%20Index :type Integer))
  (bind _originalcamerarotation (Variables|Default|GetoriginalCameraRotation))
  (bind _cameraturret (Variables|Default|GetCameraTurret))
  (bind _cameraturret_2 (Variables|Default|GetCameraTurret))
  (bind _camera (Variables|Default|GetCamera))
  (bind _returnvalue (Transformation|GetWorldLocation _cameraturret_2))
  ;[1 1 1] Camera Rotation / Setup
  ;;[1 1 1] Dispatcher Functions
  (if (not (Variables|Default|Getdestroyed))
    (Variables|Default|SetisActive false)
    (Rendering|Material|SetMaterial (Variables|Default|GetCameraBase) 0 "/Game/StealthMaster/Art/Materials/Characters/Enemies/Robotic/Emily_D/Camera/M_Camera_Red.M_Camera_Red")
    (Utilities|FlowControl|Sequence
      (:then_0
        (bind _alpha (Timeline|Lerp1 Stop)
          (:Update
            (Transformation|SetWorldRotation _camera (Math|Interpolation|RInterpTo _originalcamerarotation (Math|Rotator|FindLookatRotation _returnvalue (Transformation|GetWorldLocation (Variables|Default|GetBillboard))) _alpha 1.0) false false)
            (Transformation|SetWorldRotation _cameraturret (Math|Rotator|MakeRotator 0.0 0.0 (.yaw (Math|Rotator|CombineRotators (Math|Rotator|MakeRotator 0.0 0.0 -9e+01) (Math|Rotator|MakeRotator 0.0 0.0 (.Yaw (Math|Rotator|BreakRotator (Math|Interpolation|RInterpTo _originalcamerarotation (Math|Rotator|FindLookatRotation _returnvalue (Transformation|GetWorldLocation (Variables|Default|GetBillboard))) _alpha 1.0))))))) false false))
          (:Finished
            (CallFunction|FUpdateRotation)
            (bind _alpha_2 (Timeline|Lerp2 PlayFromStart)
              (:Update
                (Transformation|SetWorldRotation _camera (Math|Interpolation|RInterpTo _originalcamerarotation (Math|Rotator|FindLookatRotation _returnvalue (Transformation|GetWorldLocation (Variables|Default|GetBillboard1))) _alpha_2 1.0) false false)
                (Transformation|SetWorldRotation _cameraturret (Math|Rotator|MakeRotator 0.0 0.0 (.yaw (Math|Rotator|CombineRotators (Math|Rotator|MakeRotator 0.0 0.0 -9e+01) (Math|Rotator|MakeRotator 0.0 0.0 (.Yaw (Math|Rotator|BreakRotator (Math|Interpolation|RInterpTo _originalcamerarotation (Math|Rotator|FindLookatRotation _returnvalue (Transformation|GetWorldLocation (Variables|Default|GetBillboard1))) _alpha_2 1.0))))))) false false))
              (:Finished
                (CallFunction|FUpdateRotation)
                (Timeline|Lerp1 PlayFromStart))))))
      (:then_1
        (Timeline|Lerp2 Stop)))))

(event Custom|D_Enable
  (params (Sector%20Index :type Integer))
  (bind _originalcamerarotation (Variables|Default|GetoriginalCameraRotation))
  (bind _cameraturret (Variables|Default|GetCameraTurret))
  (bind _cameraturret_2 (Variables|Default|GetCameraTurret))
  (bind _camera (Variables|Default|GetCamera))
  (bind _returnvalue (Transformation|GetWorldLocation _cameraturret_2))
  ;[1 1 1] Camera Rotation / Setup
  ;;[1 1 1] Dispatcher Functions
  (if (not (Variables|Default|Getdestroyed))
    (Variables|Default|SetisActive true)
    (Rendering|Material|SetMaterial (Variables|Default|GetCameraBase) 0 "/Game/StealthMaster/Art/Materials/Characters/Enemies/Robotic/Emily_D/Camera/M_Camera_Green.M_Camera_Green")
    (bind _alpha (Timeline|Lerp1 PlayFromStart)
      (:Update
        (Transformation|SetWorldRotation _camera (Math|Interpolation|RInterpTo _originalcamerarotation (Math|Rotator|FindLookatRotation _returnvalue (Transformation|GetWorldLocation (Variables|Default|GetBillboard))) _alpha 1.0) false false)
        (Transformation|SetWorldRotation _cameraturret (Math|Rotator|MakeRotator 0.0 0.0 (.yaw (Math|Rotator|CombineRotators (Math|Rotator|MakeRotator 0.0 0.0 -9e+01) (Math|Rotator|MakeRotator 0.0 0.0 (.Yaw (Math|Rotator|BreakRotator (Math|Interpolation|RInterpTo _originalcamerarotation (Math|Rotator|FindLookatRotation _returnvalue (Transformation|GetWorldLocation (Variables|Default|GetBillboard))) _alpha 1.0))))))) false false))
      (:Finished
        (CallFunction|FUpdateRotation)
        (bind _alpha_2 (Timeline|Lerp2 PlayFromStart)
          (:Update
            (Transformation|SetWorldRotation _camera (Math|Interpolation|RInterpTo _originalcamerarotation (Math|Rotator|FindLookatRotation _returnvalue (Transformation|GetWorldLocation (Variables|Default|GetBillboard1))) _alpha_2 1.0) false false)
            (Transformation|SetWorldRotation _cameraturret (Math|Rotator|MakeRotator 0.0 0.0 (.yaw (Math|Rotator|CombineRotators (Math|Rotator|MakeRotator 0.0 0.0 -9e+01) (Math|Rotator|MakeRotator 0.0 0.0 (.Yaw (Math|Rotator|BreakRotator (Math|Interpolation|RInterpTo _originalcamerarotation (Math|Rotator|FindLookatRotation _returnvalue (Transformation|GetWorldLocation (Variables|Default|GetBillboard1))) _alpha_2 1.0))))))) false false))
          (:Finished
            (CallFunction|FUpdateRotation)
            (Timeline|Lerp1 PlayFromStart)))))))

(event EventBeginPlay
  (bind _cameraturret (Variables|Default|GetCameraTurret))
  (bind _cameraturret_2 (Variables|Default|GetCameraTurret))
  (bind _camera (Variables|Default|GetCamera))
  (bind _returnvalue (Transformation|GetWorldLocation _cameraturret_2))
  ;[1 1 1] Camera Rotation / Setup
  (Utilities|FlowControl|Delay 0.2)
  (CallFunction|FSetup)
  (Transformation|SetWorldRotation (Variables|Default|GetCamera) (Math|Rotator|FindLookatRotation (Transformation|GetWorldLocation (Variables|Default|GetCameraTurret)) (Transformation|GetWorldLocation (Variables|Default|GetBillboard))) false false)
  (bind _output (Class|IAI|IGetSectorIndex(Message) (Variables|Default|GetsectorActorRef)))
  (bind _output_2 (Class|IAI|IGetSectorIndex(Message) (Game|GetGameMode)))
  (Variables|Default|SetoriginalCameraRotation (Transformation|GetWorldRotation (Variables|Default|GetCamera)))
  (if (== _output_2 _output)
    (Variables|Default|SetisActive true)
    (bind _alpha (Timeline|Lerp1 PlayFromStart)
      (:Update
        (Transformation|SetWorldRotation _camera (Math|Interpolation|RInterpTo (Variables|Default|GetoriginalCameraRotation) (Math|Rotator|FindLookatRotation _returnvalue (Transformation|GetWorldLocation (Variables|Default|GetBillboard))) _alpha 1.0) false false)
        (Transformation|SetWorldRotation _cameraturret (Math|Rotator|MakeRotator 0.0 0.0 (.yaw (Math|Rotator|CombineRotators (Math|Rotator|MakeRotator 0.0 0.0 -9e+01) (Math|Rotator|MakeRotator 0.0 0.0 (.Yaw (Math|Rotator|BreakRotator (Math|Interpolation|RInterpTo (Variables|Default|GetoriginalCameraRotation) (Math|Rotator|FindLookatRotation _returnvalue (Transformation|GetWorldLocation (Variables|Default|GetBillboard))) _alpha 1.0))))))) false false))
      (:Finished
        (CallFunction|FUpdateRotation)
        (bind _alpha_2 (Timeline|Lerp2 PlayFromStart)
          (:Update
            (Transformation|SetWorldRotation _camera (Math|Interpolation|RInterpTo (Variables|Default|GetoriginalCameraRotation) (Math|Rotator|FindLookatRotation _returnvalue (Transformation|GetWorldLocation (Variables|Default|GetBillboard1))) _alpha_2 1.0) false false)
            (Transformation|SetWorldRotation _cameraturret (Math|Rotator|MakeRotator 0.0 0.0 (.yaw (Math|Rotator|CombineRotators (Math|Rotator|MakeRotator 0.0 0.0 -9e+01) (Math|Rotator|MakeRotator 0.0 0.0 (.Yaw (Math|Rotator|BreakRotator (Math|Interpolation|RInterpTo (Variables|Default|GetoriginalCameraRotation) (Math|Rotator|FindLookatRotation _returnvalue (Transformation|GetWorldLocation (Variables|Default|GetBillboard1))) _alpha_2 1.0))))))) false false))
          (:Finished
            (CallFunction|FUpdateRotation)
            (Timeline|Lerp1 PlayFromStart)))))))

(event EventISectorPassThrough
  (params (Sector :type BP%20Sector%20Object%20Reference))
  ;[1 1 1] Setup Dispatchers
  (EventDispatchers|BindEventtoDEnableSector Sector (EventDispatchers|CreateEvent :!event Custom|D_Enable))
  (EventDispatchers|BindEventtoDDisableSector Sector (EventDispatchers|CreateEvent :!event Custom|D_Disable))
  (Variables|Default|SetsectorActorRef Sector))

(event Game|Damage|EventAnyDamage
  (params (Damage :type Float%20%28single-precision%29) (DamageType :type Damage%20Type%20Object%20Reference) (InstigatedBy :type Controller%20Object%20Reference) (DamageCauser :type Actor%20Object%20Reference))
  (bind _cameraturret (Variables|Default|GetCameraTurret))
  (bind _returnvalue (Transformation|GetWorldLocation _cameraturret))
  (Effects|SpawnEmitteratLocation "/Game/StarterContent/Particles/P_Explosion.P_Explosion" (Math|Vector|MakeVector (.x _returnvalue) (.y _returnvalue) (- (.z _returnvalue) 2e+01)) "0, 0, 0" "0.500000,0.500000,0.500000")
  (CallFunction|DDisable)
  (Components|DestroyComponent (Variables|Default|GetCameraTurret))
  (Variables|Default|Setdestroyed true)
  (Rendering|Components|Light|SetIntensity (Variables|Default|GetSpotLight) 0.0))

(event EventTick
  (params (DeltaSeconds :type Float%20%28single-precision%29))
  ;[1 1 1] Camera Rotation / Setup
  (CallFunction|FTrace))

(fn ConstructionScript)

(fn FTrace
  (bind _camera (Variables|Default|GetCamera))
  (bind _cameraturret (Variables|Default|GetCameraTurret))
  (bind _returnvalue (Transformation|GetWorldLocation _camera))
  (bind _returnvalue_2 (Transformation|GetWorldLocation _cameraturret))
  (if (Variables|Default|GetisActive)
    (bind (_outhit _returnvalue_3) (Collision|SphereTraceForObjects _returnvalue (+ _returnvalue (* (Math|Vector|GetForwardVector (Variables|Default|GetCamera)) 1e+04)) 125.0 (Utilities|Array|MakeArray "ObjectTypeQuery3") false 0 "None"))
    (bind _output (Class|IAI|IGetActor(Message) (.HitActor (Collision|BreakHitResult _outhit))))
    (if (== _output (Variables|Default|GetPlayerRef))
      (bind _asbp_stealth_master_class (Utilities|Casting|CastToBP_StealthMaster_Class (.HitActor (Collision|BreakHitResult _outhit))))
      (if _returnvalue_3
        (for _index (range 0 4)
          (switch int _index
            (:0
              (bind _returnvalue_4 (Collision|LineTraceByChannel _returnvalue_2 (Transformation|GetSocketLocation (Variables|/Script/Engine.Character|GetMesh _asbp_stealth_master_class) "head") "TraceTypeQuery1" false 0 "ForDuration"))
              (if (not _returnvalue_4)
                (Math|Integer|IncrementInt (LocalVariables|GethitCount))))
            (:1
              (bind _returnvalue_5 (Collision|LineTraceByChannel _returnvalue_2 (Transformation|GetSocketLocation (Variables|/Script/Engine.Character|GetMesh _asbp_stealth_master_class) "neck_01") "TraceTypeQuery1" false 0 "ForDuration"))
              (if (not _returnvalue_5)
                (Math|Integer|IncrementInt (LocalVariables|GethitCount))))
            (:2
              (bind _returnvalue_6 (Collision|LineTraceByChannel _returnvalue_2 (Transformation|GetSocketLocation (Variables|/Script/Engine.Character|GetMesh _asbp_stealth_master_class) "chest") "TraceTypeQuery1" false 0 "ForDuration"))
              (if (not _returnvalue_6)
                (Math|Integer|IncrementInt (LocalVariables|GethitCount))))
            (:3
              (bind _returnvalue_7 (Collision|LineTraceByChannel _returnvalue_2 (Transformation|GetSocketLocation (Variables|/Script/Engine.Character|GetMesh _asbp_stealth_master_class) "clavicle_l") "TraceTypeQuery1" false 0 "ForDuration"))
              (if (not _returnvalue_7)
                (Math|Integer|IncrementInt (LocalVariables|GethitCount))))
            (:4
              (bind _returnvalue_8 (Collision|LineTraceByChannel _returnvalue_2 (Transformation|GetSocketLocation (Variables|/Script/Engine.Character|GetMesh _asbp_stealth_master_class) "clavicle_r") "TraceTypeQuery1" false 0 "ForDuration"))
              (if (not _returnvalue_8)
                (Math|Integer|IncrementInt (LocalVariables|GethitCount))))))
        (if (> (LocalVariables|GethitCount) 3)
          (Default|CallAlertAI (Transformation|GetActorLocation)))))))

(fn FSetup
  (bind _output (Class|IAI|IGetActor(Message) (Pawn|GetControlledPawn (Game|GetPlayerController 0))))
  (Variables|Default|SetPlayerRef _output)
  (Transformation|AddLocalOffset (Variables|Default|GetBillboard) (Variables|Default|GetPoint1) false false)
  (Transformation|AddLocalOffset (Variables|Default|GetBillboard1) (Variables|Default|GetPoint2) false false))

(fn FUpdateRotation
  (Variables|Default|SetoriginalCameraRotation (Transformation|GetWorldRotation (Variables|Default|GetCamera))))

(fn IGetActive
  (return false))

(fn IGetActor
  (return 0))

(fn IGetCameraObject
  (return self))

(fn IGetCanTakeDamage
  (return false))

(fn IGetCodeLockNumber
  (return ""))

(fn IGetController
  (return 0))

(fn IGetElevatorLevel
  (return 0))

(fn IGetEnemyCurr/Max
  (return 0 0))

(fn IGetGenericController
  (return 0))

(fn IGetIsDrone
  (return false))

(fn IGetIsEnemy
  (return false))

(fn IGetLookforCover
  (return false))

(fn IGetObjectType
  (return (Variables|Default|GetType)))

(fn IGetOccupied
  (return false))

(fn IGetOverlappingActors
  (return 0))

(fn IGetPatrol?
  (return false))

(fn IGetPatrolLoop?
  (return false))

(fn IGetPatrolPathActor
  (return 0))

(fn IGetPatrolPathPoints
  (return 0))

(fn IGetPawnReference
  (return 0))

(fn IGetPlayerSector
  (return 0))

(fn IGetPlaystyle
  (return "NewEnumerator0"))

(fn IGetRange
  (return 0.0))

(fn IGetSector
  (params (Input :type Integer))
  (return (Variables|Default|GetsectorActorRef)))

(fn IGetSectorIndex
  (bind _output (Class|IAI|IGetSectorIndex(Message) (Variables|Default|GetsectorActorRef)))
  (return _output))

(fn IGetSectorSize
  (return "0, 0, 0"))

(fn IGetStance
  (return "NewEnumerator0"))

(fn IGetStunned?
  (return false))

(fn IGetVisibilityGM
  (return 0.0 false false false))

(fn IGetVisibilitySL
  (return 0.0))

(fn IGetWaitTime
  (return 0.0))

(fn IReturnDetectedVariables
  (return 0.0 0.0))

(fn ISectorGetContainedEnemies
  (return 0))