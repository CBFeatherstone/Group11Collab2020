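; BP_AICharacterTest_V1 is a test AI character with walk and run speeds, a hitscan attack and simple health.
; Attack snaps yaw to the control rotation, then fires a debug-drawn Camera-channel trace with slight random yaw spread, applying damage if it hits a BP_Character.
; The Attacking flag clears only after such a hit, as a failed cast ends the event early.
; Incoming damage reduces Health, and Death destroys the actor at zero or below.
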(event Custom|Walk
  (Variables|/Script/Engine.CharacterMovementComponent|SetMaxWalkSpeed (Variables|Character|GetCharacterMovement) (Variables|Default|GetWalkSpeed)))

(event Custom|Run
  (Variables|/Script/Engine.CharacterMovementComponent|SetMaxWalkSpeed (Variables|Character|GetCharacterMovement) (Variables|Default|GetRunSpeed)))

(event Custom|Attack
  (bind _returnvalue (Transformation|GetActorLocation))
  (bind _returnvalue_2 (Pawn|GetControlRotation :!class /Script/Engine.Pawn))
  (bind (_roll _pitch _yaw) (Math|Rotator|BreakRotator _returnvalue_2))
  (bind (_x _y _z) (Math|Vector|BreakVector _returnvalue))
  (bind _returnvalue_3 (+ _z 6e+01))
  (bind _returnvalue_4 (Math|Vector|MakeVector _x _y _returnvalue_3))
  (Variables|Default|SetAttacking true)
  (Transformation|SetActorRotation (Math|Rotator|MakeRotator 0.0 0.0 (.Yaw (Math|Rotator|BreakRotator _returnvalue_2))))
  (bind _outhit (Collision|LineTraceByChannel _returnvalue_4 (+ _returnvalue_4 (* (Math|Rotator|GetRotationXVector (Math|Rotator|MakeRotator _roll _pitch (+ _yaw (Math|Random|RandomFloatinRange -5.0 5.0)))) 2.5e+03)) "TraceTypeQuery2" false 0 "ForDuration"))
  (Utilities|Casting|CastToBP_Character (.HitActor (Collision|BreakHitResult _outhit)))
  (Game|Damage|ApplyDamage 0 5e+01 0 0)
  (Variables|Default|SetAttacking false))

(event Custom|Death
  (Actor|DestroyActor))

(event Game|Damage|EventAnyDamage
  (params (Damage :type Float%20%28single-precision%29) (DamageType :type Damage%20Type%20Object%20Reference) (InstigatedBy :type Controller%20Object%20Reference) (DamageCauser :type Actor%20Object%20Reference))
  (bind _output_get (Variables|Default|SetHealth (- (Variables|Default|GetHealth) Damage)))
  (if (<= _output_get 0.0)
    (CallFunction|Death)))

(fn ConstructionScript)