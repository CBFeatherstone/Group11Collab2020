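; AI spawner actor that creates an enemy character and its AIController at its own location when SpawnAI fires.
; With a valid PatrolPath, both spawn in patrol mode and the character occupies the path; otherwise they spawn without one.
; It then registers with the game mode via the patrol-branch character reference, even after a non-patrol spawn.
; Interface getters expose the path and its occupancy; the rest are stubs.
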(event Custom|SpawnAI
  (bind _defaultsceneroot (Variables|Default|GetDefaultSceneRoot))
  (bind _patrolpath (Variables|Default|GetPatrolPath))
  (bind _returnvalue (Transformation|GetWorldLocation _defaultsceneroot))
  (if (Utilities|IsValid (Variables|Default|GetPatrolPath))
    (bind _returnvalue_2 (Game|SpawnActorfromClass "/Game/StealthMaster/Tech/AI/BP_AI_Character_Testing.BP_AI_Character_Testing_C" (Math|Transform|MakeTransform _returnvalue "0, 0, 0" "1,1,1") "Undefined" 0 _patrolpath true false 0))
    (Game|SpawnActorfromClass "/Game/StealthMaster/Tech/AI/BP_AIController.BP_AIController_C" (Math|Transform|MakeTransform "0, 0, 0" "0, 0, 0" "1,1,1") "Undefined" 0 _patrolpath _returnvalue_2 true 0)
    (Class|IAI|IOccupyPatrolPoint(Message) _patrolpath _returnvalue_2)
    (else
      (bind _returnvalue_3 (Game|SpawnActorfromClass "/Game/StealthMaster/Tech/AI/BP_AI_Character_Testing.BP_AI_Character_Testing_C" (Math|Transform|MakeTransform _returnvalue "0, 0, 0" "1,1,1") "Undefined" 0 0 false false 0))
      (Game|SpawnActorfromClass "/Game/StealthMaster/Tech/AI/BP_AIController.BP_AIController_C" (Math|Transform|MakeTransform "0, 0, 0" "0, 0, 0" "1,1,1") "Undefined" 0 0 _returnvalue_3 false 0)))
  (bind _output (Class|IAI|IGetActor(Message) _returnvalue_2))
  (Class|IAI|IGMAddEnemy(Message) (Game|GetGameMode) _output))

(fn ConstructionScript)

(fn IGetActor
  (return 0))

(fn IGetController
  (return 0))

(fn IGetLookforCover
  (return false))

(fn IGetOccupied
  (bind _output (Class|IAI|IGetOccupied(Message) (Variables|Default|GetPatrolPath)))
  (return _output))

(fn IGetPatrol?
  (return false))

(fn IGetPatrolLoop?
  (return false))

(fn IGetPatrolPathActor
  (return (Variables|Default|GetPatrolPath)))

(fn IGetPatrolPathPoints
  (return 0))

(fn IGetRange
  (return 0.0))

(fn IGetStunned?
  (return false))

(fn IGetWaitTime
  (return 0.0))