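; Configurable phase objective for a stealth game: key card, button, specimen to burn or timed capture, with its mesh chosen in the construction script.
; Player interaction works within the sphere once the game mode's phase dispatcher activates it; capture runs on a looping timer whose progress decays outside.
; Completion adds score, advances the phase for last or fully collected group objectives, and, except specimens, messages linked doors.
; BeginPlay randomizes a code and optionally the location.
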(event OnComponentBeginOverlap(indicatorSphere)
  (params (OverlappedComponent :type Primitive%20Component%20Object%20Reference) (OtherActor :type Actor%20Object%20Reference) (OtherComp :type Primitive%20Component%20Object%20Reference) (OtherBodyIndex :type Integer) (bFromSweep :type Boolean) (SweepResult :type Hit%20Result%20Structure%20%28by%20ref%29))
  (if (Variables|Default|GetphaseActivated)
    (bind _output (Class|IAI|IGetActor(Message) OtherActor))
    (Utilities|IsValid _output
      (:Is%20Valid
        (if (== _output (Pawn|GetControlledPawn (Game|GetPlayerController 0)))
          _)))))

(event OnComponentEndOverlap(indicatorSphere)
  (params (OverlappedComponent :type Primitive%20Component%20Object%20Reference) (OtherActor :type Actor%20Object%20Reference) (OtherComp :type Primitive%20Component%20Object%20Reference) (OtherBodyIndex :type Integer))
  (if (Variables|Default|GetphaseActivated)
    (bind _output (Class|IAI|IGetActor(Message) OtherActor))
    (Utilities|IsValid _output
      (:Is%20Valid
        (if (== _output (Pawn|GetControlledPawn (Game|GetPlayerController 0)))
          _)))))

(event OnComponentBeginOverlap(Sphere)
  (params (OverlappedComponent :type Primitive%20Component%20Object%20Reference) (OtherActor :type Actor%20Object%20Reference) (OtherComp :type Primitive%20Component%20Object%20Reference) (OtherBodyIndex :type Integer) (bFromSweep :type Boolean) (SweepResult :type Hit%20Result%20Structure%20%28by%20ref%29))
  (if (Variables|Default|GetphaseActivated)
    (bind _output (Class|IAI|IGetActor(Message) OtherActor))
    (Utilities|IsValid _output
      (:Is%20Valid
        (if (== _output (Pawn|GetControlledPawn (Game|GetPlayerController 0)))
          (Variables|Default|SetisActive true))))))

(event OnComponentEndOverlap(Sphere)
  (params (OverlappedComponent :type Primitive%20Component%20Object%20Reference) (OtherActor :type Actor%20Object%20Reference) (OtherComp :type Primitive%20Component%20Object%20Reference) (OtherBodyIndex :type Integer))
  (if (Variables|Default|GetphaseActivated)
    (bind _output (Class|IAI|IGetActor(Message) OtherActor))
    (Utilities|IsValid _output
      (:Is%20Valid
        (if (== _output (Pawn|GetControlledPawn (Game|GetPlayerController 0)))
          (Variables|Default|SetisActive false))))))

(event Custom|AnimateButton
  (Variables|Default|SetoriginalLocationsBase (Transformation|GetWorldLocation (Variables|Default|GetButtonBaseMesh)))
  (Variables|Default|SetoriginalLocationsButton (Transformation|GetWorldLocation (Variables|Default|GetButtonMesh)))
  (bind _alpha (Timeline|Lerp Play)
    (:Update
      (Transformation|SetWorldLocation (Variables|Default|GetButtonMesh) (Math|Vector|Lerp(Vector) (Variables|Default|GetoriginalLocationsButton) (Variables|Default|GetoriginalLocationsBase) _alpha) false false))
    (:Finished
      (Rendering|Material|SetMaterial (Variables|Default|GetButtonBaseMesh) 0 "/Game/StealthMaster/Art/Materials/Props_Weapons/Gameplay/Button/M_Button_Green.M_Button_Green")
      (CallFunction|ButtonAnimated)
      (Audio|PlaySoundatLocation "/Game/StealthMaster/Art/Sound_Design/Enviroment/Buttons/Button_Pressed.Button_Pressed" (Variables|Default|GetoriginalLocationsButton) "0, 0, 0" 2.0 1.0 0.0 "/Game/StealthMaster/Art/Sound_Design/BasicAttenuation.BasicAttenuation" 0 0))))

(event Custom|ButtonAnimated
  (for _array_element (Variables|Default|GetlinkedActorRef)
    (Class|IAI|IActivateDoor(Message) _array_element self))
  (CallFunction|FPhaseCheck)
  (CallFunction|FAddScore))

(event EventBeginPlay
  (CallFunction|FRandomizeCode)
  (CallFunction|FSubscribetoGameMode)
  (CallFunction|FRandomizeLocation))

(event EventIInteract
  (params (isPlayer :type Boolean))
  (if isPlayer
    (if (Variables|Default|GetisActive)
      (switch Utilities|FlowControl|Switch|SwitchonE_ObjectiveType (Variables|Default|GetObjectiveType)
        (:NewEnumerator0
          (for _array_element (Variables|Default|GetlinkedActorRef)
            (Class|IAI|IActivateDoor(Message) _array_element self)
            (Audio|SpawnSoundatLocation "/Game/StealthMaster/Art/Sound_Design/UI/Objetive_Noti.Objetive_Noti" (Transformation|GetWorldLocation (Variables|Default|GetDefaultSceneRoot)) "0, 0, 0" 2.0 1.0 0.0 "/Game/StealthMaster/Art/Sound_Design/BasicAttenuation.BasicAttenuation" 0)
            (Actor|DestroyActor))
          (CallFunction|FPhaseCheck)
          (CallFunction|FAddScore))
        (:NewEnumerator1
          (CallFunction|AnimateButton))
        (:NewEnumerator3
          (for _array_element_2 (Variables|Default|GetfireLocations)
            (Effects|SpawnEmitteratLocation "/Game/TemplateContent/StarterContent/Particles/P_Fire.P_Fire" (+ (Transformation|GetWorldLocation (Variables|Default|GetDefaultSceneRoot)) _array_element_2)))
          (Audio|SpawnSoundatLocation "/Game/StarterContent/Audio/Fire_Sparks01_Cue.Fire_Sparks01_Cue" (Transformation|GetWorldLocation (Variables|Default|GetDefaultSceneRoot)) "0, 0, 0" 0.4 1.0 0.0 "/Game/StealthMaster/Art/Sound_Design/BasicAttenuation.BasicAttenuation" 0)
          (CallFunction|FPhaseCheck)
          (CallFunction|FAddScore))
        (:NewEnumerator4
          (Utilities|Time|SetTimerbyFunctionName 0 "F_CaptureObjective" 0.1 true)
          (Variables|Default|SetbeginCapture true))))))

(fn ConstructionScript
  (switch Utilities|FlowControl|Switch|SwitchonE_ObjectiveType (Variables|Default|GetObjectiveType)
    (:NewEnumerator0
      (CallFunction|FSetKeyCardVisible))
    (:NewEnumerator1
      (CallFunction|FSetButtonVisible))
    (:NewEnumerator3
      (CallFunction|FSetCodeVisible))
    (:NewEnumerator4
      (CallFunction|FSetCaptureObjectiveVisible)))
  (CallFunction|FUpdateCollisionVariables))

(fn FRandomizeCode
  (Utilities|FlowControl|Sequence
    (:then_0
      (Variables|Default|Setclodelock_1 (Math|Random|RandomIntegerinRange 0 9)))
    (:then_1
      (Variables|Default|Setcodelock_2 (Math|Random|RandomIntegerinRange 0 9)))
    (:then_2
      (Variables|Default|Setcodelock_3 (Math|Random|RandomIntegerinRange 0 9)))
    (:then_3
      (Variables|Default|Setcodelock_4 (Math|Random|RandomIntegerinRange 0 9)))))

(fn FCaptureObjective
  (if (< (Variables|Default|GetcurrentCaptureProgress) (Variables|Default|GetrequiredCaptureProgress))
    (if (Variables|Default|GetisActive)
      (Rendering|SetVisibility (Variables|Default|GetProgressBar) true false)
      (Variables|Default|SetcurrentCaptureProgress (+ (Variables|Default|GetcurrentCaptureProgress) 0.1))
      (Class|BPIObjPB|SetPercent(Message) (UserInterface|GetUserWidgetObject (Variables|Default|GetProgressBar)) (/ (Variables|Default|GetcurrentCaptureProgress) (Variables|Default|GetrequiredCaptureProgress)) :!label _label)
      (else
        (bind _output_get (Variables|Default|SetcurrentCaptureProgress (- (Variables|Default|GetcurrentCaptureProgress) 0.05)))
        (Utilities|FlowControl|Sequence
          (:then_0
            (goto _label))
          (:then_1
            (Rendering|SetVisibility (Variables|Default|GetProgressBar) false false))
          (:then_2
            (if (<= _output_get 0.0)
              (Variables|Default|SetbeginCapture false)
              (Class|KismetSystemLibrary|PauseTimer 0 "F_CaptureObjective"))))))
    (else
      (CallFunction|FObjectiveCaptured)
      (Rendering|SetVisibility (Variables|Default|GetProgressBar) false false))))

(fn FObjectiveCaptured
  (Class|KismetSystemLibrary|PauseTimer 0 "F_CaptureObjective")
  (Rendering|Material|SetMaterial (Variables|Default|GetLaptopBaseMesh) 0 "/Game/StealthMaster/Art/Materials/Props_Weapons/Gameplay/Tablet/M_Tablet_Inactive.M_Tablet_Inactive")
  (for _array_element (Variables|Default|GetlinkedActorRef)
    (Class|IAI|IActivateDoor(Message) _array_element)
    (CallFunction|FPhaseCheck)
    (Audio|SpawnSoundatLocation "/Game/StealthMaster/Art/Sound_Design/UI/Objetive_Noti.Objetive_Noti" (Transformation|GetWorldLocation (Variables|Default|GetDefaultSceneRoot)) "0, 0, 0" 5.0 1.0 0.0 "/Game/StealthMaster/Art/Sound_Design/BasicAttenuation.BasicAttenuation" 0)
    (CallFunction|FAddScore)))

(fn FSetKeyCardVisible
  (Rendering|SetVisibility (Variables|Default|GetKeyCardMesh) true true))

(fn FSetButtonVisible
  (Rendering|SetVisibility (Variables|Default|GetButtonBaseMesh) true true))

(fn FSetCaptureObjectiveVisible
  (Rendering|SetVisibility (Variables|Default|GetLaptopBaseMesh) true true))

(fn FSetCodeVisible
  (Rendering|SetVisibility (Variables|Default|GetStaticMesh) true true))

(fn FPhaseCheck
  (if (Variables|Default|GetlastObjectiveInPhase)
    (Variables|Default|SetobjectiveCollected true)
    (Variables|Default|SetlastObjectiveInPhase false)
    (if (Variables|Default|GetisGroupObjective)
      (bind _success (CallFunction|FCheckGroup))
      (if _success
        (Class|IAI|IUpdateGameModePhase(Message) (Game|GetGameMode))
        (else
          (Class|IAI|IDisableObjectiveMarker(Message) (Variables|/Script/Engine.ChildActorComponent|GetChildActor (Variables|Default|GetObjectiveMarker)))))
      (else
        (Class|IAI|IUpdateGameModePhase(Message) (Game|GetGameMode))))
    (else
      (Class|IAI|IDisableObjectiveMarker(Message) (Variables|/Script/Engine.ChildActorComponent|GetChildActor (Variables|Default|GetObjectiveMarker)))
      (Variables|Default|SetobjectiveCollected true))))

(fn FSubscribetoGameMode
  (bind _asbp_stealth_master_gm (Utilities|Casting|CastToBP_StealthMaster_GM (Game|GetGameMode)))
  (EventDispatchers|BindEventtoDUpdatePhase _asbp_stealth_master_gm (EventDispatchers|CreateEvent :!event FUpdatePhase))
  (Class|IAI|ISetObjectiveMarkerPhase(Message) (Variables|/Script/Engine.ChildActorComponent|GetChildActor (Variables|Default|GetObjectiveMarker)) (Variables|Default|Getphase) (Variables|Default|GetrequiredObjectiveMarker) (Variables|Default|GetrequiresStagger)))

(fn FUpdatePhase
  (params (Phase :type Integer))
  (if (== Phase (Variables|Default|Getphase))
    (Variables|Default|SetphaseActivated true)))

(fn FUpdateCollisionVariables
  (bind _sphere (Variables|Default|GetSphere))
  (Transformation|AddWorldOffset _sphere (Variables|Default|GetcollisionLocation) false false)
  (Components|Sphere|SetSphereRadius _sphere (Variables|Default|GetcollisionSize) true))

(fn FRandomizeLocation
  (bind _randomlocationset (Variables|Default|GetrandomLocationSet))
  (bind _defaultsceneroot (Variables|Default|GetDefaultSceneRoot))
  (bind _returnvalue (Utilities|Map|Length _randomlocationset))
  (bind _returnvalue_2 (Math|Random|RandomInteger _returnvalue))
  (if (Variables|Default|GetrandomizeLocaion)
    (bind _keys (Utilities|Map|Keys _randomlocationset))
    (bind _values (Utilities|Map|Values _randomlocationset))
    (Transformation|SetWorldLocation _defaultsceneroot (Utilities|Array|Get(acopy) _keys _returnvalue_2) false false)
    (Transformation|SetWorldRotation _defaultsceneroot (Utilities|Array|Get(acopy) _values _returnvalue_2) false false)))

(fn FCheckGroup
  (for _array_element (Variables|Default|GetgroupObjectives)
    (bind _output (Class|IAI|IGetCollected(Message) _array_element))
    (if (not _output)
      (return false)))
  (return true))

(fn FAddScore
  (bind _returnvalue (Game|GetGameMode))
  (switch Utilities|FlowControl|Switch|SwitchonE_ObjectiveType (Variables|Default|GetObjectiveType)
    (:NewEnumerator0
      (Class|IAI|IModifyScore(Message) _returnvalue 1e+03))
    (:NewEnumerator1
      (Class|IAI|IModifyScore(Message) _returnvalue 5e+02))
    (:NewEnumerator3
      (Class|IAI|IModifyScore(Message) _returnvalue 5e+03))
    (:NewEnumerator4
      (Class|IAI|IModifyScore(Message) _returnvalue 2.5e+02))))

(fn IGetActive
  (return false))

(fn IGetActor
  (return 0))

(fn IGetCameraObject
  (return 0))

(fn IGetCanTakeDamage
  (return false))

(fn IGetCodeLockNumber
  (return (Utilities|String|Append (Utilities|String|ToString(Integer) (Variables|Default|Getclodelock_1)) (Utilities|String|ToString(Integer) (Variables|Default|Getcodelock_2)) (Utilities|String|ToString(Integer) (Variables|Default|Getcodelock_3)) (Utilities|String|ToString(Integer) (Variables|Default|Getcodelock_4)))))

(fn IGetCollected
  (return (Variables|Default|GetobjectiveCollected)))

(fn IGetController
  (return 0))

(fn IGetCurrentPhase
  (return 0))

(fn IGetElevatorLevel
  (return 0))

(fn IGetEnemyCurr/Max
  (return 0 0))

(fn IGetFinalePhase
  (return false))

(fn IGetGenericController
  (return 0))

(fn IGetIsDrone
  (return false))

(fn IGetIsEnemy
  (return false))

(fn IGetLookforCover
  (return false))

(fn IGetObjectType
  (return "NewEnumerator3"))

(fn IGetOccupied
  (return false))

(fn IGetOverlappingActors
  (return 0))

(fn IGetPatrol?
  (return false))

(fn IGetPatrolLoop?
  (return false))

(fn IGetPatrolPathActor
  (return 0))

(fn IGetPatrolPathPoints
  (return 0))

(fn IGetPawnReference
  (return 0))

(fn IGetPlayerSector
  (return 0))

(fn IGetPlaystyle
  (return "NewEnumerator0"))

(fn IGetRange
  (return 0.0))

(fn IGetSceneComponentHumanoid
  (return 0))

(fn IGetScore
  (return 0.0))

(fn IGetSector
  (params (Input :type Integer))
  (return 0))

(fn IGetSectorIndex
  (return 0))

(fn IGetSectorSize
  (return "0, 0, 0"))

(fn IGetStance
  (return "NewEnumerator0"))

(fn IGetStunned?
  (return false))

(fn IGetVisibilityGM
  (return 0.0 false false false))

(fn IGetVisibilitySL
  (return 0.0))

(fn IGetWaitTime
  (return 0.0))

(fn IReturnDetectedVariables
  (return 0.0 0.0))

(fn ISectorGetContainedEnemies
  (return 0))