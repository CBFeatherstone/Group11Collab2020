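; BP_Elevator is a two-level elevator that players ride and non-player callers can also trigger through the interact interface.
; A box overlap gates player use, and an InProgress flag blocks repeat calls during travel.
; One timeline moves the root vertically between two points, reversed for ascent, while landing door actors close on departure and open on arrival.
; A second timeline slides the cab doors, and the current level is exposed through the interface.
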(event OnComponentBeginOverlap(Box)
  (params (OverlappedComponent :type Primitive%20Component%20Object%20Reference) (OtherActor :type Actor%20Object%20Reference) (OtherComp :type Primitive%20Component%20Object%20Reference) (OtherBodyIndex :type Integer) (bFromSweep :type Boolean) (SweepResult :type Hit%20Result%20Structure%20%28by%20ref%29))
  (bind _output (Class|IAI|IGetActor(Message) OtherActor))
  (Utilities|IsValid _output
    (:Is%20Valid
      (if (== _output (Pawn|GetControlledPawn (Game|GetPlayerController 0)))
        (Variables|Default|SetisActive true)))))

(event OnComponentEndOverlap(Box)
  (params (OverlappedComponent :type Primitive%20Component%20Object%20Reference) (OtherActor :type Actor%20Object%20Reference) (OtherComp :type Primitive%20Component%20Object%20Reference) (OtherBodyIndex :type Integer))
  (bind _output (Class|IAI|IGetActor(Message) OtherActor))
  (Utilities|IsValid _output
    (:Is%20Valid
      (if (== _output (Pawn|GetControlledPawn (Game|GetPlayerController 0)))
        (Variables|Default|SetisActive false)))))

(event Custom|Close%20Elevator%20Doors
  (bind _defaultscenerootlocation (Variables|Default|GetdefaultSceneRootLocation))
  (bind _alpha (Timeline|Timeline_0 Reverse)
    (:Update
      (Variables|Default|Setalpha _alpha)
      (Transformation|SetWorldLocation (Variables|Default|GetElevatorDoor1) (Math|Vector|MakeVector (.x (Math|Vector|Lerp(Vector) _defaultscenerootlocation (+ _defaultscenerootlocation (* (Math|Vector|GetForwardVector (Variables|Default|GetElevatorDoor1)) 68.0)) _alpha)) (.y (Math|Vector|Lerp(Vector) _defaultscenerootlocation (+ _defaultscenerootlocation (* (Math|Vector|GetForwardVector (Variables|Default|GetElevatorDoor1)) 68.0)) _alpha)) (.z (Transformation|GetWorldLocation (Variables|Default|GetElevatorDoor1)))) false false)
      (Transformation|SetWorldLocation (Variables|Default|GetElevatorDoor2) (Math|Vector|MakeVector (.x (Math|Vector|Lerp(Vector) _defaultscenerootlocation (+ _defaultscenerootlocation (* (Math|Vector|GetForwardVector (Variables|Default|GetElevatorDoor2)) 68.0)) _alpha)) (.y (Math|Vector|Lerp(Vector) _defaultscenerootlocation (+ _defaultscenerootlocation (* (Math|Vector|GetForwardVector (Variables|Default|GetElevatorDoor2)) 68.0)) _alpha)) (.z (Transformation|GetWorldLocation (Variables|Default|GetElevatorDoor2)))) false false))
    (:Finished
      (Audio|SpawnSoundatLocation "/Game/StealthMaster/Art/Sound_Design/Enviroment/Elevator/Elevator_Ding.Elevator_Ding" (Transformation|GetWorldLocation (Variables|Default|GetDefaultSceneRoot)) "0, 0, 0" 1.0 1.0 0.0 "/Game/StealthMaster/Art/Sound_Design/BasicAttenuation.BasicAttenuation" 0)
      (Audio|Components|Audio|Stop (Variables|Default|GetAudioInSide)))))

(event Custom|Elevator_Down
  (bind _pointa (Variables|Default|GetpointA))
  (for _array_element (Variables|Default|GetdoorActors)
    (Default|CloseDoors _array_element (Variables|Default|GetcurrentLevel) false))
  (bind _returnvalue (Audio|SpawnSoundAttached "/Game/StealthMaster/Art/Sound_Design/Enviroment/Elevator/Elevator_Running.Elevator_Running" (Variables|Default|GetDefaultSceneRoot) "None" "0, 0, 0" "0, 0, 0" "KeepRelativeOffset" false 0.1 1.0 0.0 "/Game/StealthMaster/Art/Sound_Design/BasicAttenuation.BasicAttenuation" 0))
  (Variables|Default|SetAudioInSide _returnvalue)
  (Utilities|FlowControl|Delay 0.2)
  (CallFunction|CloseElevatorDoors)
  (bind _newtrack_0 (Timeline|Lerp PlayFromStart)
    (:Update
      (Transformation|SetWorldLocation (Variables|Default|GetDefaultSceneRoot) (Math|Vector|MakeVector (.x _pointa) (.y _pointa) (Math|Float|Lerp (.z _pointa) (.z (Variables|Default|GetpointB)) _newtrack_0)) false false))
    (:Finished
      (if (Variables|Default|GetelevatorUp)
        (Variables|Default|SetelevatorUp false)
        (Variables|Default|SetcurrentLevel 2)
        (else
          (Variables|Default|SetelevatorUp true)
          (Variables|Default|SetcurrentLevel 1)))
      (Variables|Default|SetinProgress false)
      (Utilities|FlowControl|Delay 0.2)
      (for _array_element_2 (Variables|Default|GetdoorActors)
        (Default|OpenDoors _array_element_2 (Variables|Default|GetcurrentLevel) false)))))

(event Custom|Elevator_Up
  (bind _pointa (Variables|Default|GetpointA))
  (for _array_element (Variables|Default|GetdoorActors)
    (Default|CloseDoors _array_element (Variables|Default|GetcurrentLevel) false))
  (bind _returnvalue (Audio|SpawnSoundAttached "/Game/StealthMaster/Art/Sound_Design/Enviroment/Elevator/Elevator_Running.Elevator_Running" (Variables|Default|GetDefaultSceneRoot) "None" "0, 0, 0" "0, 0, 0" "KeepRelativeOffset" false 0.1 1.0 0.0 "/Game/StealthMaster/Art/Sound_Design/BasicAttenuation.BasicAttenuation" 0))
  (Variables|Default|SetAudioInSide _returnvalue)
  (bind _newtrack_0 (Timeline|Lerp ReverseFromEnd)
    (:Update
      (Transformation|SetWorldLocation (Variables|Default|GetDefaultSceneRoot) (Math|Vector|MakeVector (.x _pointa) (.y _pointa) (Math|Float|Lerp (.z _pointa) (.z (Variables|Default|GetpointB)) _newtrack_0)) false false))
    (:Finished
      (if (Variables|Default|GetelevatorUp)
        (Variables|Default|SetelevatorUp false)
        (Variables|Default|SetcurrentLevel 2)
        (else
          (Variables|Default|SetelevatorUp true)
          (Variables|Default|SetcurrentLevel 1)))
      (Variables|Default|SetinProgress false)
      (Utilities|FlowControl|Delay 0.2)
      (for _array_element_2 (Variables|Default|GetdoorActors)
        (Default|OpenDoors _array_element_2 (Variables|Default|GetcurrentLevel) false)))))

(event Custom|Open%20Elevator%20Doors
  (bind _defaultscenerootlocation (Variables|Default|GetdefaultSceneRootLocation))
  (bind _alpha (Timeline|Timeline_0 PlayFromStart)
    (:Update
      (Variables|Default|Setalpha _alpha)
      (Transformation|SetWorldLocation (Variables|Default|GetElevatorDoor1) (Math|Vector|MakeVector (.x (Math|Vector|Lerp(Vector) _defaultscenerootlocation (+ _defaultscenerootlocation (* (Math|Vector|GetForwardVector (Variables|Default|GetElevatorDoor1)) 68.0)) _alpha)) (.y (Math|Vector|Lerp(Vector) _defaultscenerootlocation (+ _defaultscenerootlocation (* (Math|Vector|GetForwardVector (Variables|Default|GetElevatorDoor1)) 68.0)) _alpha)) (.z (Transformation|GetWorldLocation (Variables|Default|GetElevatorDoor1)))) false false)
      (Transformation|SetWorldLocation (Variables|Default|GetElevatorDoor2) (Math|Vector|MakeVector (.x (Math|Vector|Lerp(Vector) _defaultscenerootlocation (+ _defaultscenerootlocation (* (Math|Vector|GetForwardVector (Variables|Default|GetElevatorDoor2)) 68.0)) _alpha)) (.y (Math|Vector|Lerp(Vector) _defaultscenerootlocation (+ _defaultscenerootlocation (* (Math|Vector|GetForwardVector (Variables|Default|GetElevatorDoor2)) 68.0)) _alpha)) (.z (Transformation|GetWorldLocation (Variables|Default|GetElevatorDoor2)))) false false))
    (:Finished
      (Audio|SpawnSoundatLocation "/Game/StealthMaster/Art/Sound_Design/Enviroment/Elevator/Elevator_Ding.Elevator_Ding" (Transformation|GetWorldLocation (Variables|Default|GetDefaultSceneRoot)) "0, 0, 0" 1.0 1.0 0.0 "/Game/StealthMaster/Art/Sound_Design/BasicAttenuation.BasicAttenuation" 0)
      (Audio|Components|Audio|Stop (Variables|Default|GetAudioInSide)))))

(event EventBeginPlay
  (bind _elevatorpoints (Variables|Default|GetelevatorPoints))
  (bind _defaultsceneroot (Variables|Default|GetDefaultSceneRoot))
  (bind _returnvalue (Transformation|GetWorldLocation _defaultsceneroot))
  (Variables|Default|SetpointA (+ (Utilities|Array|Get(acopy) _elevatorpoints) _returnvalue))
  (Variables|Default|SetpointB (+ (Utilities|Array|Get(acopy) _elevatorpoints 1) _returnvalue))
  (Variables|Default|SetdefaultSceneRootLocation (Transformation|GetWorldLocation (Variables|Default|GetDefaultSceneRoot))))

(event EventIInteract
  (params (isPlayer :type Boolean))
  (if isPlayer
    (if (Variables|Default|GetisActive)
      (if (not (Variables|Default|GetinProgress)) :!label _label
        (Variables|Default|SetinProgress true)
        (if (Variables|Default|GetelevatorUp)
          (CallFunction|ElevatorDown)
          (else
            (CallFunction|ElevatorUp)))))
    (else
      (goto _label))))

(fn ConstructionScript)

(fn IGetActive
  (return (Variables|Default|GetisActive)))

(fn IGetActor
  (return 0))

(fn IGetCameraObject
  (return 0))

(fn IGetCanTakeDamage
  (return false))

(fn IGetCodeLockNumber
  (return ""))

(fn IGetCollected
  (return false))

(fn IGetController
  (return 0))

(fn IGetCurrentPhase
  (return 0))

(fn IGetElevatorLevel
  (return (Variables|Default|GetcurrentLevel)))

(fn IGetEnemyCurr/Max
  (return 0 0))

(fn IGetFinalePhase
  (return false))

(fn IGetGenericController
  (return 0))

(fn IGetIsDrone
  (return false))

(fn IGetIsEnemy
  (return false))

(fn IGetLookforCover
  (return false))

(fn IGetObjectType
  (return "NewEnumerator3"))

(fn IGetOccupied
  (return false))

(fn IGetOverlappingActors
  (return 0))

(fn IGetPatrol?
  (return false))

(fn IGetPatrolLoop?
  (return false))

(fn IGetPatrolPathActor
  (return 0))

(fn IGetPatrolPathPoints
  (return 0))

(fn IGetPawnReference
  (return 0))

(fn IGetPlayerSector
  (return 0))

(fn IGetPlaystyle
  (return "NewEnumerator0"))

(fn IGetRange
  (return 0.0))

(fn IGetSceneComponentHumanoid
  (return 0))

(fn IGetScore
  (return 0.0))

(fn IGetSector
  (params (Input :type Integer))
  (return 0))

(fn IGetSectorIndex
  (return 0))

(fn IGetSectorSize
  (return "0, 0, 0"))

(fn IGetStance
  (return "NewEnumerator0"))

(fn IGetStunned?
  (return false))

(fn IGetVisibilityGM
  (return 0.0 false false false))

(fn IGetVisibilitySL
  (return 0.0))

(fn IGetWaitTime
  (return 0.0))

(fn IReturnDetectedVariables
  (return 0.0 0.0))

(fn ISectorGetContainedEnemies
  (return 0))