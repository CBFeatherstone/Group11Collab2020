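; Level door actor for StealthMaster with normal, elevator and button variants, optionally locked behind key card or button objectives.
; Construction script enables the variant's meshes and trigger; timelines swing single doors or slide elevator pairs alongside the linked elevator's doors.
; Interaction toggles the door once all mapped objectives are activated through the interface.
; Players must be inside the trigger and may first summon the elevator with a fixed delay; non-players skip both checks.
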(event OnComponentBeginOverlap(Box)
  (params (OverlappedComponent :type Primitive%20Component%20Object%20Reference) (OtherActor :type Actor%20Object%20Reference) (OtherComp :type Primitive%20Component%20Object%20Reference) (OtherBodyIndex :type Integer) (bFromSweep :type Boolean) (SweepResult :type Hit%20Result%20Structure%20%28by%20ref%29))
  (bind _output (Class|IAI|IGetActor(Message) OtherActor))
  (if (== _output (Pawn|GetControlledPawn (Game|GetPlayerController 0)))
    (Variables|Default|SetisActive true)))

(event OnComponentEndOverlap(Box)
  (params (OverlappedComponent :type Primitive%20Component%20Object%20Reference) (OtherActor :type Actor%20Object%20Reference) (OtherComp :type Primitive%20Component%20Object%20Reference) (OtherBodyIndex :type Integer))
  (bind _output (Class|IAI|IGetActor(Message) OtherActor))
  (if (== _output (Pawn|GetControlledPawn (Game|GetPlayerController 0)))
    (Variables|Default|SetisActive false)))

(event OnComponentBeginOverlap(Sphere)
  (params (OverlappedComponent :type Primitive%20Component%20Object%20Reference) (OtherActor :type Actor%20Object%20Reference) (OtherComp :type Primitive%20Component%20Object%20Reference) (OtherBodyIndex :type Integer) (bFromSweep :type Boolean) (SweepResult :type Hit%20Result%20Structure%20%28by%20ref%29))
  (bind _output (Class|IAI|IGetActor(Message) OtherActor))
  (if (== _output (Pawn|GetControlledPawn (Game|GetPlayerController 0)))
    (Variables|Default|SetisActive true)))

(event OnComponentEndOverlap(Sphere)
  (params (OverlappedComponent :type Primitive%20Component%20Object%20Reference) (OtherActor :type Actor%20Object%20Reference) (OtherComp :type Primitive%20Component%20Object%20Reference) (OtherBodyIndex :type Integer))
  (bind _output (Class|IAI|IGetActor(Message) OtherActor))
  (if (== _output (Pawn|GetControlledPawn (Game|GetPlayerController 0)))
    (Variables|Default|SetisActive false)))

(event Custom|Open_Doors
  (params (Level :type Integer))
  (bind _baserotation (Variables|Default|GetbaseRotation))
  (bind _defaultlocation (Variables|Default|GetdefaultLocation))
  (if (== Level (Variables|Default|Getlevel))
    (switch Utilities|FlowControl|Switch|SwitchonE_DoorType (Variables|Default|GetdoorType)
      (:NewEnumerator1
        (bind _alpha (Timeline|Timeline_0 PlayFromStart)
          (:Update
            (Transformation|SetWorldRotation (Variables|Default|GetNormalDoor) (Math|Rotator|Lerp(Rotator) _baserotation (Math|Rotator|CombineRotators _baserotation "0.000000,-130.000000,0.000000") _alpha true) false false))
          (:Finished
            (if (Variables|Default|GetdoorsClosed)
              (Variables|Default|SetdoorsClosed false)
              (else
                (Variables|Default|SetdoorsClosed true)))
            (Variables|Default|SetinProgress false))))
      (:NewEnumerator0
        (Default|OpenElevatorDoors (Variables|Default|GetelevatorRef))
        (Utilities|FlowControl|Delay 0.2)
        (bind _alpha_2 (Timeline|Lerp PlayFromStart)
          (:Update
            (Transformation|SetWorldLocation (Variables|Default|GetElevatorDoor1) (Math|Vector|Lerp(Vector) _defaultlocation (Variables|Default|Getlocation1) _alpha_2) false false)
            (Transformation|SetWorldLocation (Variables|Default|GetElevatorDoor2) (Math|Vector|Lerp(Vector) _defaultlocation (Variables|Default|Getlocation2) _alpha_2) false false))
          (:Finished
            (if (Variables|Default|GetdoorsClosed)
              (Variables|Default|SetdoorsClosed false)
              (else
                (Variables|Default|SetdoorsClosed true)))
            (Variables|Default|SetinProgress false))))
      (:NewEnumerator2
        (Timeline|Timeline_0 PlayFromStart)))))

(event Custom|Close_Doors
  (params (level :type Integer))
  (bind _baserotation (Variables|Default|GetbaseRotation))
  (bind _defaultlocation (Variables|Default|GetdefaultLocation))
  (if (== level (Variables|Default|Getlevel))
    (switch Utilities|FlowControl|Switch|SwitchonE_DoorType (Variables|Default|GetdoorType)
      (:NewEnumerator1
        (bind _alpha (Timeline|Timeline_0 ReverseFromEnd)
          (:Update
            (Transformation|SetWorldRotation (Variables|Default|GetNormalDoor) (Math|Rotator|Lerp(Rotator) _baserotation (Math|Rotator|CombineRotators _baserotation "0.000000,-130.000000,0.000000") _alpha true) false false))
          (:Finished
            (if (Variables|Default|GetdoorsClosed)
              (Variables|Default|SetdoorsClosed false)
              (else
                (Variables|Default|SetdoorsClosed true)))
            (Variables|Default|SetinProgress false))))
      (:NewEnumerator0
        (Default|CloseElevatorDoors (Variables|Default|GetelevatorRef))
        (Utilities|FlowControl|Delay 0.2)
        (bind _alpha_2 (Timeline|Lerp ReverseFromEnd)
          (:Update
            (Transformation|SetWorldLocation (Variables|Default|GetElevatorDoor1) (Math|Vector|Lerp(Vector) _defaultlocation (Variables|Default|Getlocation1) _alpha_2) false false)
            (Transformation|SetWorldLocation (Variables|Default|GetElevatorDoor2) (Math|Vector|Lerp(Vector) _defaultlocation (Variables|Default|Getlocation2) _alpha_2) false false))
          (:Finished
            (if (Variables|Default|GetdoorsClosed)
              (Variables|Default|SetdoorsClosed false)
              (else
                (Variables|Default|SetdoorsClosed true)))
            (Variables|Default|SetinProgress false))))
      (:NewEnumerator2
        (Timeline|Timeline_0 ReverseFromEnd)))))

(event EventIActivateDoor
  (params (Activator :type BP%20Objective%20Object%20Reference))
  (CallFunction|FActivateDoor Activator))

(event EventBeginPlay
  (Variables|Default|SetdefaultLocation (Transformation|GetWorldLocation (Variables|Default|GetDefaultSceneRoot)))
  (CallFunction|FSetupObjectiveMap)
  (CallFunction|FSetupDoorLocations))

(event EventIInteract
  (params (isPlayer :type Boolean))
  (bind _level (Variables|Default|Getlevel))
  (bind _success (CallFunction|FCheckActive))
  (if _success
    (if isPlayer
      (if (Variables|Default|GetisActive)
        (switch Utilities|FlowControl|Switch|SwitchonE_DoorType (Variables|Default|GetdoorType)
          (:NewEnumerator1
            _)
          (:NewEnumerator0
            (bind _level_2 (Class|IAI|IGetElevatorLevel(Message) (Variables|Default|GetelevatorRef)))
            (if (== _level_2 (Variables|Default|Getlevel))
              _
              (else
                (Class|IAI|IInteract(Message) (Variables|Default|GetelevatorRef) false)
                (Utilities|FlowControl|Delay 8.0))))
          (:NewEnumerator2
            _))
        (if (not (Variables|Default|GetinProgress)) :!label _label
          (Variables|Default|SetinProgress true)
          (if (Variables|Default|GetdoorsClosed)
            (CallFunction|OpenDoors _level)
            (else
              (CallFunction|CloseDoors _level)))))
      (else
        (goto _label)))))

(fn ConstructionScript
  (bind _normaldoor (Variables|Default|GetNormalDoor))
  (switch Utilities|FlowControl|Switch|SwitchonE_DoorType (Variables|Default|GetdoorType)
    (:NewEnumerator1
      (Rendering|SetVisibility _normaldoor true false :!label _label)
      (Collision|SetCollisionEnabled _normaldoor "QueryAndPhysics")
      (Collision|SetCollisionEnabled (Variables|Default|GetSphere) "QueryAndPhysics"))
    (:NewEnumerator0
      (Rendering|SetVisibility (Variables|Default|GetElevatorDoor1) true false)
      (Rendering|SetVisibility (Variables|Default|GetElevatorDoor2) true false)
      (Collision|SetCollisionEnabled (Variables|Default|GetElevatorDoor1) "QueryAndPhysics")
      (Collision|SetCollisionEnabled (Variables|Default|GetElevatorDoor2) "QueryAndPhysics")
      (Collision|SetCollisionEnabled (Variables|Default|GetBox) "QueryAndPhysics"))
    (:NewEnumerator2
      (goto _label))))

(fn FCheckActive
  (switch Utilities|FlowControl|Switch|SwitchonE_ObjectiveType (Variables|Default|GetobjectiveType)
    (:NewEnumerator2
      (return true))
    (:NewEnumerator0
      _)
    (:NewEnumerator1
      _))
  (bind _values (Utilities|Map|Values (Variables|Default|GetobjectiveMap)))
  (for _array_element _values
    (if (not _array_element)
      (return false)))
  (return true))

(fn FSetupObjectiveMap
  (for _array_element (Variables|Default|GetObjectiveArray)
    (Utilities|Map|Add (Variables|Default|GetobjectiveMap) _array_element false)))

(fn FActivateDoor
  (params (Objective :type BP%20Objective%20Object%20Reference))
  (if (.ReturnValue (Utilities|Map|Find (Variables|Default|GetobjectiveMap) Objective))
    (Utilities|Map|Add (Variables|Default|GetobjectiveMap) Objective (Class|KismetSystemLibrary|MakeLiteralBool true))
    (else
      (Development|PrintString (Utilities|String|Append "ITME NOT FOUND!:      " (Utilities|GetDisplayName Objective))))))

(fn FSetupDoorLocations
  (switch Utilities|FlowControl|Switch|SwitchonE_DoorType (Variables|Default|GetdoorType)
    (:NewEnumerator1
      (Variables|Default|SetbaseRotation (Transformation|GetWorldRotation (Variables|Default|GetNormalDoor)) :!label _label))
    (:NewEnumerator0
      (Variables|Default|Setlocation1 (+ (Variables|Default|GetdefaultLocation) (* (* (Math|Vector|GetForwardVector (Variables|Default|GetElevatorDoor1)) 1.0) (Variables|Default|GetdoorMovementRange))))
      (Variables|Default|Setlocation2 (+ (Variables|Default|GetdefaultLocation) (* (* (Math|Vector|GetForwardVector (Variables|Default|GetElevatorDoor2)) 1.0) (Variables|Default|GetdoorMovementRange)))))
    (:NewEnumerator2
      (goto _label))))

(fn IGetActive
  (return false))

(fn IGetActor
  (return 0))

(fn IGetCameraObject
  (return 0))

(fn IGetController
  (return 0))

(fn IGetElevatorLevel
  (return 0))

(fn IGetEnemyCurr/Max
  (return 0 0))

(fn IGetIsDrone
  (return false))

(fn IGetIsEnemy
  (return false))

(fn IGetLookforCover
  (return false))

(fn IGetObjectType
  (return "NewEnumerator3"))

(fn IGetOccupied
  (return false))

(fn IGetOverlappingActors
  (return 0))

(fn IGetPatrol?
  (return false))

(fn IGetPatrolLoop?
  (return false))

(fn IGetPatrolPathActor
  (return 0))

(fn IGetPatrolPathPoints
  (return 0))

(fn IGetPawnReference
  (return 0))

(fn IGetPlayerSector
  (return 0))

(fn IGetPlaystyle
  (return "NewEnumerator0"))

(fn IGetRange
  (return 0.0))

(fn IGetSector
  (params (Input :type Integer))
  (return 0))

(fn IGetSectorIndex
  (return 0))

(fn IGetSectorSize
  (return "0, 0, 0"))

(fn IGetStance
  (return "NewEnumerator0"))

(fn IGetStunned?
  (return false))

(fn IGetVisibilityGM
  (return 0.0 false false false))

(fn IGetWaitTime
  (return 0.0))

(fn IReturnDetectedVariables
  (return 0.0 0.0))

(fn ISectorGetContainedEnemies
  (return 0))