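; BP_Target is a damageable objective actor for StealthMaster's phase-based missions.
; It binds to the game mode's phase update, highlighting its mesh through custom depth, and passes its phase to a child-actor objective marker.
; Any damage marks it collected and clears the highlight.
; It then either disables its marker or, as last objective, advances the game mode phase, with group objectives first checking all members via interface.
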(event EventBeginPlay
  (CallFunction|FSubscribetoGameMode))

(event Game|Damage|EventAnyDamage
  (params (Damage :type Float%20%28single-precision%29) (DamageType :type Damage%20Type%20Object%20Reference) (InstigatedBy :type Controller%20Object%20Reference) (DamageCauser :type Actor%20Object%20Reference))
  (CallFunction|FPhaseCheck)
  (Rendering|SetRenderCustomDepth (Variables|Default|GetStaticMesh) false))

(fn ConstructionScript)

(fn FUpdatePhase
  (params (Phase :type Integer))
  (if (== Phase (Variables|Default|Getphase))
    (Variables|Default|SetphaseActivated true)
    (Rendering|SetRenderCustomDepth (Variables|Default|GetStaticMesh) true)))

(fn FPhaseCheck
  (if (Variables|Default|GetlastObjectiveInPhase)
    (Variables|Default|SetobjectiveCollected true)
    (Variables|Default|SetlastObjectiveInPhase false)
    (if (Variables|Default|GetisGroupObjective)
      (bind _newparam (CallFunction|FCheckGroup))
      (if _newparam
        (Class|IAI|IUpdateGameModePhase(Message) (Game|GetGameMode))
        (else
          (Class|IAI|IDisableObjectiveMarker(Message) (Variables|/Script/Engine.ChildActorComponent|GetChildActor (Variables|Default|GetObjectiveMarker)))))
      (else
        (Class|IAI|IUpdateGameModePhase(Message) (Game|GetGameMode))))
    (else
      (Class|IAI|IDisableObjectiveMarker(Message) (Variables|/Script/Engine.ChildActorComponent|GetChildActor (Variables|Default|GetObjectiveMarker)))
      (Variables|Default|SetobjectiveCollected true))))

(fn FSubscribetoGameMode
  (bind _asbp_stealth_master_gm (Utilities|Casting|CastToBP_StealthMaster_GM (Game|GetGameMode)))
  (EventDispatchers|BindEventtoDUpdatePhase _asbp_stealth_master_gm (EventDispatchers|CreateEvent :!event FUpdatePhase))
  (Class|IAI|ISetObjectiveMarkerPhase(Message) (Variables|/Script/Engine.ChildActorComponent|GetChildActor (Variables|Default|GetObjectiveMarker)) (Variables|Default|Getphase) (Variables|Default|GetrequiresObjectiveMarker) false))

(fn FCheckGroup
  (for _array_element (Variables|Default|GetgroupObjectiveActors)
    (bind _output (Class|IAI|IGetCollected(Message) _array_element))
    (if (not _output)
      (return false)))
  (return true))

(fn IGetActive
  (return false))

(fn IGetActor
  (return 0))

(fn IGetCameraObject
  (return 0))

(fn IGetCanTakeDamage
  (return false))

(fn IGetCodeLockNumber
  (return ""))

(fn IGetCollected
  (return (Variables|Default|GetobjectiveCollected)))

(fn IGetController
  (return 0))

(fn IGetCurrentPhase
  (return 0))

(fn IGetElevatorLevel
  (return 0))

(fn IGetEnemyCurr/Max
  (return 0 0))

(fn IGetFinalePhase
  (return false))

(fn IGetGenericController
  (return 0))

(fn IGetIsDrone
  (return false))

(fn IGetIsEnemy
  (return false))

(fn IGetLookforCover
  (return false))

(fn IGetObjectType
  (return "NewEnumerator3"))

(fn IGetOccupied
  (return false))

(fn IGetOverlappingActors
  (return 0))

(fn IGetPatrol?
  (return false))

(fn IGetPatrolLoop?
  (return false))

(fn IGetPatrolPathActor
  (return 0))

(fn IGetPatrolPathPoints
  (return 0))

(fn IGetPawnReference
  (return 0))

(fn IGetPlayerSector
  (return 0))

(fn IGetPlaystyle
  (return "NewEnumerator0"))

(fn IGetRange
  (return 0.0))

(fn IGetSceneComponentHumanoid
  (return 0))

(fn IGetScore
  (return 0.0))

(fn IGetSector
  (params (Input :type Integer))
  (return 0))

(fn IGetSectorIndex
  (return 0))

(fn IGetSectorSize
  (return "0, 0, 0"))

(fn IGetStance
  (return "NewEnumerator0"))

(fn IGetStunned?
  (return false))

(fn IGetVisibilityGM
  (return 0.0 false false false))

(fn IGetVisibilitySL
  (return 0.0))

(fn IGetWaitTime
  (return 0.0))

(fn IReturnDetectedVariables
  (return 0.0 0.0))

(fn ISectorGetContainedEnemies
  (return 0))