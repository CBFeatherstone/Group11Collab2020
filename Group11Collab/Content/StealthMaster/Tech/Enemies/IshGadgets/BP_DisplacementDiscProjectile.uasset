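; BP_DisplacementDiscProjectile is a gadget projectile that swaps the locations of its owner and an actor it hits.
; Its collision sphere's begin-overlap passes a DoOnce, then checks that the other actor is not the projectile owner.
; It caches both locations before setting each actor to the other's, without sweeping.
; The DoOnce precedes the owner check, so a first overlap with the owner uses up the swap.
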(event OnComponentBeginOverlap(SphereCollision)
  (params (OverlappedComponent :type Primitive%20Component%20Object%20Reference) (OtherActor :type Actor%20Object%20Reference) (OtherComp :type Primitive%20Component%20Object%20Reference) (OtherBodyIndex :type Integer) (bFromSweep :type Boolean) (SweepResult :type Hit%20Result%20Structure%20%28by%20ref%29))
  (Utilities|FlowControl|DoOnce false
    (:Completed
      (Variables|Default|SetOtherActor OtherActor)
      (if (!= (Variables|Default|GetOtherActor) (Variables|Default|GetProjectileOwner))
        (CallFunction|CachePositions)
        (CallFunction|SwitchPositions)))))

(event Custom|SwitchPositions
  (Transformation|SetActorLocation (Variables|Default|GetProjectileOwner) (Variables|Default|GetEnemyPosition) false false)
  (Transformation|SetActorLocation (Variables|Default|GetOtherActor) (Variables|Default|GetPlayerLocation) false false))

(event Custom|CachePositions
  (Variables|Default|SetPlayerLocation (Transformation|GetActorLocation (Variables|Default|GetProjectileOwner)))
  (Variables|Default|SetEnemyPosition (Transformation|GetActorLocation (Variables|Default|GetOtherActor))))

(event EventBeginPlay
  (|CallParentFunction))

(event Collision|EventActorBeginOverlap
  (params (OtherActor :type Actor%20Object%20Reference)))

(fn ConstructionScript
  (|CallParentFunction))