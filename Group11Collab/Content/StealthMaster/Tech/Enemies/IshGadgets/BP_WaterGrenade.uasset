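; BP_WaterGrenade is a gadget grenade that leaves a water spill on timeout or affects enemies it touches.
; A looping one-second timer drives a countdown that spawns WaterSpill and destroys the grenade at zero.
; The first capsule overlap with a valid actor cancels the timer; exact class checks stun base enemies or kill drones, destroying the grenade.
; Other classes only print a message, leaving it without a countdown.
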(event OnComponentBeginOverlap(Capsule)
  (params (OverlappedComponent :type Primitive%20Component%20Object%20Reference) (OtherActor :type Actor%20Object%20Reference) (OtherComp :type Primitive%20Component%20Object%20Reference) (OtherBodyIndex :type Integer) (bFromSweep :type Boolean) (SweepResult :type Hit%20Result%20Structure%20%28by%20ref%29))
  (Utilities|FlowControl|DoOnce false
    (:Completed
      (Utilities|IsValid OtherActor
        (:Is%20Valid
          (Variables|Default|SetOtherActor OtherActor)
          (Utilities|Time|ClearandInvalidateTimerbyHandle (Variables|Default|GetGrenadeTimer))
          (if (== (Utilities|GetClass (Variables|Default|GetOtherActor)) "/Game/StealthMaster/Tech/Enemies/Enemy_BaseCharacter_Class.Enemy_BaseCharacter_Class_C")
            (Class|EnemyInterface|IStunEnemy(Message) (Variables|Default|GetOtherActor))
            (Actor|DestroyActor)
            (elif (== (Utilities|GetClass (Variables|Default|GetOtherActor)) "/Game/StealthMaster/Tech/Enemies/New_Enemy_Drone_Class.New_Enemy_Drone_Class_C")
              (Class|EnemyDroneInterface|IDeath(Message) (Variables|Default|GetOtherActor))
              (Actor|DestroyActor)
              (else
                (Development|PrintString "It was neither class" true true "(R=1.000000,G=0.104262,B=0.005208,A=1.000000)")))))))))

(event Custom|DetonationTimer
  (bind _returnvalue (Utilities|Time|SetTimerbyEvent (EventDispatchers|CreateEvent :!event Custom|TimeLeft) 1.0 true))
  (Variables|Default|SetGrenadeTimer _returnvalue))

(event Custom|TimeLeft
  (Math|Float|DecrementFloat (Variables|Default|GetTimer)
    (:%20%20
      (if (<= (Variables|Default|GetTimer) 0.0)
        (Development|PrintString "No time left explode!!!!" true true "(R=0.209480,G=1.000000,B=0.161475,A=1.000000)")
        (Utilities|Time|ClearandInvalidateTimerbyHandle (Variables|Default|GetGrenadeTimer))
        (CallFunction|SpawnWaterSpill)
        (else
          (Development|PrintString "Timer Still left" true true "(R=1.000000,G=0.000000,B=0.009362,A=1.000000)"))))))

(event Custom|SpawnWaterSpill
  (Game|SpawnActorfromClass "/Game/StealthMaster/Tech/Enemies/IshGadgets/WaterSpill.WaterSpill_C" (Transformation|GetActorTransform) "Undefined" self 0)
  (Actor|DestroyActor))

(event EventBeginPlay
  (CallFunction|DetonationTimer))

(fn ConstructionScript)