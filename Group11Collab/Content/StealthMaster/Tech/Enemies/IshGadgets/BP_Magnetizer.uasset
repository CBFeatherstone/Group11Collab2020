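; BP_Magnetizer is a gadget weapon that fires positive and negative magnet projectiles from its fire point, with its parent actor's instigator.
; Positive projectiles accumulate in an array, with a function to remove them.
; Only one negative projectile is kept, as firing another destroys and replaces it.
; Each negative shot passes its reference to every stored positive projectile through MagnetRef.
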(event Custom|SpawnProjectile-
  (bind _self self)
  (bind _self_2 self)
  (if (Variables|Default|GetNegativeUsed)
    (Development|PrintString "Negative Being Used" true true "(R=1.000000,G=0.195761,B=0.000000,A=1.000000)" 5.0)
    (Actor|DestroyActor (Variables|Default|GetProjectile-Var))
    (Variables|Default|SetProjectile-Var 0)
    (Variables|Default|SetNegativeUsed false)
    (bind _returnvalue (Game|SpawnActorfromClass "/Game/StealthMaster/Tech/Enemies/IshGadgets/Projectile-.Projectile-_C" (Transformation|GetWorldTransform (Variables|Default|GetWeaponFirePoint)) "Undefined" _self _self (Game|GetInstigator (Actor|GetParentActor))))
    (Variables|Default|SetProjectile-Var _returnvalue)
    (CallFunction|SetMagnetRef)
    (else
      (Variables|Default|SetNegativeUsed true)
      (bind _returnvalue_2 (Game|SpawnActorfromClass "/Game/StealthMaster/Tech/Enemies/IshGadgets/Projectile-.Projectile-_C" (Transformation|GetWorldTransform (Variables|Default|GetWeaponFirePoint)) "Undefined" _self_2 _self_2 (Game|GetInstigator (Actor|GetParentActor))))
      (Variables|Default|SetProjectile-Var _returnvalue_2)
      (CallFunction|SetMagnetRef))))

(event Custom|SetMagnetRef
  (for _array_element (Variables|Default|GetProjectile+Array)
    (Default|MagnetRef _array_element (Variables|Default|GetProjectile-Var))))

(event Custom|SpawnProjectile+
  (bind _self self)
  (bind _returnvalue (Game|SpawnActorfromClass "/Game/StealthMaster/Tech/Enemies/IshGadgets/Projectile+.Projectile+_C" (Transformation|GetWorldTransform (Variables|Default|GetWeaponFirePoint)) "Undefined" _self _self _self (Game|GetInstigator (Actor|GetParentActor))))
  (Utilities|Array|AddUnique (Variables|Default|GetProjectile+Array) _returnvalue))

(event Input|KeyboardEvents|J
  (params (Key :type Key%20Structure)))

(event Input|KeyboardEvents|K
  (params (Key :type Key%20Structure)))

(fn ConstructionScript
  (|CallParentFunction))

(fn RemoveProjectilefromArray
  (params (Projectile :type Projectile+%20Object%20Reference))
  (Utilities|Array|RemoveItem (Variables|Default|GetProjectile+Array) Projectile))