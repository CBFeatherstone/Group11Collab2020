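; BP_TaserProjectile is a taser weapon projectile that stuns the actor it hits.
; On overlap it checks that the other actor is valid and uses a macro to exclude the projectile's owner.
; It then sends the stun-enemy interface message to that actor and destroys itself, whether or not the actor implements the interface.
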(event EventBeginPlay
  (|CallParentFunction) ; This node is disabled and will not be called.\nDrag off pins to build functionality.
)

(event Collision|EventActorBeginOverlap
  (params (OtherActor :type Actor%20Object%20Reference))
  ;[1 1 1] Stun Enemy
  (bind _output_get (Variables|Default|SetOtherActor OtherActor))
  (Utilities|IsValid _output_get
    (:Is%20Valid
      (Utilities|IsOtherActor!=ProjectileOwner?
        (:True
          (Class|EnemyInterface|IStunEnemy(Message) (Variables|Default|GetOtherActor))
          (Actor|DestroyActor))))))

(fn ConstructionScript
  (|CallParentFunction))