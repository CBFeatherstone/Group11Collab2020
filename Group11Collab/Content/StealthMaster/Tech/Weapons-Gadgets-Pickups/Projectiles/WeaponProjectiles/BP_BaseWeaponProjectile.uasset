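; Base weapon projectile that damages the actor it hits and then destroys itself.
; BeginPlay caches the Instigator and its controller, and a macro makes collision-sphere hits ignore that owner.
; Valid hits spawn a scaled-down Splatter emitter on Base_Character_Class actors or BulletHit on anything else, oriented against the projectile's forward vector.
; Damage comes from the PlayerWeapon reference and is credited to the cached controller.
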(event OnComponentHit(SphereCollision)
  (params (HitComponent :type Primitive%20Component%20Object%20Reference) (OtherActor :type Actor%20Object%20Reference) (OtherComp :type Primitive%20Component%20Object%20Reference) (NormalImpulse :type Vector :default "0, 0, 0") (Hit :type Hit%20Result%20Structure%20%28by%20ref%29))
  (bind _spherecollision (Variables|Default|GetSphereCollision))
  (bind _sphere (Variables|Default|GetSphere))
  (bind _returnvalue (Transformation|GetWorldLocation _sphere))
  (bind _returnvalue_2 (Math|Vector|GetForwardVector _spherecollision))
  (bind _returnvalue_3 (Math|Vector|GetRightVector _spherecollision))
  (bind _returnvalue_4 (* _returnvalue_2 -1.0))
  (bind _returnvalue_5 (Math|Rotator|MakeRotfromXY _returnvalue_4 _returnvalue_3))
  ;[1 1 1] Deal Damage
  (bind _output_get (Variables|Default|SetOtherActor OtherActor))
  (Utilities|IsValid _output_get
    (:Is%20Valid
      (Utilities|IsOtherActor!=ProjectileOwner?
        (:Yes
          (Utilities|Casting|CastToBase_Character_Class OtherActor
            (:then
              (Effects|SpawnEmitteratLocation "/Game/StealthMaster/Art/ParticleSystems/JohnMc/BloodSplatter/Splatter.Splatter" _returnvalue _returnvalue_5 "0.200000,0.200000,0.200000"))
            (:CastFailed
              (Effects|SpawnEmitteratLocation "/Game/StealthMaster/Art/ParticleSystems/JohnMc/BulletHit/BulletHit.BulletHit" _returnvalue _returnvalue_5)))
          (CallFunction|ApplyDamage OtherActor)
          (Actor|DestroyActor))))))

(event EventBeginPlay
  (bind _instigator (Variables|Actor|GetInstigator))
  ;[1 1 1] Get and Set Owner
  (Variables|Default|SetProjectileOwner _instigator)
  (Variables|Default|SetOwnerController (Pawn|GetController _instigator)))

(fn ConstructionScript)

(fn ApplyDamage
  (params (Other%20Actor :type Actor%20Object%20Reference))
  (Game|Damage|ApplyDamage Other%20Actor (Variables|/Game/StealthMaster/Tech/Weapons-Gadgets-Pickups/Weapons/BP_BaseWeapon.BP_BaseWeapon_C|GetDamage (Variables|Default|GetPlayerWeapon)) (Variables|Default|GetOwnerController) self))