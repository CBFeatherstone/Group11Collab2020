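; Grenade projectile that explodes on overlapping any actor other than its owner, or when play ends for it, as when its time runs out.
; BeginPlay caches the instigator as owner and its controller for damage attribution.
; Explode fires a radial force impulse, applies full radial damage from the EnemyGadget damage value while ignoring the owner, then destroys the actor.
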(event Custom|Explode
  ;[1 1 1] Explode
  (Class|RadialForceComponent|FireImpulse (Variables|Default|GetRadialForce))
  (CallFunction|ApplyRadialDamage)
  (Actor|DestroyActor))

(event EventBeginPlay
  (bind _returnvalue (Game|GetInstigator))
  ;[1 1 1] Get and Set Owner
  (Variables|Default|SetProjectileOwner _returnvalue)
  (Variables|Default|SetOwnerController (Game|GetInstigatorController _returnvalue)))

(event EventEndPlay
  (params (EndPlayReason :type EEndPlayReason%20Enum :default "Destroyed"))
  ;[1 1 1] Time Runs Out
  (CallFunction|Explode))

(event EventTick
  (params (DeltaSeconds :type Float%20%28single-precision%29))
  (|CallParentFunction DeltaSeconds) ; This node is disabled and will not be called.\nDrag off pins to build functionality.
)

(event Collision|EventActorBeginOverlap
  (params (OtherActor :type Actor%20Object%20Reference))
  ;[1 1 1] Direct Hit
  (bind _output_get (Variables|Default|SetOtherActor OtherActor))
  (Utilities|IsValid _output_get
    (:Is%20Valid
      (Utilities|IsOtherActor!=ProjectileOwner?
        (:Yes
          (CallFunction|Explode))))))

(fn ConstructionScript
  (|CallParentFunction))

(fn ApplyRadialDamage
  (Game|Damage|ApplyRadialDamage (Variables|/Game/StealthMaster/Tech/Weapons-Gadgets-Pickups/Gadgets/BP_GrenadeGadget.BP_GrenadeGadget_C|GetDamage (Variables|Default|GetEnemyGadget)) (Transformation|GetActorLocation) (Variables|Default|GetExplosionRadius) 0 (Utilities|Array|MakeArray (Variables|Default|GetProjectileOwner)) self (Variables|Default|GetOwnerController) true "ECC_Visibility"))