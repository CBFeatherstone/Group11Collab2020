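; BP_BeeProjectile is a gadget projectile that deals damage over time to an actor overlapping it.
; Begin overlap stores the actor and starts a looping timer at DamageTickTime, which applies damage on each tick unless that actor is the projectile's owner.
; It tracks only the latest actor and timer handle, and any end overlap clears that timer.
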(event Custom|DamageOverTime
  ;[1 1 1] Deal Damage
  (Utilities|IsOtherActor!=ProjectileOwner?
    (:Yes
      (CallFunction|ApplyDamage))))

(event Collision|EventActorEndOverlap
  (params (OtherActor :type Actor%20Object%20Reference))
  ;[1 1 1] Deal Damage
  (Utilities|Time|ClearandInvalidateTimerbyHandle (stale Collision|EventActorBeginOverlap _returnvalue)))

(event EventTick
  (params (DeltaSeconds :type Float%20%28single-precision%29))
  (|CallParentFunction DeltaSeconds) ; This node is disabled and will not be called.\nDrag off pins to build functionality.
)

(event Collision|EventActorBeginOverlap
  (params (OtherActor :type Actor%20Object%20Reference))
  ;[1 1 1] Deal Damage
  (bind _output_get (Variables|Default|SetOtherActor OtherActor))
  (Utilities|IsValid _output_get
    (:Is%20Valid
      (bind _returnvalue (Utilities|Time|SetTimerbyEvent (delegate Custom|DamageOverTime) (Variables|Default|GetDamageTickTime) true)))))

(fn ConstructionScript
  (|CallParentFunction))