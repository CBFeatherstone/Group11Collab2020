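; Base projectile Blueprint for player gadgets that damages actors it overlaps.
; On BeginPlay it caches its Instigator as owner, along with that Instigator's controller.
; A valid overlapping actor other than the owner takes damage equal to the gadget's Damage, credited to the owner's controller, and the projectile then destroys itself.
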(event EventBeginPlay
  (bind _instigator (Variables|Actor|GetInstigator))
  ;[1 1 1] Get and Set Owner
  (Variables|Default|SetProjectileOwner _instigator)
  (Variables|Default|SetOwnerController (Game|GetInstigatorController _instigator)))

(event EventTick
  (params (DeltaSeconds :type Float%20%28single-precision%29)))

(event Collision|EventActorBeginOverlap
  (params (OtherActor :type Actor%20Object%20Reference))
  ;[1 1 1] Deal Damage
  (bind _output_get (Variables|Default|SetOtherActor OtherActor))
  (Utilities|IsValid _output_get
    (:Is%20Valid
      (Utilities|IsOtherActor!=ProjectileOwner?
        (:Yes
          (CallFunction|ApplyDamage)
          (Actor|DestroyActor))))))

(fn ConstructionScript)

(fn ApplyDamage
  (Game|Damage|ApplyDamage (Variables|Default|GetOtherActor) (Variables|/Game/StealthMaster/Tech/Weapons-Gadgets-Pickups/Gadgets/BP_BaseProjectileGadget.BP_BaseProjectileGadget_C|GetDamage (Variables|Default|GetPlayerGadget)) (Variables|Default|GetOwnerController) self))