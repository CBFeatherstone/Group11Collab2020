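; BP_DistractionProjectile is a gadget projectile that lures with AI noise events and can damage actors it overlaps.
; Overlapping a valid actor other than its owner applies damage and reports a noise at its location.
; On hit, it stops sphere physics simulation to stick in place and starts a looping cooldown timer that repeats the noise with configurable loudness and range, plus a debug print.
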(event Custom|AutoMakeNoise
  ;[1 1 1] Stick to Objects
  (CallFunction|ReportNoiseEvent)
  (Development|PrintString "Hello"))

(event Collision|EventHit
  (params (MyComp :type Primitive%20Component%20Object%20Reference) (Other :type Actor%20Object%20Reference) (OtherComp :type Primitive%20Component%20Object%20Reference) (bSelfMoved :type Boolean) (HitLocation :type Vector :default "0, 0, 0") (HitNormal :type Vector :default "0, 0, 0") (NormalImpulse :type Vector :default "0, 0, 0") (Hit :type Hit%20Result%20Structure%20%28by%20ref%29))
  ;[1 1 1] Stick to Objects
  (Physics|SetSimulatePhysics (Variables|Default|GetSphereCollision) false)
  (Utilities|Time|SetTimerbyEvent (delegate Custom|AutoMakeNoise) (Variables|Default|GetDistractionCooldown) true))

(event EventTick
  (params (DeltaSeconds :type Float%20%28single-precision%29)))

(event Collision|EventActorBeginOverlap
  (params (OtherActor :type Actor%20Object%20Reference))
  ;[1 1 1] Deal Damage
  (bind _output_get (Variables|Default|SetOtherActor OtherActor))
  (Utilities|IsValid _output_get
    (:Is%20Valid
      (Utilities|IsOtherActor!=ProjectileOwner?
        (:Yes
          (CallFunction|ApplyDamage)
          (CallFunction|ReportNoiseEvent))))))

(fn ConstructionScript)

(fn ReportNoiseEvent
  (Class|AISenseHearing|ReportNoiseEvent (Transformation|GetActorLocation) (Variables|Default|GetDistractionLoudness) self (Variables|Default|GetDistractionRange) "None"))