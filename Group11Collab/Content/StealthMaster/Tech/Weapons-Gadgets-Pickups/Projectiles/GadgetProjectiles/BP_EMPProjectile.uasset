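; EMP gadget projectile that explodes on overlap with any valid actor other than its owner.
; EndPlay also triggers the explosion, labelled as the explosion delay, so removal of the actor by any means calls it.
; Exploding reports an AI noise event, fires a radial force impulse, applies full radial damage using the player gadget's damage value, then destroys the projectile.
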(event Custom|Explode
  ;[1 1 1] Explode
  (CallFunction|ReportNoiseEvent)
  (Class|RadialForceComponent|FireImpulse (Variables|Default|GetRadialForce))
  (CallFunction|ApplyRadialDamage)
  (Actor|DestroyActor))

(event EventEndPlay
  (params (EndPlayReason :type EEndPlayReason%20Enum :default "Destroyed"))
  ;[1 1 1] Explosion Delay
  (CallFunction|Explode))

(event EventTick
  (params (DeltaSeconds :type Float%20%28single-precision%29))
  (|CallParentFunction DeltaSeconds) ; This node is disabled and will not be called.\nDrag off pins to build functionality.
)

(event Collision|EventActorBeginOverlap
  (params (OtherActor :type Actor%20Object%20Reference))
  ;[1 1 1] Direct Hit
  (bind _output_get (Variables|Default|SetOtherActor OtherActor))
  (Utilities|IsValid _output_get
    (:Is%20Valid
      (Utilities|IsOtherActor!=ProjectileOwner?
        (:Yes
          (CallFunction|Explode))))))

(fn ConstructionScript
  (|CallParentFunction))

(fn ReportNoiseEvent
  (Class|AISenseHearing|ReportNoiseEvent (Transformation|GetActorLocation) (Variables|Default|GetWeaponLoudness) self (Variables|Default|GetWeaponLoudnessRange) "None"))

(fn ApplyRadialDamage
  (Game|Damage|ApplyRadialDamage (Variables|/Game/StealthMaster/Tech/Weapons-Gadgets-Pickups/Gadgets/BP_BaseProjectileGadget.BP_BaseProjectileGadget_C|GetDamage (Variables|Default|GetPlayerGadget)) (Transformation|GetActorLocation) (Variables|Default|GetExplosionRadius) 0 0 self (Variables|Default|GetOwnerController) true "ECC_Visibility"))