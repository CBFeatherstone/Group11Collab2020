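; Player hamster ball gadget that launches a projectile pawn when used through the Use Gadget interface.
; A CanUseGadget check requires the ready flag and remaining ammo, then each use decrements the amount and re-enables the gadget after a cooldown delay.
; The pawn always spawns at the gadget's fire point, with the gadget as owner and passed in as its HamsterGadget reference.
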(event Custom|UseGadget
  (bind _self self)
  ;[1 1 1] I_Use Gadget
  (Game|SpawnActorfromClass (Variables|Default|GetProjectilePawn) (Transformation|GetWorldTransform (Variables|Default|GetGadgetFirePoint)) "AlwaysSpawn" _self _self 0))

(event EventBeginPlay)

(event Collision|EventActorBeginOverlap
  (params (OtherActor :type Actor%20Object%20Reference)))

(event EventTick
  (params (DeltaSeconds :type Float%20%28single-precision%29)))

(event EventIUseGadget
  ;[1 1 1] I_Use Gadget
  (Utilities|CanUseGadget?
    (:Yes
      (Variables|Default|SetCanUse false)
      (CallFunction|UseGadget)
      (Math|Integer|DecrementInt (Variables|Default|GetAmount)
        (:%20%20
          (Utilities|FlowControl|Delay (Variables|Default|GetCooldown))
          (Variables|Default|SetCanUse true))))))

(fn ConstructionScript)