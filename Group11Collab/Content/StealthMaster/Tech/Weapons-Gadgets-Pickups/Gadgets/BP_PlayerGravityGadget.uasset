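; BP_PlayerGravityGadget is a player gadget that temporarily makes the player character lighter.
; On UseGadget, it gets the character from player controller 0's pawn through an interface message and halves its movement gravity scale.
; After a Duration delay, it sets the scale to a fixed normal value rather than restoring the previous one.
; A CanUseGadget? macro branches on CanUse, but UseGadget does not call it.
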(event Custom|UseGadget
  ;[1 1 1] I_Use Gadget
  (bind _weapontestcharacter (Class|WeaponTestCharacterInterface|IGetWeaponTestCharacter(Message) (Pawn|GetControlledPawn (Game|GetPlayerController 0))))
  (Variables|/Script/Engine.CharacterMovementComponent|SetGravityScale (Variables|/Script/Engine.Character|GetCharacterMovement _weapontestcharacter) 0.5)
  (Utilities|FlowControl|Delay (Variables|Default|GetDuration))
  (Variables|/Script/Engine.CharacterMovementComponent|SetGravityScale (Variables|/Script/Engine.Character|GetCharacterMovement _weapontestcharacter) 1.0))

(event EventBeginPlay
  (|CallParentFunction) ; This node is disabled and will not be called.\nDrag off pins to build functionality.
)

(event Collision|EventActorBeginOverlap
  (params (OtherActor :type Actor%20Object%20Reference))
  (|CallParentFunction OtherActor) ; This node is disabled and will not be called.\nDrag off pins to build functionality.
)

(event EventTick
  (params (DeltaSeconds :type Float%20%28single-precision%29))
  (|CallParentFunction DeltaSeconds) ; This node is disabled and will not be called.\nDrag off pins to build functionality.
)

(fn ConstructionScript
  (|CallParentFunction))