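; Player EMP gadget projectile that detonates on a timer or on any actor overlap.
; BeginPlay waits for the explosion timer, while an overlap triggers the blast immediately.
; Explode fires a radial force impulse, applies full radial damage using the player gadget's damage value with the first player controller as instigator, then destroys the projectile.
; No EMP-specific effect appears in its graphs.
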(event Custom|Explode
  ;[1 1 1] Explode
  (Class|RadialForceComponent|FireImpulse (Variables|Default|GetRadialForce))
  (Game|Damage|ApplyRadialDamage (Variables|/Game/StealthMaster/Tech/Weapons-Gadgets-Pickups/Gadgets/BP_PlayerBaseProjectileGadget.BP_PlayerBaseProjectileGadget_C|GetDamage (Variables|Default|GetPlayerGadget)) (Transformation|GetActorLocation) (Variables|Default|GetExplosionRadius) 0 0 self (Game|GetPlayerController 0) true "ECC_Visibility")
  (Actor|DestroyActor))

(event EventTick
  (params (DeltaSeconds :type Float%20%28single-precision%29))
  (|CallParentFunction DeltaSeconds) ; This node is disabled and will not be called.\nDrag off pins to build functionality.
)

(event EventBeginPlay
  ;[1 1 1] Explosion Delay
  (Utilities|FlowControl|Delay (Variables|Default|GetExplosionTimer))
  (CallFunction|Explode)
  (Actor|DestroyActor))

(event Collision|EventActorBeginOverlap
  (params (OtherActor :type Actor%20Object%20Reference))
  ;[1 1 1] Direct Hit
  (CallFunction|Explode)
  (Actor|DestroyActor))

(fn ConstructionScript
  (|CallParentFunction))