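; Base gadget projectile for the player that damages what it hits.
; On BeginPlay it stores the parent actor of its owner as ProjectileOwner.
; Overlapping any valid actor applies the PlayerGadget damage, credited to player controller 0, then destroys the projectile.
; The overlap does not filter out ProjectileOwner or any other actor.
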(event EventBeginPlay
  ;[1 1 1] Get and Set Owner
  (Variables|Default|SetProjectileOwner (Actor|GetParentActor (Components|GetOwner))))

(event EventTick
  (params (DeltaSeconds :type Float%20%28single-precision%29)))

(event Collision|EventActorBeginOverlap
  (params (OtherActor :type Actor%20Object%20Reference))
  ;[1 1 1] Deal Damage
  (bind _output_get (Variables|Default|SetOtherActor OtherActor))
  (Utilities|IsValid _output_get
    (:Is%20Valid
      (Game|Damage|ApplyDamage (Variables|Default|GetOtherActor) (Variables|/Game/StealthMaster/Tech/Weapons-Gadgets-Pickups/PlayerGadgets/BP_PlayerBasePawnGadget.BP_PlayerBasePawnGadget_C|GetDamage (Variables|Default|GetPlayerGadget)) (Game|GetPlayerController 0) self)
      (Actor|DestroyActor))))

(fn ConstructionScript)