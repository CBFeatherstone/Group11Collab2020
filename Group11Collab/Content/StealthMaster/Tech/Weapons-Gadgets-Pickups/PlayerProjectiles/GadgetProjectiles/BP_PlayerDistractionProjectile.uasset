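; BP_PlayerDistractionProjectile is a player gadget projectile that creates noise events as a distraction.
; Overlapping a valid actor other than the projectile owner applies the gadget's damage and reports noise at the projectile's location with configurable loudness and range.
; On hit, it stops sphere physics to stay in place and starts a looping cooldown timer that reports further noise and prints a debug string.
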(event Custom|AutoMakeNoise
  ;[1 1 1] Stick to Objects
  (Class|AISenseHearing|ReportNoiseEvent "0, 0, 0" 1.0 0 0.0 "None")
  (Development|PrintString "Hello"))

(event Collision|EventHit
  (params (MyComp :type Primitive%20Component%20Object%20Reference) (Other :type Actor%20Object%20Reference) (OtherComp :type Primitive%20Component%20Object%20Reference) (bSelfMoved :type Boolean) (HitLocation :type Vector :default "0, 0, 0") (HitNormal :type Vector :default "0, 0, 0") (NormalImpulse :type Vector :default "0, 0, 0") (Hit :type Hit%20Result%20Structure%20%28by%20ref%29))
  ;[1 1 1] Stick to Objects
  (Physics|SetSimulatePhysics (Variables|Default|GetSphereCollision) false)
  (Utilities|Time|SetTimerbyEvent (delegate Custom|AutoMakeNoise) (Variables|Default|GetDistractionCooldown) true))

(event EventTick
  (params (DeltaSeconds :type Float%20%28single-precision%29)))

(event Collision|EventActorBeginOverlap
  (params (OtherActor :type Actor%20Object%20Reference))
  ;[1 1 1] Deal Damage
  (bind _output_get (Variables|Default|SetOtherActor OtherActor))
  (Utilities|IsValid _output_get
    (:Is%20Valid
      (Utilities|IsOtherActor!=ProjectileOwner?
        (:Yes
          (Game|Damage|ApplyDamage (Variables|Default|GetOtherActor) (Variables|/Game/StealthMaster/Tech/Weapons-Gadgets-Pickups/PlayerGadgets/BP_PlayerBaseProjectileGadget.BP_PlayerBaseProjectileGadget_C|GetDamage (Variables|Default|GetPlayerGadget)) (Game|GetPlayerController 0) self)
          (Class|AISenseHearing|ReportNoiseEvent (Transformation|GetActorLocation) (Variables|Default|GetDistractionLoudness) 0 (Variables|Default|GetDistractionRange) "None"))))))

(fn ConstructionScript)