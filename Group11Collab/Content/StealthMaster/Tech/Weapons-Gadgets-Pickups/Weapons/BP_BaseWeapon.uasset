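; Base weapon for the stealth game, handling semi- and full-auto fire, reloading and ammo.
; Fire input runs through a rate gate and looping timer; multi-projectile weapons use spread line traces, while single-shot weapons spawn projectiles aimed from screen centre or, for AI, near the player.
; Ammo changes go through the inventory, whose change event updates cached counts.
; Every weapon except the pistol reports firing noise.
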(event Custom|AutoFireWeapon
  ;[1 0.2789 0 1 36] Not In Use
  (Variables|NOTINUSE|SetCanFire false)
  (CallFunction|FireWeapon))

(event Custom|FireWeapon
  ;[1 1 1] Firing Logic
  (Utilities|FlowControl|Sequence
    (:then_0
      (if (not (== (Utilities|GetClass self) "/Game/StealthMaster/Tech/Weapons-Gadgets-Pickups/Weapons/BP_PistolWeapon.BP_PistolWeapon_C"))
        (CallFunction|ReportNoiseEvent)))
    (:then_1
      (Utilities|CanWeaponFire?
        (:Yes
          ;;[1 1 1 1 16] Spawn projectiles or line trace
          (for _index (range 1 (Variables|Config|WeaponSettings|GetProjectileCount))
            (Utilities|IsProjectileCount>1?
              (:Yes
                (bind _hitactor (CallFunction|LineTraceforObjects))
                (bind _output (Class|IAI|IGetActor(Message) _hitactor))
                (CallFunction|ApplyDamage _output))
              (:No
                (if (== (Variables|Default|GetFireSound) "/Game/StealthMaster/Art/Sound_Design/Weapons/Pistol/Pistol_Fire_001.Pistol_Fire_001")
                  (Audio|SpawnSoundAttached (Variables|Default|GetFireSound) (Variables|Default|GetWeaponFirePoint) "None" "0, 0, 0" "0, 0, 0" "KeepRelativeOffset" false 1.0 1.0 0.2 "/Game/StealthMaster/Art/Sound_Design/BasicAttenuation.BasicAttenuation" 0)
                  (else
                    (Audio|SpawnSoundAttached (Variables|Default|GetFireSound) (Variables|Default|GetWeaponFirePoint) "None" "0, 0, 0" "0, 0, 0" "KeepRelativeOffset" false 1.0 1.0 0.1 "/Game/StealthMaster/Art/Sound_Design/BasicAttenuation.BasicAttenuation" 0)))
                (CallFunction|SpawnProjectile))))
          (Utilities|IsValid (Variables|Default|GetInventory)
            (:Is%20Valid
              (Default|UpdateAmmo (Variables|Default|GetInventory) (Utilities|GetClass self) -1))))
        (:No
          (Utilities|Time|PauseTimerbyHandle (Variables|Data|Timers|GetAutoFireWeaponTimer)))))))

(event Custom|AutoFireTimer
  ;[1 0.2789 0 1 36] Not In Use
  (bind _returnvalue (Utilities|Time|SetTimerbyEvent (delegate Custom|AutoFireWeapon) (Variables|Config|WeaponSettings|GetRateOfFire) true))
  (bind _output_get (Variables|Data|Timers|SetAutoFireWeaponTimer _returnvalue)))

(event Custom|FullAutoFire
  ;[1 1 1] Firing Logic
  (CallFunction|FireWeapon))

(event Custom|Event_OnAmmoChanged
  (params (Equipment%20Data :type Equipment%20Data%20Structure))
  ;[0.2433 1 0.07432] INIT
  ;;[1 1 1 1 16] Keep track of any changes in ammo via the inventory
  (CallFunction|UpdateAmmo Equipment%20Data))

(event Custom|FullAutoTimer
  ;[1 1 1] Firing Logic
  (bind _returnvalue (Utilities|Time|SetTimerbyEvent (delegate Custom|FullAutoFire) (Variables|Config|WeaponSettings|GetRateOfFire) true))
  (Variables|Data|Timers|SetAutoFireWeaponTimer _returnvalue))

(event Custom|FiringGate
  ;[1 1 1] Firing Logic
  (Utilities|FlowControl|Gate false :!label _label
    (:Exit
      (Utilities|FlowControl|Sequence
        (:then_0
          (goto _label Close))
        (:then_1
          (Utilities|FlowControl|Delay (Variables|Config|WeaponSettings|GetRateOfFire))
          (goto _label Open))
        (:then_2
          (CallFunction|FireWeapon))))))

(event EventIReloadWeapon
  (bind _ammo_clip_max (Variables|Default|GetAmmo_Clip_Max))
  (bind _ammo_clip_cur (Variables|Default|GetAmmo_Clip_Cur))
  (bind _ammo_clip_max_2 (Variables|Default|GetAmmo_Clip_Max))
  (bind _ammo_clip_max_3 (Variables|Default|GetAmmo_Clip_Max))
  (bind _ammo_spare_cur (Variables|Default|GetAmmo_Spare_Cur))
  (bind _ammo_spare_cur_2 (Variables|Default|GetAmmo_Spare_Cur))
  (bind _ammo_clip_max_4 (Variables|Default|GetAmmo_Clip_Max))
  (bind _returnvalue (- _ammo_spare_cur _ammo_clip_max))
  (bind _returnvalue_2 (- _ammo_clip_max_3 _ammo_clip_cur))
  (bind _returnvalue_3 (>= _returnvalue 0))
  (bind _returnvalue_4 (Math|Integer|Absolute(Integer) _returnvalue))
  (bind _returnvalue_5 (== _returnvalue_2 _ammo_clip_max_2))
  (bind _returnvalue_6 (Math|Integer|Clamp(Integer) _returnvalue_4 0 _ammo_spare_cur_2))
  (bind _returnvalue_7 (Math|Integer|SelectInt _ammo_clip_max_4 _returnvalue_6 _returnvalue_3))
  (bind _returnvalue_8 (Math|Integer|Min(Integer) _returnvalue_7 _returnvalue_2))
  (bind _returnvalue_9 (Math|Integer|SelectInt _returnvalue_7 _returnvalue_8 _returnvalue_5))
  ;[1 1 1] Reloading Logic
  ;;[1 1 1] Ensure reloading is nessecary
  (Utilities|IsAmmoClipCur<AmmoClipMax?
    (:Yes
      (Default|UpdateAmmo (Variables|Default|GetInventory) (Utilities|GetClass self) _returnvalue_9 (* _returnvalue_9 -1))
      (Audio|PlaySoundatLocation (Variables|Default|GetReloadSound) (Transformation|GetWorldLocation (Variables|Default|GetWeaponFirePoint)) "0, 0, 0" 1.0 1.0 0.0 0 0 0))))

(event EventIFireReleased
  ;[1 1 1] Firing Input Logic
  (Utilities|Time|PauseTimerbyHandle (Variables|Data|Timers|GetAutoFireWeaponTimer)))

(event EventIStopFiringWeapon
  ;[1 0.2789 0 1 36] Not In Use
  (Utilities|Time|ClearandInvalidateTimerbyHandle (stale Custom|AutoFireTimer _output_get))
  (Utilities|FlowControl|Delay (Variables|Config|WeaponSettings|GetRateOfFire))
  (Variables|NOTINUSE|SetCanFire true))

(event EventIFirePressed
  ;[1 1 1] Firing Input Logic
  (Utilities|CanWeaponFire?
    (:Yes
      (switch Utilities|FlowControl|Switch|SwitchonFireMode (Variables|Config|WeaponSettings|GetFireMode)
        (:NewEnumerator0
          (CallFunction|FiringGate))
        (:NewEnumerator1
          (CallFunction|FiringGate)
          (CallFunction|FullAutoTimer))))))

(event EventIInitWeapon
  (params (Inventory :type Inventory%20Object%20Reference) (EquipmentData :type Equipment%20Data%20Structure))
  ;[0.2433 1 0.07432] INIT
  ;;[1 1 1 1 14] Cache incoming data
  (Variables|Default|SetInventory Inventory)
  (CallFunction|UpdateAmmo EquipmentData)
  ;;[1 1 1 1 16] Keep track of any changes in ammo via the inventory
  (EventDispatchers|BindEventtoOnAmmoChanged (Variables|Default|GetInventory) (delegate Custom|Event_OnAmmoChanged)))

(fn ConstructionScript)

(fn CalcProjectileSpread
  (params (ConeHalfAngleInDegrees :type Float%20%28single-precision%29))
  (bind _weaponfirepoint (Variables|Default|GetWeaponFirePoint))
  (bind _returnvalue (Transformation|GetWorldTransform _weaponfirepoint))
  (return (Math|Transform|MakeTransform (.location _returnvalue) (Math|Rotator|MakeRotfromX (Math|Random|RandomUnitVectorinConeinDegrees (Math|Vector|GetForwardVector _weaponfirepoint) ConeHalfAngleInDegrees)) (.scale _returnvalue))))

(fn UpdateAmmo
  (params (EquipmentData :type Equipment%20Data%20Structure))
  (bind _output_get (LocalVariables|Set_Data EquipmentData))
  (if (== (.Class (Utilities|Struct|BreakEquipment_Data _output_get)) (Utilities|GetClass self))
    (Variables|Default|SetAmmo_Clip_Cur (Utilities|Struct|BreakEquipment_Data (LocalVariables|Get_Data)))
    (Variables|Default|SetAmmo_Spare_Cur (Utilities|Struct|BreakEquipment_Data (LocalVariables|Get_Data)))))

(fn SpawnProjectile
  (bind _returnvalue (Viewport|GetViewportSize))
  (bind _returnvalue_2 (Game|GetPlayerController 0))
  (bind _returnvalue_3 (Game|GetPlayerController 0))
  (bind _self self)
  (bind _self_2 self)
  (bind _weaponfirepoint (Variables|Default|GetWeaponFirePoint))
  (bind _weaponfirepoint_2 (Variables|Default|GetWeaponFirePoint))
  (bind _returnvalue_4 (/ _returnvalue 2.0))
  (bind _returnvalue_5 (Pawn|GetControlledPawn _returnvalue_3))
  (bind _returnvalue_6 (Transformation|GetWorldTransform _weaponfirepoint_2))
  (bind _returnvalue_7 (Transformation|GetWorldLocation _weaponfirepoint))
  (bind (_worldposition _worlddirection) (Class|GameplayStatics|DeprojectScreentoWorld _returnvalue_2 _returnvalue_4))
  (bind _returnvalue_8 (Transformation|GetActorLocation _returnvalue_5))
  (bind _controller (Class|IAI|IGetGenericController(Message) (Actor|GetParentActor)))
  (if (== (Utilities|GetClass _controller) "/Game/StealthMaster/Tech/AI/BP_AIController.BP_AIController_C")
    (bind _outhit (Collision|LineTraceByChannel (Transformation|GetWorldLocation (Variables|Default|GetWeaponFirePoint)) (+ (Math|Vector|MakeVector (.x _returnvalue_8) (.y _returnvalue_8) (.z _returnvalue_8)) (Math|Vector|MakeVector (Math|Random|RandomFloatinRange -25.0 25.0) (Math|Random|RandomFloatinRange -25.0 25.0) (+ 4e+01 (Math|Random|RandomFloatinRange -15.0 15.0)))) "TraceTypeQuery1" false (Utilities|Array|MakeArray (Actor|GetParentActor)) "None"))
    (Game|SpawnActorfromClass (Variables|Config|WeaponSettings|GetProjectile) (Math|Transform|MakeTransform (.location _returnvalue_6) (Math|Rotator|FindLookatRotation (.location _returnvalue_6) (.TraceEnd (Collision|BreakHitResult _outhit))) (.scale _returnvalue_6)) "AlwaysSpawn" _self _self (CallFunction|GetInstigator))
    (else
      (bind _outhit_2 (Collision|LineTraceByChannel _worldposition (+ _worldposition (* _worlddirection 2000)) "TraceTypeQuery1" false (Utilities|Array|MakeArray (Actor|GetParentActor)) "None"))
      (Game|SpawnActorfromClass (Variables|Config|WeaponSettings|GetProjectile) (Math|Transform|MakeTransform _returnvalue_7 (Math|Rotator|FindLookatRotation _returnvalue_7 (.TraceEnd (Collision|BreakHitResult _outhit_2)))) "AlwaysSpawn" _self_2 _self_2 (CallFunction|GetInstigator))))
  (Effects|SpawnEmitterAttached "/Game/StealthMaster/Art/ParticleSystems/JoeD/MuzzleFlash/P_MuzzleFlash.P_MuzzleFlash" (Variables|Default|GetWeaponFirePoint) "None" "0, 0, 0" "0,180.000000, 0" "0.300000,0.300000,0.300000"))

(fn GetInstigator
  (return (Game|GetInstigator (Actor|GetParentActor))))

(fn ReportNoiseEvent
  (Class|AISenseHearing|ReportNoiseEvent (Transformation|GetActorLocation) (Variables|Config|WeaponSettings|GetWeaponLoudness) self (Variables|Config|WeaponSettings|GetWeaponLoudnessRange) "Noise"))

(fn CalcWeaponSpread
  (bind _weaponfirepoint (Variables|Default|GetWeaponFirePoint))
  (return (+ (+ (Transformation|GetWorldLocation _weaponfirepoint) (* (Math|Vector|GetForwardVector _weaponfirepoint) 5e+03)) (Math|Vector|MakeVector (Math|Random|RandomFloatinRange (Variables|Config|WeaponSettings|GetMinTraceSpread) (Variables|Config|WeaponSettings|GetMaxTraceSpread)) (Math|Random|RandomFloatinRange (Variables|Config|WeaponSettings|GetMinTraceSpread) (Variables|Config|WeaponSettings|GetMaxTraceSpread)) (Math|Random|RandomFloatinRange (Variables|Config|WeaponSettings|GetMinTraceSpread) (Variables|Config|WeaponSettings|GetMaxTraceSpread))))))

(fn LineTraceforObjects
  (bind (_outhit _returnvalue) (Collision|LineTraceByChannel (Transformation|GetWorldLocation (Variables|Default|GetWeaponFirePoint)) (CallFunction|CalcWeaponSpread) "TraceTypeQuery1" false (Utilities|Array|MakeArray (Pawn|GetControlledPawn (Game|GetPlayerController 0))) "None"))
  (Effects|SpawnEmitteratLocation "/Game/StarterContent/Particles/P_Explosion.P_Explosion" (.ImpactPoint (Collision|BreakHitResult _outhit)))
  (return (.HitActor (Collision|BreakHitResult _outhit)) _returnvalue))

(fn ApplyDamage
  (params (DamagedActor :type Actor%20Object%20Reference))
  (bind _returnvalue (Game|GetPlayerController 0))
  (Game|Damage|ApplyDamage DamagedActor (Variables|Config|WeaponSettings|GetDamage) _returnvalue (Pawn|GetControlledPawn _returnvalue)))

(fn ICanReload
  (if (and (< (Variables|Default|GetAmmo_Clip_Cur) (Variables|Default|GetAmmo_Clip_Max)) (> (Variables|Default|GetAmmo_Spare_Cur) 0))
    (return true)
    (else
      (return false))))

(fn IGetActive
  (return false))

(fn IGetActor
  (return 0))

(fn IGetAmmo
  (return 0))

(fn IGetCameraObject
  (return 0))

(fn IGetCanTakeDamage
  (return false))

(fn IGetCodeLockNumber
  (return ""))

(fn IGetController
  (return 0))

(fn IGetElevatorLevel
  (return 0))

(fn IGetEnemyCurr/Max
  (return 0 0))

(fn IGetGenericController
  (return 0))

(fn IGetIsDrone
  (return false))

(fn IGetIsEnemy
  (return false))

(fn IGetLookforCover
  (return false))

(fn IGetObjectType
  (return "NewEnumerator3"))

(fn IGetOccupied
  (return false))

(fn IGetOverlappingActors
  (return 0))

(fn IGetPatrol?
  (return false))

(fn IGetPatrolLoop?
  (return false))

(fn IGetPatrolPathActor
  (return 0))

(fn IGetPatrolPathPoints
  (return 0))

(fn IGetPawnReference
  (return 0))

(fn IGetPlayerSector
  (return 0))

(fn IGetPlaystyle
  (return "NewEnumerator0"))

(fn IGetRange
  (return 0.0))

(fn IGetSceneComponentHumanoid
  (return 0))

(fn IGetSector
  (params (Input :type Integer))
  (return 0))

(fn IGetSectorIndex
  (return 0))

(fn IGetSectorSize
  (return "0, 0, 0"))

(fn IGetStance
  (return "NewEnumerator0"))

(fn IGetStunned?
  (return false))

(fn IGetVisibilityGM
  (return 0.0 false false false))

(fn IGetVisibilitySL
  (return 0.0))

(fn IGetWaitTime
  (return 0.0))

(fn IReturnDetectedVariables
  (return 0.0 0.0))

(fn ISectorGetContainedEnemies
  (return 0))