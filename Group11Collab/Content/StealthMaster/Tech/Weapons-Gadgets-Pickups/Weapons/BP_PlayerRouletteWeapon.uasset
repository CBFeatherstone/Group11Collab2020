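; Player roulette weapon that takes on the stats of a random pistol, shotgun, assault rifle or revolver with every shot.
; FiringGate throttles shots with a gate and delay, rolling a new type before each FireWeapon call, so the cooldown uses the previous roll's RateOfFire.
; Each roll copies stats from that weapon Blueprint's class defaults, sets the fire mode and uses a fixed reload speed.
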(event Custom|ShotgunRoll
  ;[1 1 1] Roll A Weapon Type
  (CallFunction|SetShotgunStats))

(event Custom|PistolRoll
  ;[1 1 1] Roll A Weapon Type
  (CallFunction|SetPistolStats))

(event Custom|AssaultRifleRoll
  ;[1 1 1] Roll A Weapon Type
  (CallFunction|SetAssaultRifleStats))

(event Custom|RevolverRoll
  ;[1 1 1] Roll A Weapon Type
  (CallFunction|SetRevolverStats))

(event EventBeginPlay
  (|CallParentFunction) ; This node is disabled and will not be called.\nDrag off pins to build functionality.
)

(event Collision|EventActorBeginOverlap
  (params (OtherActor :type Actor%20Object%20Reference))
  (|CallParentFunction OtherActor) ; This node is disabled and will not be called.\nDrag off pins to build functionality.
)

(event EventTick
  (params (DeltaSeconds :type Float%20%28single-precision%29))
  (|CallParentFunction DeltaSeconds) ; This node is disabled and will not be called.\nDrag off pins to build functionality.
)

(event EventIRouletteRoll
  (bind _weapontypes (Variables|Default|GetWeaponTypes))
  ;[1 1 1] Roll A Weapon Type
  (switch Utilities|FlowControl|Switch|SwitchonWeaponType (Utilities|Array|Get(acopy) _weapontypes (Math|Random|RandomInteger (Utilities|Array|Length _weapontypes)))
    (:NewEnumerator0
      (CallFunction|PistolRoll)
      (Development|PrintString "Pistol Rolled"))
    (:NewEnumerator1
      (CallFunction|ShotgunRoll)
      (Development|PrintString "Shotgun Rolled"))
    (:NewEnumerator2
      (CallFunction|AssaultRifleRoll)
      (Development|PrintString "Assault Rifle Rolled"))
    (:NewEnumerator4
      (CallFunction|RevolverRoll)
      (Development|PrintString "Revolver Rolled"))))

(event EventFiringGate
  (Utilities|FlowControl|Gate false :!label _label
    (:Exit
      (Utilities|FlowControl|Sequence
        (:then_0
          (goto _label Close))
        (:then_1
          (Utilities|FlowControl|Delay (Variables|Default|GetRateOfFire))
          (goto _label Open))
        (:then_2
          (CallFunction|IRouletteRoll)
          (CallFunction|FireWeapon))))))

(fn ConstructionScript
  (|CallParentFunction))

(fn SetPistolStats
  (bind (_damage _rateoffire _projectilespread _projectilecount) (Utilities|GetClassDefaults "/Game/StealthMaster/Tech/Weapons-Gadgets-Pickups/Weapons/BP_PistolWeapon.BP_PistolWeapon_C"))
  (Variables|Default|SetDamage _damage)
  (Variables|Default|SetRateOfFire _rateoffire)
  (Variables|Default|SetProjectileSpread _projectilespread)
  (Variables|Default|SetReloadSpeed 2.0)
  (Variables|Default|SetProjectileCount _projectilecount)
  (Variables|Default|SetFireMode "NewEnumerator0")
  (return))

(fn SetShotgunStats
  (bind (_damage _rateoffire _mintracespread _maxtracespread _projectilecount) (Utilities|GetClassDefaults "/Game/StealthMaster/Tech/Weapons-Gadgets-Pickups/Weapons/BP_ShotgunWeapon.BP_ShotgunWeapon_C"))
  (Variables|Default|SetDamage _damage)
  (Variables|Default|SetRateOfFire _rateoffire)
  (Variables|Default|SetMinTraceSpread _mintracespread)
  (Variables|Default|SetMaxTraceSpread _maxtracespread)
  (Variables|Default|SetReloadSpeed 2.0)
  (Variables|Default|SetProjectileCount _projectilecount)
  (Variables|Default|SetFireMode "NewEnumerator0")
  (return))

(fn SetAssaultRifleStats
  (bind (_damage _rateoffire _projectilespread _projectilecount) (Utilities|GetClassDefaults "/Game/StealthMaster/Tech/Weapons-Gadgets-Pickups/Weapons/BP_AssaultRifleWeapon.BP_AssaultRifleWeapon_C"))
  (Variables|Default|SetDamage _damage)
  (Variables|Default|SetRateOfFire _rateoffire)
  (Variables|Default|SetProjectileSpread _projectilespread)
  (Variables|Default|SetReloadSpeed 2.0)
  (Variables|Default|SetProjectileCount _projectilecount)
  (Variables|Default|SetFireMode "NewEnumerator1")
  (return))

(fn SetRevolverStats
  (bind (_damage _rateoffire _projectilespread _projectilecount) (Utilities|GetClassDefaults "/Game/StealthMaster/Tech/Weapons-Gadgets-Pickups/Weapons/BP_RevolverWeapon.BP_RevolverWeapon_C"))
  (Variables|Default|SetDamage _damage)
  (Variables|Default|SetRateOfFire _rateoffire)
  (Variables|Default|SetProjectileSpread _projectilespread)
  (Variables|Default|SetReloadSpeed 2.0)
  (Variables|Default|SetProjectileCount _projectilecount)
  (Variables|Default|SetFireMode "NewEnumerator0")
  (return))