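; Base hitscan weapon actor that handles firing, automatic fire, ammo and reloading through fire pressed/released events.
; Each shot reports AI noise, then runs spread-randomized object line traces per projectile, applying damage credited to player controller 0.
; A looping timer drives automatic fire, while delays gate draw, refire and the automatic reload when ammo empties.
; Ammo drops per projectile, traces draw debug lines, and the ammo getter returns zero.
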(event Custom|AutoFireWeapon
  ;[1 1 1] Spawn Line Trace
  (Variables|Default|SetCanFire false)
  (CallFunction|FireWeapon))

(event Custom|FireWeapon
  ;[1 1 1] Spawn Line Trace
  (CallFunction|ReportNoiseEvent)
  (for _index (range 0 (Variables|Default|GetProjectileCount))
    (bind _outhit (CallFunction|LineTraceforObjects))
    (Math|Integer|DecrementInt (Variables|Default|GetAmmo)
      (:%20%20
        (CallFunction|ApplyDamage _outhit)
        (Utilities|IsAmmo<=0?
          (:Yes
            (Variables|Default|SetCanFire false)
            (Utilities|Time|ClearandInvalidateTimerbyHandle (Variables|Default|GetAutoFireWeaponTimer))
            (Utilities|FlowControl|Delay (Variables|Default|GetReloadSpeed))
            (Variables|Default|SetAmmo (Variables|Default|GetMaxAmmo))
            (Variables|Default|SetCanFire true)))))))

(event Custom|AutoFireTimer
  ;[1 1 1] Spawn Line Trace
  (bind _returnvalue (Utilities|Time|SetTimerbyEvent (delegate Custom|AutoFireWeapon) (Variables|Default|GetFireSpeed) true))
  (bind _output_get (Variables|Default|SetAutoFireWeaponTimer _returnvalue)))

(event EventIFireReleased
  ;[1 1 1] Spawn Line Trace
  (Utilities|Time|ClearandInvalidateTimerbyHandle (stale Custom|AutoFireTimer _output_get))
  (Utilities|FlowControl|Delay (Variables|Default|GetFireSpeed))
  (Variables|Default|SetCanFire true))

(event Collision|EventActorBeginOverlap
  (params (OtherActor :type Actor%20Object%20Reference)))

(event EventTick
  (params (DeltaSeconds :type Float%20%28single-precision%29)))

(event EventIFirePressed
  ;[1 1 1] Spawn Line Trace
  (Utilities|CanWeaponFire?
    (:Yes
      (Variables|Default|SetCanFire false)
      (CallFunction|FireWeapon)
      (Utilities|IsWeaponAutomatic?
        (:Yes
          (CallFunction|AutoFireTimer))))))

(event EventBeginPlay
  ;[1 1 1] Draw Weapon Firing Delay
  (Variables|Default|SetCanFire false)
  (Utilities|FlowControl|Delay (Variables|Default|GetFireSpeed))
  (Variables|Default|SetCanFire true))

(fn ConstructionScript)

(fn CalcWeaponFirePoint,RangeandSpread
  (bind _weaponfirepoint (Variables|Default|GetWeaponFirePoint))
  (bind _returnvalue (Transformation|GetWorldLocation _weaponfirepoint))
  (return _returnvalue (+ (+ _returnvalue (* (Math|Vector|GetForwardVector _weaponfirepoint) (Variables|Default|GetRange))) (Math|Vector|MakeVector (Math|Random|RandomFloatinRange (Variables|Default|GetMinSpread) (Variables|Default|GetMaxSpread)) (Math|Random|RandomFloatinRange (Variables|Default|GetMinSpread) (Variables|Default|GetMaxSpread)) (Math|Random|RandomFloatinRange (Variables|Default|GetMinSpread) (Variables|Default|GetMaxSpread))))))

(fn HitResult
  (params (Hit :type Hit%20Result%20Structure%20%28by%20ref%29))
  (return (.HitActor (Collision|BreakHitResult Hit))))

(fn ApplyDamage
  (params (Hit :type Hit%20Result%20Structure%20%28by%20ref%29))
  (Game|Damage|ApplyDamage (CallFunction|HitResult Hit) (Variables|Default|GetDamage) (Game|GetPlayerController 0) self))

(fn LineTraceforObjects
  (bind (_start _end) (CallFunction|CalcWeaponFirePoint,RangeandSpread))
  (bind (_outhit _returnvalue) (Collision|LineTraceForObjects _start _end (Utilities|Array|MakeArray "ObjectTypeQuery7") false 0 "ForDuration"))
  (return _outhit _returnvalue))

(fn ReportNoiseEvent
  (Class|AISenseHearing|ReportNoiseEvent (Transformation|GetActorLocation) (Variables|Default|GetWeaponLoudness) self (Variables|Default|GetWeaponLoudnessRange) "None"))

(fn IGetAmmo
  (return 0))