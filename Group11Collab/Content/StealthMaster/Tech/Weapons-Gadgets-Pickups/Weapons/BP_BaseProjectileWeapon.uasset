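; Base weapon Blueprint for StealthMaster that handles semi-auto and full-auto firing, ammo and reloading, and reports a noise event on each fire attempt.
; A delayed gate limits trigger presses, and a looping timer drives automatic fire.
; Single shots spawn projectiles within a spread cone, while multi-projectile weapons apply damage through randomly spread line traces.
; Ammo changes go through the Inventory, whose change event refreshes the cached counts.
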(event Custom|AutoFireWeapon
  ;[1 0.2789 0 1 36] Not In Use
  (Variables|NOTINUSE|SetCanFire false)
  (CallFunction|FireWeapon))

(event Custom|FireWeapon
  (bind _returnvalue (Game|GetPlayerController 0))
  (bind _projectilecount (Variables|Config|WeaponSettings|GetProjectileCount))
  (bind _inventory (Variables|Default|GetInventory))
  ;[1 1 1] Firing Logic
  (CallFunction|ReportNoiseEvent)
  (Utilities|CanWeaponFire?
    (:Yes
      ;;[1 1 1 1 16] Spawn bullets
      (for _index (range 1 _projectilecount)
        (if (> _projectilecount 1)
          (bind _end (CallFunction|CalcWeaponSpread))
          (bind _outhit (Collision|LineTraceForObjects (Transformation|GetWorldLocation (Variables|Default|GetWeaponFirePoint)) _end (Utilities|Array|MakeArray "ObjectTypeQuery7") false (Utilities|Array|MakeArray (Pawn|GetControlledPawn (Game|GetPlayerController 0))) "ForDuration"))
          (bind _output (Class|IAI|IGetActor(Message) (.HitActor (Collision|BreakHitResult _outhit))))
          (Game|Damage|ApplyDamage _output 1e+01 _returnvalue (Pawn|GetControlledPawn _returnvalue))
          (else
            (CallFunction|SpawnProjectile))))
      (Utilities|IsValid _inventory
        (:Is%20Valid
          (Default|UpdateAmmo _inventory (Utilities|GetClass self) -1))))
    (:No
      (Utilities|Time|PauseTimerbyHandle (Variables|Data|Timers|GetAutoFireWeaponTimer)))))

(event Custom|AutoFireTimer
  ;[1 0.2789 0 1 36] Not In Use
  (bind _returnvalue (Utilities|Time|SetTimerbyEvent (delegate Custom|AutoFireWeapon) (Variables|Config|WeaponSettings|GetRateOfFire) true))
  (bind _output_get (Variables|Data|Timers|SetAutoFireWeaponTimer _returnvalue)))

(event Custom|FullAutoFire
  ;[1 1 1] Firing Logic
  (CallFunction|FireWeapon))

(event Custom|Event_OnAmmoChanged
  (params (Equipment%20Data :type Equipment%20Data%20Structure))
  ;[0.2433 1 0.07432] INIT
  ;;[1 1 1 1 16] Keep track of any changes in ammo via the inventory
  (CallFunction|UpdateAmmo Equipment%20Data))

(event Custom|FullAutoTimer
  ;[1 1 1] Firing Logic
  (bind _returnvalue (Utilities|Time|SetTimerbyEvent (delegate Custom|FullAutoFire) (Variables|Config|WeaponSettings|GetRateOfFire) true))
  (Variables|Data|Timers|SetAutoFireWeaponTimer _returnvalue))

(event Custom|FiringGate
  ;[1 1 1] Firing Logic
  (Utilities|FlowControl|Gate false :!label _label
    (:Exit
      (Utilities|FlowControl|Sequence
        (:then_0
          (goto _label Close))
        (:then_1
          (Utilities|FlowControl|Delay (Variables|Config|WeaponSettings|GetRateOfFire))
          (goto _label Open))
        (:then_2
          (CallFunction|FireWeapon))))))

(event EventIReloadWeapon
  (bind _ammo_clip_max (Variables|Default|GetAmmo_Clip_Max))
  (bind _ammo_clip_cur (Variables|Default|GetAmmo_Clip_Cur))
  (bind _ammo_clip_max_2 (Variables|Default|GetAmmo_Clip_Max))
  (bind _ammo_clip_max_3 (Variables|Default|GetAmmo_Clip_Max))
  (bind _ammo_spare_cur (Variables|Default|GetAmmo_Spare_Cur))
  (bind _ammo_spare_cur_2 (Variables|Default|GetAmmo_Spare_Cur))
  (bind _ammo_clip_max_4 (Variables|Default|GetAmmo_Clip_Max))
  (bind _returnvalue (- _ammo_spare_cur _ammo_clip_max))
  (bind _returnvalue_2 (- _ammo_clip_max_3 _ammo_clip_cur))
  (bind _returnvalue_3 (>= _returnvalue 0))
  (bind _returnvalue_4 (Math|Integer|Absolute(Integer) _returnvalue))
  (bind _returnvalue_5 (== _returnvalue_2 _ammo_clip_max_2))
  (bind _returnvalue_6 (Math|Integer|Clamp(Integer) _returnvalue_4 0 _ammo_spare_cur_2))
  (bind _returnvalue_7 (Math|Integer|SelectInt _ammo_clip_max_4 _returnvalue_6 _returnvalue_3))
  (bind _returnvalue_8 (Math|Integer|Min(Integer) _returnvalue_7 _returnvalue_2))
  (bind _returnvalue_9 (Math|Integer|SelectInt _returnvalue_7 _returnvalue_8 _returnvalue_5))
  ;[1 1 1] Reloading Logic
  ;;[1 1 1] Ensure reloading is nessecary
  (Utilities|IsAmmoClipCur<AmmoClipMax?
    (:Yes
      (Default|UpdateAmmo (Variables|Default|GetInventory) (Utilities|GetClass self) _returnvalue_9 (* _returnvalue_9 -1)))))

(event EventIFireReleased
  ;[1 1 1] Firing Input Logic
  (Utilities|Time|PauseTimerbyHandle (Variables|Data|Timers|GetAutoFireWeaponTimer)))

(event EventIStopFiringWeapon
  ;[1 0.2789 0 1 36] Not In Use
  (Utilities|Time|ClearandInvalidateTimerbyHandle (stale Custom|AutoFireTimer _output_get))
  (Utilities|FlowControl|Delay (Variables|Config|WeaponSettings|GetRateOfFire))
  (Variables|NOTINUSE|SetCanFire true))

(event EventIFirePressed
  ;[1 1 1] Firing Input Logic
  (Utilities|CanWeaponFire?
    (:Yes
      (switch Utilities|FlowControl|Switch|SwitchonFireMode (Variables|Config|WeaponSettings|GetFireMode)
        (:NewEnumerator0
          (CallFunction|FiringGate))
        (:NewEnumerator1
          (CallFunction|FiringGate)
          (CallFunction|FullAutoTimer))))))

(event EventIInitWeapon
  (params (Inventory :type Inventory%20Object%20Reference) (EquipmentData :type Equipment%20Data%20Structure))
  ;[0.2433 1 0.07432] INIT
  ;;[1 1 1 1 14] Cache incoming data
  (Variables|Default|SetInventory Inventory)
  (CallFunction|UpdateAmmo EquipmentData)
  ;;[1 1 1 1 16] Keep track of any changes in ammo via the inventory
  (EventDispatchers|BindEventtoOnAmmoChanged (Variables|Default|GetInventory) (delegate Custom|Event_OnAmmoChanged)))

(fn ConstructionScript)

(fn CalcProjectileSpread
  (params (ConeHalfAngleInDegrees :type Float%20%28single-precision%29))
  (bind _weaponfirepoint (Variables|Default|GetWeaponFirePoint))
  (bind _returnvalue (Transformation|GetWorldTransform _weaponfirepoint))
  (return (Math|Transform|MakeTransform (.location _returnvalue) (Math|Rotator|MakeRotfromX (Math|Random|RandomUnitVectorinConeinDegrees (Math|Vector|GetForwardVector _weaponfirepoint) ConeHalfAngleInDegrees)) (.scale _returnvalue))))

(fn UpdateAmmo
  (params (EquipmentData :type Equipment%20Data%20Structure))
  (LocalVariables|Set_Data EquipmentData)
  (Variables|Default|SetAmmo_Clip_Cur (Utilities|Struct|BreakEquipment_Data (LocalVariables|Get_Data)))
  (Variables|Default|SetAmmo_Spare_Cur (Utilities|Struct|BreakEquipment_Data (LocalVariables|Get_Data))))

(fn SpawnProjectile
  (bind _self self)
  (Game|SpawnActorfromClass (Variables|Config|WeaponSettings|GetProjectile) (CallFunction|CalcProjectileSpread (Variables|Config|WeaponSettings|GetBulletSpread)) "AlwaysSpawn" _self _self (CallFunction|GetInstigator)))

(fn GetInstigator
  (return (Game|GetInstigator (Actor|GetParentActor))))

(fn ReportNoiseEvent
  (Class|AISenseHearing|ReportNoiseEvent (Transformation|GetActorLocation) (Variables|Config|WeaponSettings|GetWeaponLoudness) self (Variables|Config|WeaponSettings|GetWeaponLoudnessRange) "Noise"))

(fn CalcWeaponSpread
  (bind _weaponfirepoint (Variables|Default|GetWeaponFirePoint))
  (return (+ (+ (Transformation|GetWorldLocation _weaponfirepoint) (* (Math|Vector|GetForwardVector _weaponfirepoint) 5e+03)) (Math|Vector|MakeVector (Math|Random|RandomFloatinRange (Variables|Default|GetMinSpread) (Variables|Default|GetMaxSpread)) (Math|Random|RandomFloatinRange (Variables|Default|GetMinSpread) (Variables|Default|GetMaxSpread)) (Math|Random|RandomFloatinRange (Variables|Default|GetMinSpread) (Variables|Default|GetMaxSpread))))))

(fn IGetActive
  (return false))

(fn IGetActor
  (return 0))

(fn IGetAmmo
  (return 0))

(fn IGetCameraObject
  (return 0))

(fn IGetCodeLockNumber
  (return ""))

(fn IGetController
  (return 0))

(fn IGetElevatorLevel
  (return 0))

(fn IGetEnemyCurr/Max
  (return 0 0))

(fn IGetIsDrone
  (return false))

(fn IGetIsEnemy
  (return false))

(fn IGetLookforCover
  (return false))

(fn IGetObjectType
  (return "NewEnumerator3"))

(fn IGetOccupied
  (return false))

(fn IGetOverlappingActors
  (return 0))

(fn IGetPatrol?
  (return false))

(fn IGetPatrolLoop?
  (return false))

(fn IGetPatrolPathActor
  (return 0))

(fn IGetPatrolPathPoints
  (return 0))

(fn IGetPawnReference
  (return 0))

(fn IGetPlayerSector
  (return 0))

(fn IGetPlaystyle
  (return "NewEnumerator0"))

(fn IGetRange
  (return 0.0))

(fn IGetSector
  (params (Input :type Integer))
  (return 0))

(fn IGetSectorIndex
  (return 0))

(fn IGetSectorSize
  (return "0, 0, 0"))

(fn IGetStance
  (return "NewEnumerator0"))

(fn IGetStunned?
  (return false))

(fn IGetVisibilityGM
  (return 0.0 false false false))

(fn IGetWaitTime
  (return 0.0))

(fn IReturnDetectedVariables
  (return 0.0 0.0))

(fn ISectorGetContainedEnemies
  (return 0))