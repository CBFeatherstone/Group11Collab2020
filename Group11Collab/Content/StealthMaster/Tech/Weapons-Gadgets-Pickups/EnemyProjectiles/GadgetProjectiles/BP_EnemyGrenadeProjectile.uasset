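; BP_EnemyGrenadeProjectile is an enemy gadget grenade projectile that explodes on overlap or when it leaves play, such as when its time runs out.
; Each explosion fires a radial force impulse and deals full radial damage from EnemyGadget within ExplosionRadius, ignoring the owner's parent actor.
; An overlap explodes and then destroys the actor, so EndPlay triggers a second explosion.
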(event Custom|Explode
  ;[1 1 1] Explode
  (Class|RadialForceComponent|FireImpulse (Variables|Default|GetRadialForce))
  (Game|Damage|ApplyRadialDamage (Variables|/Game/StealthMaster/Tech/Weapons-Gadgets-Pickups/EnemyGadgets/BP_EnemyGrenadeGadget.BP_EnemyGrenadeGadget_C|GetDamage (Variables|Default|GetEnemyGadget)) (Transformation|GetActorLocation) (Variables|Default|GetExplosionRadius) 0 (Utilities|Array|MakeArray (Actor|GetParentActor (Components|GetOwner))) self 0 true "ECC_Visibility"))

(event EventEndPlay
  (params (EndPlayReason :type EEndPlayReason%20Enum :default "Destroyed"))
  ;[1 1 1] Time Runs Out
  (CallFunction|Explode))

(event EventTick
  (params (DeltaSeconds :type Float%20%28single-precision%29))
  (|CallParentFunction DeltaSeconds) ; This node is disabled and will not be called.\nDrag off pins to build functionality.
)

(event Collision|EventActorBeginOverlap
  (params (OtherActor :type Actor%20Object%20Reference))
  ;[1 1 1] Direct Hit
  (CallFunction|Explode)
  (Actor|DestroyActor))

(fn ConstructionScript
  (|CallParentFunction))