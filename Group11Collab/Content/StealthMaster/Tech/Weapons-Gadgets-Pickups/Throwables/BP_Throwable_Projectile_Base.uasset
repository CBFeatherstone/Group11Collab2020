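; BP_Throwable_Projectile_Base is a base projectile for throwables, launching a static mesh as a physics object.
; Interface-style events supply the mesh and throw power.
; ThrowMesh enables physics simulation and applies an impulse along the mesh's forward vector, scaled by that power.
; After a short delay it switches the mesh to a blocking collision profile, so full collision starts only after launch.
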(event Custom|ThrowMesh
  (Physics|SetSimulatePhysics (Variables|Default|GetStaticMesh) true)
  (Physics|AddImpulse (Variables|Default|GetStaticMesh) (* (Math|Vector|GetForwardVector (Variables|Default|GetStaticMesh)) (Variables|Default|GetThrow%20Power)) "None" false)
  (Utilities|FlowControl|Delay 0.2)
  (Collision|SetCollisionProfileName (Variables|Default|GetStaticMesh) "BlockAllDynamic" :!class /Script/Engine.PrimitiveComponent))

(event EventISetThrowPower
  (params (InThrowPower :type Float%20%28single-precision%29))
  (Variables|Default|SetThrow%20Power InThrowPower))

(event EventISetMesh
  (params (InMesh :type Static%20Mesh%20Object%20Reference))
  (Components|StaticMesh|SetStaticMesh (Variables|Default|GetStaticMesh) InMesh))

(fn ConstructionScript)