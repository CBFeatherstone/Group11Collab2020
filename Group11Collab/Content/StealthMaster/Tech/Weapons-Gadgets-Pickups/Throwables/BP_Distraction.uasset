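; BP_Distraction is a throwable gadget that makes a noise to distract AI after a countdown.
; DetonationTimer starts a looping one-second timer, and TimeLeft decrements Timer with debug prints until it runs out.
; Distract then plays a 2D mouse squeak, reports a "Noise"-tagged noise event at the mesh location for AI hearing, and destroys the actor after a short delay.
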(event Custom|Distract
  (Audio|PlaySound2D "/Game/StealthMaster/Tech/UI/Prototype/Hamsterball/Mouse_Squeak_Solo.Mouse_Squeak_Solo" 0.5 (Variables|Default|GetPitchMultiplier) 0.0 0 self)
  (Class|AISenseHearing|ReportNoiseEvent (Transformation|GetWorldLocation (Variables|Default|GetStaticMesh)) 1.0 self 5e+02 "Noise")
  (Utilities|FlowControl|Delay 0.3)
  (Actor|DestroyActor))

(event Custom|DetonationTimer
  (bind _returnvalue (Utilities|Time|SetTimerbyEvent (EventDispatchers|CreateEvent :!event Custom|TimeLeft) 1.0 true))
  (Variables|Default|SetGrenadeTimer _returnvalue))

(event Custom|TimeLeft
  (Math|Float|DecrementFloat (Variables|Default|GetTimer)
    (:%20%20
      (if (<= (Variables|Default|GetTimer) 0.0)
        (Development|PrintString "No time left explode!!!!" true true "(R=0.209480,G=1.000000,B=0.161475,A=1.000000)")
        (Utilities|Time|ClearandInvalidateTimerbyHandle (Variables|Default|GetGrenadeTimer))
        (CallFunction|Distract)
        (else
          (Development|PrintString "Timer Still left" true true "(R=1.000000,G=0.000000,B=0.009362,A=1.000000)"))))))

(fn ConstructionScript
  (|CallParentFunction))