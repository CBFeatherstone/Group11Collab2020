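; Base Blueprint for throwable items, launched through the IThrow event.
; On throw it enables physics on its static mesh and applies a velocity-change impulse along the parent actor's parent component forward plus up vectors, scaled by ThrowPower.
; After a short delay the mesh switches to BlockAllDynamic collision.
; Disconnected nodes hold an unused trajectory preview using projectile path prediction and spline meshes.
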(event EventIThrow
  (bind _returnvalue (Actor|GetParentActor))
  (bind _returnvalue_2 (Class|Actor|GetParentComponent _returnvalue))
  (Physics|SetSimulatePhysics (Variables|Default|GetStaticMesh) true)
  (Physics|AddImpulse (Variables|Default|GetStaticMesh) (* (+ (Math|Vector|GetForwardVector _returnvalue_2) (Math|Vector|GetUpVector _returnvalue_2)) (Variables|Default|GetThrowPower)) "None" true)
  (Utilities|FlowControl|Delay 0.2)
  (Collision|SetCollisionProfileName (Variables|Default|GetStaticMesh) "BlockAllDynamic" :!class /Script/Engine.PrimitiveComponent))

(fn ConstructionScript)