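; BP_BeeBriefCase_REAL is a throwable bee briefcase gadget that damages actors around it.
; It is a child Blueprint whose construction script only runs the parent's.
; DamageEnemy checks that the other actor is not the player's controlled pawn, then applies small, full-strength radial damage around the static mesh.
; The player pawn is excluded from the damage, and the player controller is credited as instigator.
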(fn ConstructionScript
  (|CallParentFunction))

(fn DamageEnemy
  (Variables|Default|SetPlayerActor (Pawn|GetControlledPawn (Variables|Default|GetPlayerController)))
  (if (!= (Variables|Default|GetOtherActor) (Variables|Default|GetPlayerActor))
    (Game|Damage|ApplyRadialDamage 2.0 (Transformation|GetWorldLocation (Variables|Default|GetStaticMesh)) 1e+02 0 (Utilities|Array|MakeArray (Variables|Default|GetPlayerActor)) self (Variables|Default|GetPlayerController) true "ECC_Visibility")))