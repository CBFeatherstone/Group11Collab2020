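; Base throwable gadget that, on throw, spawns a projectile matching its type (frag, EMP, water, distraction) from its parent component.
; Ammo is cached from the inventory and refreshed by its change event; each spawn decrements the clip there.
; A gate and delay enforce rate of fire, and an interface message passes mesh and launch vector to the projectile.
; Disconnected spline-based trajectory prediction code remains but never runs.
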(event Custom|Event_OnAmmoChanged
  (params (Equipment%20Data :type Equipment%20Data%20Structure))
  ;[0 1 0.05329] Init
  ;;[1 1 1 1 16] Keep track of any changes in ammo via the inventory
  (CallFunction|UpdateAmmo Equipment%20Data))

(event Custom|SpawnProjectile
  (Utilities|HasAmmo
    (:Yes
      (bind _returnvalue (Game|SpawnActorfromClass (.AsActor (Utilities|Casting|CastToActorClass (Utilities|Select :Index (Variables|Default|GetThowableType) :NewEnumerator0 "/Game/StealthMaster/Tech/Weapons-Gadgets-Pickups/Throwables/ThrowableProjectiles/Projectiles/BP_Frag_Projectile.BP_Frag_Projectile_C" :NewEnumerator1 "/Game/StealthMaster/Tech/Weapons-Gadgets-Pickups/Throwables/ThrowableProjectiles/Projectiles/BP_EMP_Projectile.BP_EMP_Projectile_C" :NewEnumerator2 "/Game/StealthMaster/Tech/Weapons-Gadgets-Pickups/Throwables/ThrowableProjectiles/Projectiles/BP_WaterGrenade_Projectile.BP_WaterGrenade_Projectile_C" :NewEnumerator3 0 :NewEnumerator4 "/Game/StealthMaster/Tech/Weapons-Gadgets-Pickups/Throwables/ThrowableProjectiles/Projectiles/BP_Distraction_Projectile.BP_Distraction_Projectile_C"))) (Transformation|GetWorldTransform (Class|Actor|GetParentComponent)) "AlwaysSpawn" (Actor|GetParentActor) 0))
      (Class|BPIThorwableProjectile|IInitThrowableProjectile(Message) _returnvalue (Variables|Default|GetThrowPower) (Variables|/Script/Engine.StaticMeshComponent|GetStaticMesh (Variables|Default|GetStaticMesh)) (* (Math|Vector|GetForwardVector (Class|Actor|GetParentComponent)) (Variables|Default|GetThrowPower)))
      (Collision|LineTraceByChannel "0, 0, 0" "0, 0, 0" "TraceTypeQuery1" false 0 "ForDuration" true "(R=1.000000,G=0.000000,B=0.000000,A=1.000000)" "(R=0.000000,G=1.000000,B=0.000000,A=1.000000)" 1e+01)
      (Utilities|IsValid (Variables|Default|GetInventory)
        (:Is%20Valid
          (Default|UpdateAmmo (Variables|Default|GetInventory) (Utilities|GetClass self) -1))))))

(event EventIInitThrowable
  (params (Inventory :type Inventory%20Object%20Reference) (Equipment%20Data :type Equipment%20Data%20Structure))
  ;[0 1 0.05329] Init
  (Variables|Default|SetInventory Inventory)
  (CallFunction|UpdateAmmo Equipment%20Data)
  (Variables|Default|SetThrowableClass (.Class (Utilities|Struct|BreakEquipment_Data Equipment%20Data)))
  ;;[1 1 1 1 16] Keep track of any changes in ammo via the inventory
  (EventDispatchers|BindEventtoOnAmmoChanged (Variables|Default|GetInventory) (delegate Custom|Event_OnAmmoChanged)))

(event EventIThrow
  (Utilities|HasAmmo
    (:Yes
      (Utilities|FlowControl|Gate false :!label _label
        (:Exit
          (Utilities|FlowControl|Sequence
            (:then_0
              (goto _label Close))
            (:then_1
              (Utilities|FlowControl|Delay (Variables|Default|GetRateOfFire))
              (goto _label Open))
            (:then_2
              (CallFunction|SpawnProjectile))))))))

(fn ConstructionScript)

(fn UpdateAmmo
  (params (Equipment%20Data :type Equipment%20Data%20Structure))
  (LocalVariables|Set_Data Equipment%20Data)
  (Variables|Default|SetAmmo_Clip_Cur (Utilities|Struct|BreakEquipment_Data (LocalVariables|Get_Data)))
  (Variables|Default|SetAmmo_Spare_Cur (Utilities|Struct|BreakEquipment_Data (LocalVariables|Get_Data))))