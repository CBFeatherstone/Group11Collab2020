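; Frag grenade projectile that explodes on a countdown fuse and damages the area around it.
; BeginPlay starts a looping one-second timer, and TimeLeft decrements Timer until it runs out, then clears the timer and calls Explode.
; Explode spawns an explosion particle at the mesh, plays a 2D sound, applies radial damage credited to the first player controller, then destroys the actor.
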(event Custom|Explode
  (Effects|SpawnEmitteratLocation "/Game/TemplateContent/StarterContent/Particles/P_Explosion.P_Explosion" (Transformation|GetWorldLocation (Variables|Default|GetStaticMesh)) "0, 0, 0" "5.000000,5.000000,5.000000")
  (Audio|PlaySound2D "/Game/StarterContent/Audio/Explosion01.Explosion01" 0.1 1.0 0.0 0 self)
  (Game|Damage|ApplyRadialDamage 1e+02 (Transformation|GetWorldLocation (Variables|Default|GetStaticMesh)) 5e+02 0 0 self (Game|GetPlayerController 0) false "ECC_Camera")
  (Actor|DestroyActor) ; The Jank is real
)

(event Custom|DetonationTimer
  (bind _returnvalue (Utilities|Time|SetTimerbyEvent (EventDispatchers|CreateEvent :!event Custom|TimeLeft) 1.0 true))
  (Variables|Default|SetGrenadeTimer _returnvalue))

(event Custom|TimeLeft
  (Math|Float|DecrementFloat (Variables|Default|GetTimer)
    (:%20%20
      (if (<= (Variables|Default|GetTimer) 0.0)
        (Development|PrintString "No time left explode!!!!" true true "(R=0.209480,G=1.000000,B=0.161475,A=1.000000)")
        (Utilities|Time|ClearandInvalidateTimerbyHandle (Variables|Default|GetGrenadeTimer))
        (CallFunction|Explode)
        (else
          (Development|PrintString "Timer Still left" true true "(R=1.000000,G=0.000000,B=0.009362,A=1.000000)"))))))

(event EventBeginPlay
  (CallFunction|DetonationTimer))

(fn ConstructionScript
  (|CallParentFunction))