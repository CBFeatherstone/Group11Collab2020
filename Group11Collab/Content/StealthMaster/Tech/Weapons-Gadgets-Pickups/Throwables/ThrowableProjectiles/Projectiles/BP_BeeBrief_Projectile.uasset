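; Throwable briefcase projectile that opens after landing and damages non-player actors, apparently with a bee swarm.
; A looping timer runs sideways traces from the case meshes, counting hits until a threshold shows it has settled.
; It then rotates the lid open while growing the overlap sphere, finally activating particles.
; Overlaps start a repeating timer applying radial damage around the case, ignoring the player; ending overlap stops it.
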(event OnComponentBeginOverlap(Sphere)
  (params (OverlappedComponent :type Primitive%20Component%20Object%20Reference) (OtherActor :type Actor%20Object%20Reference) (OtherComp :type Primitive%20Component%20Object%20Reference) (OtherBodyIndex :type Integer) (bFromSweep :type Boolean) (SweepResult :type Hit%20Result%20Structure%20%28by%20ref%29))
  (if (Variables|Default|GetCanDamage)
    (Variables|Default|SetOtherActor OtherActor)
    (CallFunction|DamageTimer)))

(event OnComponentEndOverlap(Sphere)
  (params (OverlappedComponent :type Primitive%20Component%20Object%20Reference) (OtherActor :type Actor%20Object%20Reference) (OtherComp :type Primitive%20Component%20Object%20Reference) (OtherBodyIndex :type Integer))
  (Variables|Default|SetOtherActor OtherActor)
  (Utilities|Time|ClearandInvalidateTimerbyHandle (Variables|Default|GetTimer)))

(event Custom|DamageTimer
  (bind _returnvalue (Utilities|Time|SetTimerbyFunctionName 0 "DamageEnemy" 0.1 true))
  (Variables|Default|SetTimer _returnvalue))

(event Custom|OpenBriefCase
  (bind _sphere (Variables|Default|GetSphere))
  (if (> (Variables|Default|GetRotationLimit) 0)
    (Math|Integer|DecrementInt (Variables|Default|GetRotationLimit)
      (:%20%20
        (Transformation|AddLocalRotation (Variables|Default|GetStaticMesh1) "0.000000,0.000000,-1.000000" false false)
        (Components|Sphere|SetSphereRadius _sphere (+ (Variables|/Script/Engine.SphereComponent|GetSphereRadius _sphere) 4e+01) true)))
    (else
      (Utilities|Time|ClearandInvalidateTimerbyHandle (Variables|Default|GetOpenBriefCaseTimer))
      (Variables|Default|SetCanDamage true)
      (Components|Activation|Activate (Variables|Default|GetParticleSystem) false))))

(event Custom|TimerEvent
  (bind _returnvalue (Utilities|Time|SetTimerbyEvent (EventDispatchers|CreateEvent :!event Custom|CheckIfCalm) 0.1 true))
  (Variables|Default|SetCheckIfCalmTimer _returnvalue))

(event Custom|CheckIfCalm
  (bind _staticmesh (Variables|Default|GetStaticMesh))
  (bind _staticmesh1 (Variables|Default|GetStaticMesh1))
  (bind _returnvalue (Transformation|GetWorldLocation _staticmesh))
  (bind _returnvalue_2 (Transformation|GetWorldLocation _staticmesh1))
  (if (> (Variables|Default|GetCounter) 20)
    (Utilities|Time|ClearandInvalidateTimerbyHandle (Variables|Default|GetCheckIfCalmTimer))
    (CallFunction|OpenBriefCaseEvent)
    (else
      (bind _returnvalue_3 (Collision|LineTraceByChannel _returnvalue_2 (+ _returnvalue_2 (* (Math|Vector|GetRightVector _staticmesh1) 1e+02)) "TraceTypeQuery1" false 0 "None"))
      (if _returnvalue_3
        (Math|Integer|IncrementInt (Variables|Default|GetCounter))
        (else
          (bind _returnvalue_4 (Collision|LineTraceByChannel _returnvalue (+ _returnvalue (* (Math|Vector|GetRightVector _staticmesh) -1e+02)) "TraceTypeQuery1" false 0 "None"))
          (if _returnvalue_4
            (Math|Integer|IncrementInt (Variables|Default|GetCounter))))))))

(event Custom|OpenBriefCaseEvent
  (Variables|Default|SetCanDamage true)
  (bind _returnvalue (Utilities|Time|SetTimerbyEvent (EventDispatchers|CreateEvent :!event Custom|OpenBriefCase) 0.05 true))
  (Variables|Default|SetOpenBriefCaseTimer _returnvalue))

(event EventBeginPlay
  (Variables|Default|SetPlayerController (Game|GetPlayerController 0))
  (CallFunction|TimerEvent))

(fn ConstructionScript
  (|CallParentFunction))

(fn DamageEnemy
  (Variables|Default|SetPlayerActor (Pawn|GetControlledPawn (Variables|Default|GetPlayerController)))
  (if (!= (Variables|Default|GetOtherActor) (Variables|Default|GetPlayerActor))
    (Game|Damage|ApplyRadialDamage 2.0 (Transformation|GetWorldLocation (Variables|Default|GetStaticMesh)) 1e+02 0 (Utilities|Array|MakeArray (Variables|Default|GetPlayerActor)) self (Variables|Default|GetPlayerController) true "ECC_Visibility")))