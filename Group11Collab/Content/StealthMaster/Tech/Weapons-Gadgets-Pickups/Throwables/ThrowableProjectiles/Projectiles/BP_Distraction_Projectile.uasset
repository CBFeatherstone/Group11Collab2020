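; BP_Distraction_Projectile is a throwable gadget that creates a noisy, moving distraction after a countdown.
; On BeginPlay a looping one-second timer counts down to activation, then starts a second looping timer for a ten-second distraction phase.
; Each distraction tick plays a random sound, reports a noise event, randomly jolts and rotates the mesh, and spawns a small explosion effect at a random arrow component.
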(event Custom|Distract
  (Math|Float|DecrementFloat (Variables|Default|GetTimer)
    (:%20%20
      (if (<= (Variables|Default|GetTimer) 0.0)
        (Development|PrintString "Trying my best to get this working")
        (Utilities|Time|ClearandInvalidateTimerbyHandle (Variables|Default|GetDistractionTimerHandle))
        (else
          (Audio|PlaySound2D (Utilities|Array|Get(acopy) (Variables|Default|GetSounds) (Math|Random|RandomIntegerinRange 0 (Variables|Default|GetLengthOfSoundArray))) 0.5 (Variables|Default|GetPitchMultiplier) 0.0 0 self)
          (Class|AISenseHearing|ReportNoiseEvent (Transformation|GetWorldLocation (Variables|Default|GetStaticMesh)) 1.0 self 3e+03 "Noise")
          (Physics|AddImpulse (Variables|Default|GetStaticMesh) (* (Math|Vector|MakeVector (Math|Random|RandomFloatinRange -25.0 25.0) (Math|Random|RandomFloatinRange -25.0 25.0) (Math|Random|RandomFloatinRange 0.0 25.0)) 1e+01) "None" true)
          (Transformation|AddLocalRotation (Variables|Default|GetStaticMesh) (Math|Rotator|MakeRotator (Math|Random|RandomFloatinRange 5e+01 1e+02) (Math|Random|RandomFloatinRange 5e+01 1e+02) (Math|Random|RandomFloatinRange 5e+01 1e+02)) false false)
          (Effects|SpawnEmitteratLocation "/Game/StarterContent/Particles/P_Explosion.P_Explosion" (Transformation|GetWorldLocation (Utilities|Array|Get(acopy) (Variables|Default|GetDirectionalArrowsArray) (Math|Random|RandomIntegerinRange 0 2))) "0, 0, 0" "0.100000,0.100000,0.100000"))))))

(event Custom|DetonationTimer
  (bind _returnvalue (Utilities|Time|SetTimerbyEvent (EventDispatchers|CreateEvent :!event Custom|TimeLeft) 1.0 true))
  (Variables|Default|SetGrenadeTimer _returnvalue))

(event Custom|TimeLeft
  (Math|Float|DecrementFloat (Variables|Default|GetTimer)
    (:%20%20
      (if (<= (Variables|Default|GetTimer) 0.0)
        (Development|PrintString "No time left explode!!!!" true true "(R=0.209480,G=1.000000,B=0.161475,A=1.000000)")
        (Utilities|Time|ClearandInvalidateTimerbyHandle (Variables|Default|GetGrenadeTimer))
        (Variables|Default|SetLengthOfSoundArray (Utilities|Array|Length (Variables|Default|GetSounds)))
        (Variables|Default|SetTimer 1e+01)
        (bind _returnvalue (Utilities|Time|SetTimerbyEvent (EventDispatchers|CreateEvent :!event Custom|Distract) 1.0 true))
        (Variables|Default|SetDistractionTimerHandle _returnvalue)
        (else
          (Development|PrintString "Timer Still left" true true "(R=1.000000,G=0.000000,B=0.009362,A=1.000000)"))))))

(event EventBeginPlay
  (Variables|Default|SetDirectionalArrowsArray (Utilities|Array|MakeArray (Variables|Default|GetDirectionalArrow0) (Variables|Default|GetDirectionalArrow1) (Variables|Default|GetDirectionalArrow2)))
  (CallFunction|DetonationTimer))

(fn ConstructionScript
  (|CallParentFunction))