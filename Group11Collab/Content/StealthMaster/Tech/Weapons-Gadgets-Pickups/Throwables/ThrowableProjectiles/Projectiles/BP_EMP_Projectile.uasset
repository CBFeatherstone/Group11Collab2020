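; EMP grenade projectile that detonates after a countdown to stun enemy drones.
; BeginPlay starts a looping half-second timer that decrements Timer and, at zero, clears itself and spawns the EMP blast emitter at the mesh.
; StunEnemy then scans the Sphere's overlaps for exact drone class matches, sends a stun interface message to OtherActor per match, and destroys the projectile.
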(event Custom|StunEnemy
  (bind _output_get (Variables|Default|SetOverlappingActors (Collision|GetOverlappingActors (Variables|Default|GetSphere) "/Game/StealthMaster/Tech/Enemies/New_Enemy_Drone_Class.New_Enemy_Drone_Class_C" :!class /Script/Engine.PrimitiveComponent)))
  (for _array_element _output_get
    (if (== (Utilities|GetClass _array_element) "/Game/StealthMaster/Tech/Enemies/New_Enemy_Drone_Class.New_Enemy_Drone_Class_C")
      (Class|EnemyInterface|IStunEnemy(Message) (Variables|Default|GetOtherActor))
      (Development|PrintString "STUNNED")))
  (Actor|DestroyActor))

(event Custom|DetonationTimer
  (bind _returnvalue (Utilities|Time|SetTimerbyEvent (EventDispatchers|CreateEvent :!event Custom|TimeLeft) 0.5 true))
  (Variables|Default|SetGrenadeTimer _returnvalue))

(event Custom|TimeLeft
  (Math|Float|DecrementFloat (Variables|Default|GetTimer)
    (:%20%20
      (if (<= (Variables|Default|GetTimer) 0.0)
        (Development|PrintString "No time left explode!!!!" true true "(R=0.209480,G=1.000000,B=0.161475,A=1.000000)")
        (Utilities|Time|ClearandInvalidateTimerbyHandle (Variables|Default|GetGrenadeTimer))
        (Effects|SpawnEmitteratLocation "/Game/StealthMaster/Art/ParticleSystems/LewisS/EMP_Blast.EMP_Blast" (Transformation|GetWorldLocation (Variables|Default|GetStaticMesh)))
        (CallFunction|StunEnemy)
        (else
          (Development|PrintString "Timer Still left" true true "(R=1.000000,G=0.000000,B=0.009362,A=1.000000)"))))))

(event EventBeginPlay
  (CallFunction|DetonationTimer))

(fn ConstructionScript
  (|CallParentFunction))