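; Base Blueprint for throwable projectiles, a physics-driven static mesh launched by an impulse.
; An interface init event receives the mesh, throw power and throw vector, then triggers the throw immediately.
; The throw enables physics simulation, applies the vector as a mass-dependent impulse, and switches collision to BlockAllDynamic after a short delay.
; Throw power is stored but not used in this graph.
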(event Custom|ThrowMesh
  (Physics|SetSimulatePhysics (Variables|Default|GetStaticMesh) true)
  (Physics|AddImpulse (Variables|Default|GetStaticMesh) (Variables|Default|GetThrow%20Vector) "None" false)
  (Utilities|FlowControl|Delay 0.2)
  (Collision|SetCollisionProfileName (Variables|Default|GetStaticMesh) "BlockAllDynamic" :!class /Script/Engine.PrimitiveComponent))

(event EventIInitThrowableProjectile
  (params (InThrowPower :type Float%20%28single-precision%29) (InMesh :type Static%20Mesh%20Object%20Reference) (ThrowVector :type Vector :default "0, 0, 0"))
  (Variables|Default|SetThrow%20Power InThrowPower)
  (Components|StaticMesh|SetStaticMesh (Variables|Default|GetStaticMesh) InMesh)
  (Variables|Default|SetThrow%20Vector ThrowVector)
  (CallFunction|ThrowMesh))

(fn ConstructionScript)