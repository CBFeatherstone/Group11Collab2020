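; BP_BeeBriefCase is a StealthMaster throwable gadget that repeatedly damages actors around it.
; Sphere overlap starts a looping timer that calls DamageEnemy, and end overlap clears it.
; Each tick applies full radial damage at the mesh, ignoring and crediting the player, unless the last overlap event's actor is the player.
; It tracks only one actor and one timer handle, so multiple overlaps overwrite each other.
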(event OnComponentBeginOverlap(Sphere)
  (params (OverlappedComponent :type Primitive%20Component%20Object%20Reference) (OtherActor :type Actor%20Object%20Reference) (OtherComp :type Primitive%20Component%20Object%20Reference) (OtherBodyIndex :type Integer) (bFromSweep :type Boolean) (SweepResult :type Hit%20Result%20Structure%20%28by%20ref%29))
  (Variables|Default|SetOtherActor OtherActor)
  (CallFunction|DamageTimer))

(event OnComponentEndOverlap(Sphere)
  (params (OverlappedComponent :type Primitive%20Component%20Object%20Reference) (OtherActor :type Actor%20Object%20Reference) (OtherComp :type Primitive%20Component%20Object%20Reference) (OtherBodyIndex :type Integer))
  (Variables|Default|SetOtherActor OtherActor)
  (Utilities|Time|ClearandInvalidateTimerbyHandle (Variables|Default|GetTimer)))

(event Custom|DamageTimer
  (bind _returnvalue (Utilities|Time|SetTimerbyFunctionName 0 "DamageEnemy" 0.1 true))
  (Variables|Default|SetTimer _returnvalue))

(event EventBeginPlay
  (Variables|Default|SetPlayerController (Game|GetPlayerController 0)))

(fn ConstructionScript
  (|CallParentFunction))

(fn DamageEnemy
  (Variables|Default|SetPlayerActor (Pawn|GetControlledPawn (Variables|Default|GetPlayerController)))
  (if (!= (Variables|Default|GetOtherActor) (Variables|Default|GetPlayerActor))
    (Game|Damage|ApplyRadialDamage 2.0 (Transformation|GetWorldLocation (Variables|Default|GetStaticMesh)) 1e+02 0 (Utilities|Array|MakeArray (Variables|Default|GetPlayerActor)) self (Variables|Default|GetPlayerController) true "ECC_Visibility")))