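; Enemy grenade gadget that fires a projectile when triggered through the gadget-use interface.
; A CanUse flag gates each use, then a delay of the Cooldown duration restores it.
; SpawnProjectile always spawns the configured Projectile class at the GadgetFirePoint transform, setting the gadget as owner and passing it in as the projectile's EnemyGadget.
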(event Custom|UseGadget
  ;[1 1 1] I_Use Gadget
  (CallFunction|SpawnProjectile))

(event EventBeginPlay
  (|CallParentFunction) ; This node is disabled and will not be called.\nDrag off pins to build functionality.
)

(event Collision|EventActorBeginOverlap
  (params (OtherActor :type Actor%20Object%20Reference))
  (|CallParentFunction OtherActor) ; This node is disabled and will not be called.\nDrag off pins to build functionality.
)

(event EventTick
  (params (DeltaSeconds :type Float%20%28single-precision%29))
  (|CallParentFunction DeltaSeconds) ; This node is disabled and will not be called.\nDrag off pins to build functionality.
)

(event EventIUseGadget
  ;[1 1 1] I_Use Gadget
  (Utilities|CanUseGadget?
    (:Yes
      (Variables|Default|SetCanUse false)
      (CallFunction|UseGadget)
      (Utilities|FlowControl|Delay (Variables|Default|GetCooldown))
      (Variables|Default|SetCanUse true))))

(fn ConstructionScript
  (|CallParentFunction))

(fn SpawnProjectile
  (bind _self self)
  (Game|SpawnActorfromClass (Variables|Default|GetProjectile) (Transformation|GetWorldTransform (Variables|Default|GetGadgetFirePoint)) "AlwaysSpawn" _self _self 0))