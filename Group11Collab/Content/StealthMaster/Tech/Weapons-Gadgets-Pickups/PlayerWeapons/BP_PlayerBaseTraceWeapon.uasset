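; Base player hitscan weapon, fired and stopped through interface events, with fire delay, ammo and optional automatic fire.
; Each shot runs line traces per projectile from the fire point with random endpoint spread and debug drawing, applying damage on hits.
; A looping timer drives automatic fire, and releasing fire clears it and re-enables firing after a delay.
; Ammo drops per trace, but the empty check and timed reload run only after a hit.
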(event Custom|AutoFireWeapon
  ;[1 1 1] Spawn Line Trace
  (Variables|Default|SetCanFire false)
  (CallFunction|FireWeapon))

(event Custom|FireWeapon
  (bind (_start _end) (CallFunction|CalcWeaponFirePoint,RangeandSpread))
  ;[1 1 1] Spawn Line Trace
  (for _index (range 0 (Variables|Default|GetProjectileCount))
    (bind (_outhit _returnvalue) (Collision|LineTraceForObjects _start _end (Utilities|Array|MakeArray "ObjectTypeQuery7") false 0 "ForDuration"))
    (Math|Integer|DecrementInt (Variables|Default|GetAmmo)
      (:%20%20
        (if _returnvalue
          (Game|Damage|ApplyDamage (CallFunction|HitResult _outhit) (Variables|Default|GetDamage) (Game|GetPlayerController 0) 0)
          (Utilities|IsAmmo<=0?
            (:Yes
              (Variables|Default|SetCanFire false)
              (Utilities|Time|ClearandInvalidateTimerbyHandle (Variables|Default|GetAutoFireWeaponTimer))
              (Utilities|FlowControl|Delay (Variables|Default|GetReloadSpeed))
              (Variables|Default|SetAmmo (Variables|Default|GetMaxAmmo))
              (Variables|Default|SetCanFire true))))))))

(event Custom|AutoFireTimer
  ;[1 1 1] Spawn Line Trace
  (bind _returnvalue (Utilities|Time|SetTimerbyEvent (delegate Custom|AutoFireWeapon) (Variables|Default|GetFireSpeed) true))
  (bind _output_get (Variables|Default|SetAutoFireWeaponTimer _returnvalue)))

(event Collision|EventActorBeginOverlap
  (params (OtherActor :type Actor%20Object%20Reference)))

(event EventTick
  (params (DeltaSeconds :type Float%20%28single-precision%29)))

(event EventIStopFiringWeapon
  ;[1 1 1] Spawn Line Trace
  (Utilities|Time|ClearandInvalidateTimerbyHandle (stale Custom|AutoFireTimer _output_get))
  (Utilities|FlowControl|Delay (Variables|Default|GetFireSpeed))
  (Variables|Default|SetCanFire true))

(event EventIFireWeapon
  ;[1 1 1] Spawn Line Trace
  (Utilities|CanWeaponFire?
    (:Yes
      (Variables|Default|SetCanFire false)
      (CallFunction|FireWeapon)
      (Utilities|IsWeaponAutomatic?
        (:Yes
          (CallFunction|AutoFireTimer))))))

(event EventBeginPlay
  ;[1 1 1] Draw Weapon Firing Delay
  (Variables|Default|SetCanFire false)
  (Utilities|FlowControl|Delay (Variables|Default|GetFireSpeed))
  (Variables|Default|SetCanFire true))

(fn ConstructionScript)

(fn CalcWeaponFirePoint,RangeandSpread
  (bind _weaponfirepoint (Variables|Default|GetWeaponFirePoint))
  (bind _returnvalue (Transformation|GetWorldLocation _weaponfirepoint))
  (return _returnvalue (+ (+ _returnvalue (* (Math|Vector|GetForwardVector _weaponfirepoint) (Variables|Default|GetRange))) (Math|Vector|MakeVector (Math|Random|RandomFloatinRange (Variables|Default|GetMinSpread) (Variables|Default|GetMaxSpread)) (Math|Random|RandomFloatinRange (Variables|Default|GetMinSpread) (Variables|Default|GetMaxSpread)) (Math|Random|RandomFloatinRange (Variables|Default|GetMinSpread) (Variables|Default|GetMaxSpread))))))

(fn HitResult
  (params (Hit :type Hit%20Result%20Structure%20%28by%20ref%29))
  (return (.HitActor (Collision|BreakHitResult Hit))))