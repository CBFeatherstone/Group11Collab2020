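; BP_PlayerRouletteWeapon is a player weapon that randomly becomes a pistol, shotgun, assault rifle or revolver when rolled.
; The IRouletteRoll event picks a random WeaponTypes entry, fires that type's roll event and prints the result.
; Each roll event calls a setter that overwrites the shared damage, fire rate, spread, reload, ammo, projectile count and automatic-fire variables with hard-coded stats.
; The file contains no firing logic, only the stat selection.
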(event Custom|ShotgunRoll
  ;[1 1 1] Roll A Weapon Type
  (CallFunction|SetShotgunStats))

(event Custom|PistolRoll
  ;[1 1 1] Roll A Weapon Type
  (CallFunction|SetPistolStats))

(event Custom|AssaultRifleRoll
  ;[1 1 1] Roll A Weapon Type
  (CallFunction|SetAssaultRifleStats))

(event Custom|RevolverRoll
  ;[1 1 1] Roll A Weapon Type
  (CallFunction|SetRevolverStats))

(event EventBeginPlay
  (|CallParentFunction) ; This node is disabled and will not be called.\nDrag off pins to build functionality.
)

(event Collision|EventActorBeginOverlap
  (params (OtherActor :type Actor%20Object%20Reference))
  (|CallParentFunction OtherActor) ; This node is disabled and will not be called.\nDrag off pins to build functionality.
)

(event EventTick
  (params (DeltaSeconds :type Float%20%28single-precision%29))
  (|CallParentFunction DeltaSeconds) ; This node is disabled and will not be called.\nDrag off pins to build functionality.
)

(event EventIRouletteRoll
  (bind _weapontypes (Variables|Default|GetWeaponTypes))
  ;[1 1 1] Roll A Weapon Type
  (switch Utilities|FlowControl|Switch|SwitchonWeaponType (Utilities|Array|Get(acopy) _weapontypes (Math|Random|RandomInteger (Utilities|Array|Length _weapontypes)))
    (:NewEnumerator0
      (CallFunction|PistolRoll)
      (Development|PrintString "Pistol Rolled"))
    (:NewEnumerator1
      (CallFunction|ShotgunRoll)
      (Development|PrintString "Shotgun Rolled"))
    (:NewEnumerator2
      (CallFunction|AssaultRifleRoll)
      (Development|PrintString "Assault Rifle Rolled"))
    (:NewEnumerator4
      (CallFunction|RevolverRoll)
      (Development|PrintString "Revolver Rolled"))))

(fn ConstructionScript
  (|CallParentFunction))

(fn SetPistolStats
  (Variables|Default|SetDamage 9.0)
  (Variables|Default|SetFireSpeed 0.5)
  (Variables|Default|SetSpread 4.0)
  (Variables|Default|SetReloadSpeed 2.0)
  (Variables|Default|SetMaxAmmo 12)
  (Variables|Default|SetProjectileCount 0)
  (Variables|Default|SetIsAutomatic false)
  (return))

(fn SetShotgunStats
  (Variables|Default|SetDamage 3.0)
  (Variables|Default|SetFireSpeed 2.0)
  (Variables|Default|SetSpread 15.0)
  (Variables|Default|SetReloadSpeed 3.0)
  (Variables|Default|SetMaxAmmo 6)
  (Variables|Default|SetProjectileCount 19)
  (Variables|Default|SetIsAutomatic false)
  (return))

(fn SetAssaultRifleStats
  (Variables|Default|SetDamage 3.0)
  (Variables|Default|SetFireSpeed 0.1)
  (Variables|Default|SetSpread 5.0)
  (Variables|Default|SetReloadSpeed 2.0)
  (Variables|Default|SetMaxAmmo 30)
  (Variables|Default|SetProjectileCount 0)
  (Variables|Default|SetIsAutomatic true)
  (return))

(fn SetRevolverStats
  (Variables|Default|SetDamage 25.0)
  (Variables|Default|SetFireSpeed 1.0)
  (Variables|Default|SetSpread 2.0)
  (Variables|Default|SetReloadSpeed 3.0)
  (Variables|Default|SetMaxAmmo 6)
  (Variables|Default|SetProjectileCount 0)
  (Variables|Default|SetIsAutomatic false)
  (return))