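; BP_PlayerAssaultRifleWeapon is the player's assault rifle weapon, with its events and construction script left to the parent class.
; Its one piece of custom logic calculates projectile spread, returning a spawn transform at the WeaponFirePoint's location and scale.
; The rotation comes from a random direction within a cone around the fire point's forward vector, sized by the half-angle passed in.
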(event EventBeginPlay
  (|CallParentFunction) ; This node is disabled and will not be called.\nDrag off pins to build functionality.
)

(event Collision|EventActorBeginOverlap
  (params (OtherActor :type Actor%20Object%20Reference))
  (|CallParentFunction OtherActor) ; This node is disabled and will not be called.\nDrag off pins to build functionality.
)

(event EventTick
  (params (DeltaSeconds :type Float%20%28single-precision%29))
  (|CallParentFunction DeltaSeconds) ; This node is disabled and will not be called.\nDrag off pins to build functionality.
)

(fn ConstructionScript
  (|CallParentFunction))

(fn CalcProjectileSpread0
  (params (ConeHalfAngleInDegrees1 :type Float%20%28single-precision%29))
  (bind _weaponfirepoint (Variables|Default|GetWeaponFirePoint))
  (bind _returnvalue (Transformation|GetWorldTransform _weaponfirepoint))
  (return (Math|Transform|MakeTransform (.location _returnvalue) (Math|Rotator|MakeRotfromX (Math|Random|RandomUnitVectorinConeinDegrees (Math|Vector|GetForwardVector _weaponfirepoint) ConeHalfAngleInDegrees1)) (.scale _returnvalue))))