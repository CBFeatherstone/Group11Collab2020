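; Player gadget Blueprint for distractions in StealthMaster that launches a projectile when used.
; The UseGadget event spawns the Projectile class at the GadgetFirePoint transform, always spawning regardless of collision.
; The gadget sets itself as the projectile's owner and passes itself in as PlayerGadget.
; It holds no distraction logic of its own beyond that spawn.
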(event EventBeginPlay
  (|CallParentFunction) ; This node is disabled and will not be called.\nDrag off pins to build functionality.
)

(event Collision|EventActorBeginOverlap
  (params (OtherActor :type Actor%20Object%20Reference))
  (|CallParentFunction OtherActor) ; This node is disabled and will not be called.\nDrag off pins to build functionality.
)

(event EventTick
  (params (DeltaSeconds :type Float%20%28single-precision%29))
  (|CallParentFunction DeltaSeconds) ; This node is disabled and will not be called.\nDrag off pins to build functionality.
)

(event EventUseGadget
  (bind _self self)
  ;[1 1 1] Use Gadget
  (Game|SpawnActorfromClass (.Projectile (Variables|Default|GetProjectile)) (Transformation|GetWorldTransform (Variables|Default|GetGadgetFirePoint)) "AlwaysSpawn" _self _self 0))

(fn ConstructionScript
  (|CallParentFunction))