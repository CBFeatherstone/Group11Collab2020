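; BP_GadgetPickup is a world pickup that gives a gadget class to whatever actor overlaps it.
; A text render component shows the gadget's class display name, set on BeginPlay.
; On overlap it passes the gadget to the other actor through an interface message, with no type check.
; It then hides itself, disables sphere collision, and respawns on a timer after RespawnTime.
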(event Custom|RespawnPickup
  ;[1 1 1] Despawn & Respawn Pickup
  (Collision|SetCollisionEnabled (Variables|Default|GetSphere) "QueryOnly")
  (Rendering|SetActorHiddenInGame false))

(event Custom|DespawnPickup
  ;[1 1 1] Despawn & Respawn Pickup
  (Collision|SetCollisionEnabled (Variables|Default|GetSphere) "NoCollision")
  (Rendering|SetActorHiddenInGame true))

(event EventBeginPlay
  ;[1 1 1] Set Text
  (Rendering|Components|TextRender|SetText (Variables|Default|GetTextRender) (Utilities|Text|ToText(String) (Utilities|GetClassDisplayName (Variables|Default|GetGadget)))))

(event EventTick
  (params (DeltaSeconds :type Float%20%28single-precision%29)))

(event Collision|EventActorBeginOverlap
  (params (OtherActor :type Actor%20Object%20Reference))
  ;[1 1 1] Actor overlap
  (Class|PickupInterface|IPickedUpGadget(Message) OtherActor (Variables|Default|GetGadget))
  (CallFunction|DespawnPickup)
  (Utilities|Time|SetTimerbyFunctionName 0 "RespawnPickup" (Variables|Default|GetRespawnTime)))

(fn ConstructionScript)