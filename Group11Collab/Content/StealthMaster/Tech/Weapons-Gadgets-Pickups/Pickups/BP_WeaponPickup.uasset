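; BP_WeaponPickup is a respawning pickup that offers its Weapon to any actor that overlaps it.
; On overlap it sends the IPickedUpWeaponMessage interface message to the other actor, without checking whether that actor handles it.
; It then hides itself and disables its Sphere collision, and a timer set to RespawnTime restores visibility and query-only collision.
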(event Custom|RespawnPickup
  ;[1 1 1] Despawn & Respawn Pickup
  (Collision|SetCollisionEnabled (Variables|Default|GetSphere) "QueryOnly")
  (Rendering|SetActorHiddenInGame false))

(event Custom|DespawnPickup
  ;[1 1 1] Despawn & Respawn Pickup
  (Collision|SetCollisionEnabled (Variables|Default|GetSphere) "NoCollision")
  (Rendering|SetActorHiddenInGame true))

(event Collision|EventActorBeginOverlap
  (params (OtherActor :type Actor%20Object%20Reference))
  ;[1 1 1] Actor overlap
  (Class|PickupInterface|IPickedUpWeapon(Message) OtherActor (Variables|Default|GetWeapon))
  (CallFunction|DespawnPickup)
  (Utilities|Time|SetTimerbyFunctionName 0 "RespawnPickup" (Variables|Default|GetRespawnTime)))

(fn ConstructionScript)