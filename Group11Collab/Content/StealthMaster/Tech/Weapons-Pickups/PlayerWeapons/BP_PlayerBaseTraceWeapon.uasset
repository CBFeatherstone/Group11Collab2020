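; BP_PlayerBaseTraceWeapon is a base player weapon that deals hitscan damage when fired.
; Its IFireWeapon event runs a debug-drawn line trace on the Visibility channel and applies WeaponDamage to the hit actor, with player controller 0 as instigator.
; CalcWeaponFirePointAndRange supplies the trace endpoints, projecting WeaponRange forward from the WeaponFirePoint component.
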(event EventBeginPlay)

(event Collision|EventActorBeginOverlap
  (params (OtherActor :type Actor%20Object%20Reference)))

(event EventTick
  (params (DeltaSeconds :type Float%20%28single-precision%29)))

(event EventIFireWeapon
  (bind (_start _end) (CallFunction|CalcWeaponFirePointandRange))
  ;[1 1 1] Spawn Line Trace
  (bind (_outhit _returnvalue) (Collision|LineTraceByChannel _start _end "TraceTypeQuery1" false 0 "ForDuration"))
  (if _returnvalue
    (Game|Damage|ApplyDamage (.HitActor (Collision|BreakHitResult _outhit)) (Variables|Default|GetWeaponDamage) (Game|GetPlayerController 0) 0)))

(fn ConstructionScript)

(fn CalcWeaponFirePointandRange
  (bind _weaponfirepoint (Variables|Default|GetWeaponFirePoint))
  (bind _returnvalue (Transformation|GetWorldLocation _weaponfirepoint))
  (return _returnvalue (+ _returnvalue (* (Math|Vector|GetForwardVector _weaponfirepoint) (Variables|Default|GetWeaponRange)))))