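; BP_HealthPickup is a respawning health pickup that heals whatever actor overlaps it.
; On overlap it sends a heal amount through a heal-health interface message, then hides itself and disables its sphere collision.
; A timer calls RespawnPickup after the respawn time, restoring visibility and query-only collision so the pickup can be used again.
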(event Custom|RespawnPickup
  ;[1 1 1] Despawn & Respawn Pickup
  (Collision|SetCollisionEnabled (Variables|Default|GetSphere) "QueryOnly")
  (Rendering|SetActorHiddenInGame false))

(event Custom|DespawnPickup
  ;[1 1 1] Despawn & Respawn Pickup
  (Collision|SetCollisionEnabled (Variables|Default|GetSphere) "NoCollision")
  (Rendering|SetActorHiddenInGame true))

(event EventBeginPlay)

(event Collision|EventActorBeginOverlap
  (params (OtherActor :type Actor%20Object%20Reference))
  ;[1 1 1] Heal Health
  (Class|PickupInterface|IHealHealth(Message) OtherActor (Variables|Default|GetHealAmount))
  (CallFunction|DespawnPickup)
  (Utilities|Time|SetTimerbyFunctionName 0 "RespawnPickup" (Variables|Default|GetRespawnTime)))

(fn ConstructionScript)