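; Player character for StealthMaster that routes input to weapons, gadgets and powers, and links health, inventory and HUD.
; Offensive, Utility and Power are child actor components, driven through interface messages and swapped by class.
; Equip changes play unequip/equip montages by one- or two-handed type, swapping the actor on an anim notify; reload reuses these montages.
; Weapon cycling is rate-limited by gates; mag-boot and melee logic is disconnected, and Z applies test damage.
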(event OnComponentBeginOverlap(Sphere)
  (params (OverlappedComponent :type Primitive%20Component%20Object%20Reference) (OtherActor :type Actor%20Object%20Reference) (OtherComp :type Primitive%20Component%20Object%20Reference) (OtherBodyIndex :type Integer) (bFromSweep :type Boolean) (SweepResult :type Hit%20Result%20Structure%20%28by%20ref%29))
  (Class|IAI|ITouchingMeTouchingYou(Message) OtherActor))

(event Custom|Use%20Grav%20Boots
  ;[1 1 1] GravBoots
)

(event Custom|PlayRelevantEquip/UnequipMontage
  (params (OldWeaponType :type Character_Weapon_Stance%20Enum :default "NewEnumerator0") (NewWeaponType :type Character_Weapon_Stance%20Enum :default "NewEnumerator0") (EquipmentDataPassthru :type Equipment%20Data%20Structure))
  ;[1 0.6527 0] Animation Stuff - pls no touch
  (Variables|Default|SetIncomingEDP EquipmentDataPassthru)
  (Utilities|FlowControl|DoOnce false
    (:Completed
      (switch Utilities|FlowControl|Switch|SwitchonCharacter_Weapon_Stance OldWeaponType
        (:NewEnumerator0
          ;;[1 1 1] 1H Unequip
          (bind _notifyname (Animation|Montage|PlayMontage (Variables|Character|GetMesh) "/Game/StealthMaster/Animation/Mannequin/WeaponUnequip1HManneq_Montage.WeaponUnequip1HManneq_Montage")
            (:then
              (Class|BPIAnimPass|TriggerON(Message) (Variables|Default|GetAnimBPRef))
              (Variables|Default|SetCharacter%20Weapon%20Stance NewWeaponType))
            (:OnNotifyBegin
              (switch name _notifyname
                (:HACF
                  (Class|AnimInstance|MontagePause (Components|SkeletalMesh|GetAnimInstance (Variables|Character|GetMesh)) "/Game/StealthMaster/Animation/Mannequin/WeaponUnequip1HManneq_Montage.WeaponUnequip1HManneq_Montage")
                  (switch Utilities|FlowControl|Switch|SwitchonCharacter_Weapon_Stance NewWeaponType :!label _label
                    (:NewEnumerator0
                      ;;[1 1 1] 1H Equip
                      (bind _notifyname_2 (Animation|Montage|PlayMontage (Variables|Character|GetMesh) "/Game/StealthMaster/Animation/Mannequin/WeaponEquip1HManneq_Montage.WeaponEquip1HManneq_Montage")
                        (:then
                          (Class|BPIAnimPass|TriggerOFF(Message) (Variables|Default|GetAnimBPRef)))
                        (:OnNotifyBegin
                          (switch name _notifyname_2
                            (:WeaponVis
                              (CallFunction|VisibilityonANIM true :!label _label_2)
                              (if (Utilities|Struct|BreakEquipment_Data (Variables|Default|GetIncomingEDP))
                                (ChildActorComponent|SetChildActorClass (Variables|Default|GetUtility) (Utilities|Struct|BreakEquipment_Data (Variables|Default|GetIncomingEDP)))
                                (Class|BPIThrowable|IInitThrowable(Message) (Variables|/Script/Engine.ChildActorComponent|GetChildActor (Variables|Default|GetUtility)) (Variables|Default|GetInventory) (Variables|Default|GetIncomingEDP))
                                (CallFunction|EquipResetMontage)
                                (else
                                  (ChildActorComponent|SetChildActorClass (Variables|Default|GetOffensive) (Utilities|Struct|BreakEquipment_Data (Variables|Default|GetIncomingEDP)))
                                  (Class|WeaponInterface|IInitWeapon(Message) (Variables|/Script/Engine.ChildActorComponent|GetChildActor (Variables|Default|GetOffensive)) (Variables|Default|GetInventory) (Variables|Default|GetIncomingEDP))
                                  (CallFunction|EquipResetMontage))))))))
                    (:NewEnumerator1
                      ;;[1 1 1] 2H Equip
                      (bind _notifyname_3 (Animation|Montage|PlayMontage (Variables|Character|GetMesh) "/Game/StealthMaster/Animation/Mannequin/WeaponEquip2HManneq_Montage.WeaponEquip2HManneq_Montage")
                        (:OnCompleted
                          (Class|BPIAnimPass|TriggerOFF(Message) (Variables|Default|GetAnimBPRef)))
                        (:OnNotifyBegin
                          (switch name _notifyname_3
                            (:WeaponVis
                              (goto _label_2))))))))))))
        (:NewEnumerator1
          ;;[1 1 1] 2H Unequip
          (bind _notifyname_4 (Animation|Montage|PlayMontage (Variables|Character|GetMesh) "/Game/StealthMaster/Animation/Mannequin/WeaponUnequip2HManneq_Montage.WeaponUnequip2HManneq_Montage")
            (:then
              (Class|BPIAnimPass|TriggerON(Message) (Variables|Default|GetAnimBPRef))
              (Variables|Default|SetCharacter%20Weapon%20Stance NewWeaponType))
            (:OnNotifyBegin
              (switch name _notifyname_4
                (:HACF
                  (Class|AnimInstance|MontagePause (Components|SkeletalMesh|GetAnimInstance (Variables|Character|GetMesh)) "/Game/StealthMaster/Animation/Mannequin/WeaponUnequip1HManneq_Montage.WeaponUnequip1HManneq_Montage")
                  (goto _label))))))))))

(event Custom|EquipResetMontage
  ;[1 0.6527 0] Animation Stuff - pls no touch
  (Utilities|FlowControl|DoOnce false) ; enters at Reset
)

(event Custom|VisibilityOnANIM
  (params (Offensive/Utility%20T/F :type Boolean))
  ;[1 0.6527 0] Animation Stuff - pls no touch
  (if Offensive/Utility%20T/F
    (Rendering|SetVisibility (Variables|Default|GetOffensive) true false)
    (else
      (Rendering|SetVisibility (Variables|Default|GetUtility) true false))))

(event Custom|VisibilityOffANIM
  (params (Offensive/Utility%20T/F :type Boolean))
  ;[1 0.6527 0] Animation Stuff - pls no touch
  (if Offensive/Utility%20T/F
    (Rendering|SetVisibility (Variables|Default|GetOffensive) false false)
    (else
      (Rendering|SetVisibility (Variables|Default|GetUtility) false false))))

(event Custom|ReloadTriggerAnim
  (bind _mesh (Variables|Character|GetMesh))
  (bind _mesh_2 (Variables|Character|GetMesh))
  (Utilities|FlowControl|DoOnce false
    (:Completed
      (switch Utilities|FlowControl|Switch|SwitchonCharacter_Weapon_Stance (Variables|Default|GetCharacter%20Weapon%20Stance)
        (:NewEnumerator0
          (bind _notifyname (Animation|Montage|PlayMontage _mesh_2 "/Game/StealthMaster/Animation/Mannequin/WeaponUnequip1HManneq_Montage.WeaponUnequip1HManneq_Montage")
            (:OnNotifyBegin
              (switch name _notifyname
                (:HACF
                  (Class|AnimInstance|MontagePause (Components|SkeletalMesh|GetAnimInstance (Variables|Character|GetMesh)) "/Game/StealthMaster/Animation/Mannequin/WeaponUnequip1HManneq_Montage.WeaponUnequip1HManneq_Montage")
                  (Animation|Montage|PlayMontage _mesh "/Game/StealthMaster/Animation/Mannequin/WeaponEquip1HManneq_Montage.WeaponEquip1HManneq_Montage"
                    (:OnCompleted
                      _)))))))
        (:NewEnumerator1
          (bind _notifyname_2 (Animation|Montage|PlayMontage _mesh_2 "/Game/StealthMaster/Animation/Mannequin/WeaponUnequip2HManneq_Montage.WeaponUnequip2HManneq_Montage" 0.7)
            (:OnNotifyBegin
              (switch name _notifyname_2
                (:HACF
                  (Class|AnimInstance|MontagePause (Components|SkeletalMesh|GetAnimInstance (Variables|Character|GetMesh)) "/Game/StealthMaster/Animation/Mannequin/WeaponUnequip1HManneq_Montage.WeaponUnequip1HManneq_Montage")
                  (Animation|Montage|PlayMontage _mesh "/Game/StealthMaster/Animation/Mannequin/WeaponEquip2HManneq_Montage.WeaponEquip2HManneq_Montage" 0.7
                    (:OnCompleted
                      _))))))))
      (Class|WeaponInterface|IReloadWeapon(Message) (Variables|/Script/Engine.ChildActorComponent|GetChildActor (Variables|Default|GetOffensive)))
      (CallFunction|ResetReloadAnim)
      (Variables|Default|SetIsReloading false))))

(event Custom|ResetReloadAnim
  (bind _mesh (Variables|Character|GetMesh))
  (bind _mesh_2 (Variables|Character|GetMesh))
  (Utilities|FlowControl|DoOnce false) ; enters at Reset
)

(event Custom|ControlledCycle_Forward
  ;[1 1 1] FUCKING ISH
  (Utilities|FlowControl|Gate false :!label _label
    (:Exit
      (Utilities|FlowControl|Sequence
        (:then_0
          (goto _label Close))
        (:then_1
          (Utilities|FlowControl|Delay (Variables|Default|GetRateOfFire))
          (goto _label Open))
        (:then_2
          (Default|Cycle (Variables|Default|GetInventory) "NewEnumerator0" "NewEnumerator0"))))))

(event Custom|ControlledCycle_Backwards
  ;[1 1 1] FUCKING ISH
  (Utilities|FlowControl|Gate false :!label _label
    (:Exit
      (Utilities|FlowControl|Sequence
        (:then_0
          (goto _label Close))
        (:then_1
          (Utilities|FlowControl|Delay (Variables|Default|GetRateOfFire))
          (goto _label Open))
        (:then_2
          (Default|Cycle (Variables|Default|GetInventory) "NewEnumerator0" "NewEnumerator1"))))))

(event EventBeginPlay
  ;[0 1 0.07173] BEGIN PLAY
  (CallFunction|Init)
  (EventDispatchers|BindEventtoOnEquip (Variables|Default|GetInventory) (EventDispatchers|CreateEvent :!event FHandleEquip))
  (bind _assm_player_char_anim_bp (Utilities|Casting|CastToSM_PlayerChar_AnimBP (Components|SkeletalMesh|GetAnimInstance (Variables|Character|GetMesh))))
  (Variables|Default|SetAnimBPRef _assm_player_char_anim_bp))

(event Game|Damage|EventAnyDamage
  (params (Damage :type Float%20%28single-precision%29) (DamageType :type Damage%20Type%20Object%20Reference) (InstigatedBy :type Controller%20Object%20Reference) (DamageCauser :type Actor%20Object%20Reference))
  ;[1 1 1] Health System Logic
  (Default|TakeDamage (Variables|Default|GetHealthSystem) Damage))

(event EventIThrowGadget
  ;[1 0.6527 0] Animation Stuff - pls no touch
  (bind _notifyname (Animation|Montage|PlayMontage (Variables|Character|GetMesh) "/Game/StealthMaster/Animation/Mannequin/GrenadeThrowMannequin_Montage.GrenadeThrowMannequin_Montage")
    (:then
      (CallFunction|VisibilityOffANIM true))
    (:OnCompleted
      (CallFunction|VisibilityonANIM true))
    (:OnNotifyBegin
      (if (Utilities|Name|Equal(Name) _notifyname "ReleasePoint")
        (Class|BPIThrowable|IThrow(Message) (Variables|/Script/Engine.ChildActorComponent|GetChildActor (Variables|Default|GetUtility)))))))

(event EventIShowInteract
  ;[1 1 1] Notification Logic
  (Default|NotificationToggle (Variables|Default|GetHUD) true))

(event EventIHideInteract
  ;[1 1 1] Notification Logic
  (Default|NotificationToggle (Variables|Default|GetHUD) false))

(event EventISetPower
  (params (Power :type Base%20Power%20Class%20Class%20Reference))
  ;[1 1 1] Ability Input Logic
  (if (Variables|Default|GetIsPossessed)
    (ChildActorComponent|SetChildActorClass (Variables|Default|GetPower) Power)))

(event EventUnpossessed
  (params (OldController :type Controller%20Object%20Reference))
  (Variables|Default|SetIsPossessed false)
  (Class|WeaponInterface|IFireReleased(Message) (Variables|/Script/Engine.ChildActorComponent|GetChildActor (Variables|Default|GetOffensive))))

(event EventIHUDRemoveObjective
  (params (ID :type Array%20of%20Integers))
  (Default|ObjectiveRemove (Variables|Default|GetHUD) ID))

(event EventPossessed
  (params (NewController :type Controller%20Object%20Reference))
  (Variables|Default|SetIsPossessed true))

(event EventIInventory
  ;[1 1 1] Inventory Logic
  (Default|ToggleShowInv (Variables|/Game/StealthMaster/Tech/UI/InGame/HUD/HUD.HUD_C|GetInvMenu (Variables|Default|GetHUD))))

(event EventOnLanded
  (params (Hit :type Hit%20Result%20Structure%20%28by%20ref%29))
  ;[1 1 1] Testing GravBoots
  (CallFunction|UpdateStance "NewEnumerator0"))

(event EventIPickupEquipment
  (params (Equipment_Class :type Equipment%20Base%20Class%20Reference) (Equip :type Boolean))
  ;[1 1 1] Inventory Logic
  (Default|Pickup (Variables|Default|GetInventory) Equipment_Class Equip))

(event EventIUseAbility
  ;[1 1 1] Ability Input Logic
  (if (Variables|Default|GetIsPossessed)
    (Class|PowersInterface|UseAbility(Message) (Variables|/Script/Engine.ChildActorComponent|GetChildActor (Variables|Default|GetPower)) (Pawn|GetController))))

(event EventIReload
  ;[1 1 1] Weapons & Gadgets Logic
  (if (Variables|Default|GetIsPossessed)
    (bind _canreload (Class|WeaponInterface|ICanReload(Message) (Variables|/Script/Engine.ChildActorComponent|GetChildActor (Variables|Default|GetOffensive))))
    (if _canreload
      (Variables|Default|SetIsReloading true)
      (CallFunction|ReloadTriggerAnim))))

(event EventIMousePrimary
  ;[1 1 1] Weapons & Gadgets Logic
  (if (Variables|Default|GetIsPossessed)
    (if (not (Variables|Default|GetIsReloading))
      (Class|WeaponInterface|IFirePressed(Message) (Variables|/Script/Engine.ChildActorComponent|GetChildActor (Variables|Default|GetOffensive))))))

(event EventTick
  (params (DeltaSeconds :type Float%20%28single-precision%29))
  (if (> (Math|Vector|VectorLengthXY (Variables|/Script/Engine.MovementComponent|GetVelocity (Variables|Character|GetCharacterMovement))) 0.0)
    (Variables|Default|SetbUseControllerRotationYaw true)
    (else
      (Variables|Default|SetbUseControllerRotationYaw false))))

(event EventIPrimaryRelease
  ;[1 1 1] Weapons & Gadgets Logic
  (Class|WeaponInterface|IFireReleased(Message) (Variables|/Script/Engine.ChildActorComponent|GetChildActor (Variables|Default|GetOffensive))))

(event Input|ActionEvents|InputActionMelee
  (params (Key :type Key%20Structure))
  ;[1 1 1] Melee Testing (disconnected)
)

(event Input|ActionEvents|InputActionCycleForward
  (params (Key :type Key%20Structure))
  ;[1 1 1] Inventory Logic
  (:Pressed
    (CallFunction|ControlledCycleForward)))

(event Input|ActionEvents|InputActionCycleBackward
  (params (Key :type Key%20Structure))
  ;[1 1 1] Inventory Logic
  (:Pressed
    (CallFunction|ControlledCycleBackwards)))

(event Input|KeyboardEvents|Z
  (params (Key :type Key%20Structure))
  ;[1 1 1] Health System Logic
  (:Pressed
    (Default|TakeDamage (Variables|Default|GetHealthSystem) 5e+01)))

(fn ConstructionScript
  (|CallParentFunction)
  (Components|Sphere|SetSphereRadius (Variables|Default|GetSphere) (Variables|Default|GetautoDetecttSphereRadius) true))

(fn Init
  (Class|PlayerControllerInterface|ISetPlayerPawnReference(Message) (Pawn|GetController) self)
  (bind _success (|CallParentFunction))
  (return _success))

(fn FHandleEquip
  (params (inventory :type Inventory%20Object%20Reference) (Equipment_Data :type Equipment%20Data%20Structure))
  (LocalVariables|Set_EquipmentData Equipment_Data)
  (switch Utilities|FlowControl|Switch|SwitchonEquipment_Type (Utilities|Struct|BreakEquipment_Data (LocalVariables|Get_EquipmentData))
    (:NewEnumerator0
      (bind _asbp_base_weapon (Utilities|Casting|CastToBP_BaseWeapon (Variables|/Script/Engine.ChildActorComponent|GetChildActor (Variables|Default|GetOffensive)))
        (:then
          (CallFunction|PlayRelevantEquip/UnequipMontage (Variables|/Game/StealthMaster/Tech/Weapons-Gadgets-Pickups/EquipmentBase/Equipment_Base.Equipment_Base_C|GetOffensiveType _asbp_base_weapon) (.OffensiveType (Utilities|GetClassDefaults (.Class (Utilities|Struct|BreakEquipment_Data (LocalVariables|Get_EquipmentData))))) Equipment_Data))
        (:CastFailed
          (bind _asbp_base_projectile_gadget (Utilities|Casting|CastToBP_BaseProjectileGadget (Variables|/Script/Engine.ChildActorComponent|GetChildActor (Variables|Default|GetOffensive))))
          (CallFunction|PlayRelevantEquip/UnequipMontage (Variables|/Game/StealthMaster/Tech/Weapons-Gadgets-Pickups/EquipmentBase/Equipment_Base.Equipment_Base_C|GetOffensiveType _asbp_base_projectile_gadget) (.OffensiveType (Utilities|GetClassDefaults (.Class (Utilities|Struct|BreakEquipment_Data (LocalVariables|Get_EquipmentData))))) Equipment_Data))))
    (:NewEnumerator1
      (if (Utilities|Struct|BreakEquipment_Data (LocalVariables|Get_EquipmentData))
        (ChildActorComponent|SetChildActorClass (Variables|Default|GetUtility) (Utilities|Struct|BreakEquipment_Data (LocalVariables|Get_EquipmentData)))
        (Class|BPIThrowable|IInitThrowable(Message) (Variables|/Script/Engine.ChildActorComponent|GetChildActor (Variables|Default|GetUtility)) (Variables|Default|GetInventory) (LocalVariables|Get_EquipmentData))
        (else
          (bind _asbp_base_weapon_2 (Utilities|Casting|CastToBP_BaseWeapon (Variables|/Script/Engine.ChildActorComponent|GetChildActor (Variables|Default|GetOffensive))))
          (CallFunction|PlayRelevantEquip/UnequipMontage (Variables|/Game/StealthMaster/Tech/Weapons-Gadgets-Pickups/EquipmentBase/Equipment_Base.Equipment_Base_C|GetOffensiveType _asbp_base_weapon_2) (.OffensiveType (Utilities|GetClassDefaults (.Class (Utilities|Struct|BreakEquipment_Data (LocalVariables|Get_EquipmentData))))) Equipment_Data))))))

(fn FCanMagBoot
  (bind _capsulecomponent (Variables|Default|GetCapsuleComponent))
  (bind _returnvalue (Transformation|GetWorldLocation _capsulecomponent))
  (if (Variables|Default|GetUsing%20Mag%20Boots)
    (bind _outhit (Collision|CapsuleTraceByChannel (Transformation|GetWorldLocation (Variables|Default|GetCapsuleComponent)) (Math|Vector|MakeVector (.x _returnvalue) (.y _returnvalue) (+ (.z _returnvalue) 2e+03)) 24.0 0.0 "TraceTypeQuery1" false 0 "ForOneFrame"))
    (if (> (.Distance (Collision|BreakHitResult _outhit)) 75.0)
      (if (< (.Distance (Collision|BreakHitResult _outhit)) 1e+03)
        (return true)
        (else
          _)))
    (return false)))

(fn AddObjective
  (params (Type :type ObjectiveType%20Enum :default "NewEnumerator0") (Text :type Text))
  (return 0))

(fn IGetHealthSystem
  (return (Variables|Default|GetHealthSystem)))

(fn IGetInventory
  (return (Variables|Default|GetInventory)))

(fn IGetPower
  (bind _asbase_power_class (Utilities|Casting|CastToBase_Power_Class (Variables|/Script/Engine.ChildActorComponent|GetChildActor (Variables|Default|GetPower))))
  (return _asbase_power_class))

(fn IHUDAddObjective
  (params (Type :type ObjectiveType%20Enum :default "NewEnumerator0") (Description :type Text))
  (bind _id_ (Default|ObjectiveAdd (Variables|Default|GetHUD) Type Description))
  (return _id_))

(fn ISetHUD
  (params (HUD%20Reference :type HUD%20Object%20Reference))
  (Variables|Default|SetHUD HUD%20Reference)
  (Default|INIT (Variables|Default|GetInventory) (Variables|Default|GetHUD))
  (bind _power (CallFunction|IGetPower))
  (Default|PowerAssign (Variables|Default|GetHUD) _power)
  (return true))