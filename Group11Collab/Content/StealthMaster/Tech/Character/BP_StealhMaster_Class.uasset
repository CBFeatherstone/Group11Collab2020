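; BP_StealhMaster_Class is the player's StealthMaster character, able to possess other objects in the world.
; On BeginPlay, Init registers it with its controller as the player pawn through an interface message, then runs the parent's Init.
; Pressing H box-traces from screen center for Possessable objects, asks the hit actor for a pawn via IPossessMessage, possesses it and calls AfterUnPossess.
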(event EventBeginPlay
  (CallFunction|Init))

(event Input|KeyboardEvents|H
  (params (Key :type Key%20Structure))
  (bind _returnvalue (Viewport|GetViewportSize))
  (bind _returnvalue_2 (Game|GetPlayerController 0))
  (bind _returnvalue_3 (/ _returnvalue 2.0))
  (bind (_worldposition _worlddirection) (Class|GameplayStatics|DeprojectScreentoWorld _returnvalue_2 _returnvalue_3))
  (:Pressed
    (bind (_outhit _returnvalue_4) (Class|KismetSystemLibrary|BoxTraceSingleforObjects _worldposition (+ _worldposition (* _worlddirection 10000)) "20.000000,20.000000,20.000000" "0, 0, 0" (Variables|Default|GetPossessable) false 0 "ForDuration" true))
    (if _returnvalue_4
      (bind _pawntopossess (Class|CharacterInterface|IPossess(Message) (.HitActor (Collision|BreakHitResult _outhit))))
      (Pawn|Possess (Pawn|GetController) _pawntopossess)
      (CallFunction|AfterUnPossess))))

(fn ConstructionScript
  (|CallParentFunction))

(fn Init
  (Class|PlayerControllerInterface|ISetPlayerPawnReference(Message) (Pawn|GetController) self)
  (bind _success (|CallParentFunction))
  (return _success))